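; HTTP client component that drives AI dialogue for historical ancient Greek characters through a Gemini-style API.
; BeginPlay loads a character JSON file, whose per-ID fields feed prompt builders for full, opening, follow-up and player-option prompts.
; SendAIRequest escapes the prompt into a JSON template, POSTs it and broadcasts the parsed text through OnAIResponseReceived.
; Failed requests broadcast three canned dialogue options through that same dispatcher, leaving the success/error event parameters unused.
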(event `self.ReceiveBeginPlay`
  (`self.Load_Character_Data`))

(event `Send AI Request`
  (params (Prompt :type String) (On_Success_Event :type String) (On_Error_Event :type String))
  (bind (_outheader _result_body) (`|HttpRequest` (`KismetStringLibrary.Concat_StrStr` (`KismetStringLibrary.Concat_StrStr` (`self.API_Base_URL`) "?key=") (`self.API_Key`)) "Post" (`|MakeRequestHeader` "Custom" "Content-Type" "application/json") (`KismetStringLibrary.Replace` (`self.JSON_Template`) "{0}" (`KismetStringLibrary.Replace` (`KismetStringLibrary.Replace` (`KismetStringLibrary.Replace` (`KismetStringLibrary.Replace` Prompt "\\" "\\\\") "\"" "\\\"") " \n" "\\n") "\\r")))
    (:`On Success`
      (bind _ai_text (`self.Parse Gemini Response` _result_body))
      (`self.OnAIResponseReceived` _ai_text))
    (:`On Error`
      (`self.OnAIResponseReceived` "OPTION1: Tell me more \nOPTION2: What else can you tell me? \nOPTION3: Goodbye"))))

(fn `Build_Followup_Prompt`
  (params (Character_ID :type String) (Player_Input :type String) (Context :type String))
  (returns (Full_Prompt :type String))
  (bind _field_value (`self.Get_Character_Field` Character_ID "display_name"))
  (bind _field_value_2 (`self.Get_Character_Field` Character_ID "occupation"))
  (bind _field_value_3 (`self.Get_Character_Field` Character_ID "location"))
  (bind _field_value_4 (`self.Get_Character_Field` Character_ID "era"))
  (bind _field_value_5 (`self.Get_Character_Field` Character_ID "speech_patterns"))
  (bind _field_value_6 (`self.Get_Character_Field` Character_ID "system_directive"))
  (bind _field_value_7 (`self.Get_Character_Field` Character_ID "personality_traits"))
  (bind _field_value_8 (`self.Get_Character_Field` Character_ID "relationships"))
  (bind _field_value_9 (`self.Get_Character_Field` Character_ID "knowledge_areas"))
  (bind _field_value_10 (`self.Get_Character_Field` Character_ID "knowledge_limitations"))
  (bind _field_value_11 (`self.Get_Character_Field` Character_ID "key_beliefs"))
  (return (`KismetStringLibrary.Concat_StrStr` (`KismetStringLibrary.Concat_StrStr` (`KismetStringLibrary.Concat_StrStr` (`KismetStringLibrary.Concat_StrStr` (`KismetStringLibrary.Concat_StrStr` (`KismetStringLibrary.Concat_StrStr` (`KismetStringLibrary.Concat_StrStr` (`KismetStringLibrary.Concat_StrStr` (`KismetStringLibrary.Concat_StrStr` (`KismetStringLibrary.Concat_StrStr` (`KismetStringLibrary.Concat_StrStr` (`KismetStringLibrary.Concat_StrStr` (`KismetStringLibrary.Concat_StrStr` (`KismetStringLibrary.Concat_StrStr` (`KismetStringLibrary.Concat_StrStr` (`KismetStringLibrary.Concat_StrStr` (`KismetStringLibrary.Concat_StrStr` (`KismetStringLibrary.Concat_StrStr` (`KismetStringLibrary.Concat_StrStr` (`KismetStringLibrary.Concat_StrStr` (`KismetStringLibrary.Concat_StrStr` (`KismetStringLibrary.Concat_StrStr` (`KismetStringLibrary.Concat_StrStr` (`KismetStringLibrary.Concat_StrStr` (`KismetStringLibrary.Concat_StrStr` (`KismetStringLibrary.Concat_StrStr` "You are " _field_value) ", a ") _field_value_2) " in ") _field_value_3) " (") _field_value_4) ").\n") _field_value_6) "\n\nPersonality: ") _field_value_7) "\nRelationships: ") _field_value_8) "\nKnowledge: ") _field_value_9) "\nLimitations: ") _field_value_10) "\nKey Beliefs: ") _field_value_11) "\nSpeech Style: ") _field_value_5) "\n\nChat History:\n") Context) "\n\nPlayer said: \"") Player_Input) "\"\n\nRespond in character. Keep response under 40 words. Stay historically accurate.")))

(fn `Build_Full_Prompt`
  (params (Character_ID :type String) (Player_Input :type String) (Context :type String :default "The player is an adventurer visiting Petra."))
  (returns (Full_Prompt :type String))
  (bind _field_value (`self.Get_Character_Field` Character_ID "display_name"))
  (bind _field_value_2 (`self.Get_Character_Field` Character_ID "occupation"))
  (bind _field_value_3 (`self.Get_Character_Field` Character_ID "location"))
  (bind _field_value_4 (`self.Get_Character_Field` Character_ID "era"))
  (bind _field_value_5 (`self.Get_Character_Field` Character_ID "personality_traits"))
  (bind _field_value_6 (`self.Get_Character_Field` Character_ID "knowledge_areas"))
  (bind _field_value_7 (`self.Get_Character_Field` Character_ID "knowledge_limitations"))
  (bind _field_value_8 (`self.Get_Character_Field` Character_ID "speech_patterns"))
  (bind _field_value_9 (`self.Get_Character_Field` Character_ID "key_beliefs"))
  (bind _field_value_10 (`self.Get_Character_Field` Character_ID "famous_quotes"))
  (bind _field_value_11 (`self.Get_Character_Field` Character_ID "teaching_topics"))
  (bind _field_value_12 (`self.Get_Character_Field` Character_ID "conversation_starters"))
  (return (`KismetTextLibrary.Conv_TextToString` (`|FormatText` "You are {character_name}, a {occupation} in {location} during {era}. \n \nPersonality: {personality} \nKey Beliefs: {key_beliefs} \nKnowledge Areas: You know about {knowledge} but are unaware of {limitations} \nTeaching Topics: {teaching_topics} \nFamous Quotes: {famous_quotes} \nSpeech Style: {speech} \n \nIMPORTANT RULES: \n- If the player's message is a greeting or the conversation is just starting, you MUST use one of these exact opening lines (chosen randomly): {conversation_starters} \n- For follow-up messages, respond naturally in character. \n- Stay historically accurate to {era}. Never reference anything beyond your time period. \n- Keep responses under 40 words. \nCurrent context: {context} \nPlayer said: \"{input}\"" _field_value _field_value_2 _field_value_3 _field_value_4 _field_value_5 _field_value_9 _field_value_6 _field_value_7 _field_value_11 _field_value_10 _field_value_8 _field_value_12 Context Player_Input))))

(fn `Build_Opening_Prompt`
  (params (Character_ID :type String) (Player_Input :type String))
  (returns (Full_Prompt :type String))
  (bind _field_value (`self.Get_Character_Field` Character_ID "display_name"))
  (bind _field_value_2 (`self.Get_Character_Field` Character_ID "occupation"))
  (bind _field_value_3 (`self.Get_Character_Field` Character_ID "location"))
  (bind _field_value_4 (`self.Get_Character_Field` Character_ID "era"))
  (bind _field_value_5 (`self.Get_Character_Field` Character_ID "speech_patterns"))
  (bind _field_value_6 (`self.Get_Character_Field` Character_ID "conversation_starters"))
  (bind _field_value_7 (`self.Get_Character_Field` Character_ID "system_directive"))
  (return (`KismetStringLibrary.Concat_StrStr` (`KismetStringLibrary.Concat_StrStr` (`KismetStringLibrary.Concat_StrStr` (`KismetStringLibrary.Concat_StrStr` (`KismetStringLibrary.Concat_StrStr` (`KismetStringLibrary.Concat_StrStr` (`KismetStringLibrary.Concat_StrStr` (`KismetStringLibrary.Concat_StrStr` (`KismetStringLibrary.Concat_StrStr` (`KismetStringLibrary.Concat_StrStr` (`KismetStringLibrary.Concat_StrStr` (`KismetStringLibrary.Concat_StrStr` (`KismetStringLibrary.Concat_StrStr` (`KismetStringLibrary.Concat_StrStr` "You are " _field_value) ", a ") _field_value_2) " in ") _field_value_3) " during ") _field_value_4) ".\n") _field_value_7) "\n\nSpeech Style: ") _field_value_5) "\n\nYou MUST respond with one of these EXACT lines (pick one randomly):\n") _field_value_6) "\n\nDo NOT generate your own greeting. Use one of the lines above word-for-word. Keep your response under 30 words.")))

(fn `Build_Options_Prompt`
  (params (Character_ID :type String) (ConversationContext :type String) (LastAIResponse :type String))
  (returns (OptionsPrompt :type String))
  (bind _field_value (`self.Get_Character_Field` Character_ID "display_name"))
  (return (`KismetStringLibrary.Concat_StrStr` (`KismetStringLibrary.Concat_StrStr` (`KismetStringLibrary.Concat_StrStr` (`KismetStringLibrary.Concat_StrStr` (`KismetStringLibrary.Concat_StrStr` (`KismetStringLibrary.Concat_StrStr` "Based on this conversation with " _field_value) ", suggest exactly 3 short dialogue options the player could say next. The options should be relevant to the conversation and in-character for the setting.\n\nLast AI response: ") LastAIResponse) "\n\nConversation context: ") ConversationContext) "\n\nRespond with ONLY 3 options in this EXACT format with no other text:\nOPTION1: [option text]\nOPTION2: [option text]\nOPTION3: [option text]")))

(fn `Get_Character_Field`
  (params (Character_ID :type String) (Field_Name :type String))
  (returns (Field_Value :type String))
  (bind _outvalue (`|GetJsonField` (`self.Character_JSON_Data`) "characters"))
  (bind _outvalue_2 (`|GetJsonField` _outvalue Character_ID))
  (bind _outvalue_3 (`|GetJsonField` _outvalue_2 Field_Name))
  (return _outvalue_3))

(fn `Load_Character_Data`
  (returns (Success :type Boolean))
  (bind (_outjsonobject _returnvalue) (`JsonBlueprintFunctionLibrary.FromFile` (make `FilePath` (`KismetStringLibrary.Concat_StrStr` (`KismetSystemLibrary.GetProjectDirectory`) "Content/Characters/ancient_greece_characters.json"))))
  (bind _output_get (set `self.Character_JSON_Data` _outjsonobject))
  (bind (_outjsonstring _returnvalue_2) (`JsonBlueprintFunctionLibrary.ToString` _output_get))
  (return _returnvalue_2))

(fn `Parse Gemini Response`
  (params (JSON_String :type String))
  (returns (AI_Text :type String))
  (bind _outjsonobject (`JsonBlueprintFunctionLibrary.FromString` JSON_String))
  (bind _outvalue (`|GetJsonField` _outjsonobject "candidates"))
  (bind _outvalue_2 (`|GetJsonField` _outvalue "content"))
  (bind _outvalue_3 (`|GetJsonField` _outvalue_2 "parts"))
  (bind _outvalue_4 (`|GetJsonField` _outvalue_3 "text"))
  (return _outvalue_4))