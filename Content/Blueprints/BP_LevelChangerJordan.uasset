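; Level-change trigger that moves the player to the Level soft reference when their character overlaps its Sphere.
; The overlap shows a timed WBP_LoadingScreen, requests an async load of the level and listens for the screen's completion event.
; On completion it adds IntroQuest00 if not active, copies player progression, quests, inventory, codex and Greece/Petra flags into BP_GameInstance, then opens the level.
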(event `self.Sphere.OnComponentBeginOverlap`
  (params (OverlappedComponent :type "PrimitiveComponent Object Reference") (OtherActor :type "Actor Object Reference") (OtherComp :type "PrimitiveComponent Object Reference") (OtherBodyIndex :type Integer) (bFromSweep :type Boolean) (SweepResult :type "HitResult Structure (by ref)"))
  (if (and (== OtherActor (`GameplayStatics.GetPlayerCharacter` 0)) (`KismetSystemLibrary.IsValidSoftObjectReference` (`self.Level`)))
    (bind _returnvalue (`|CreateWidget` "/Game/ThirdPerson/MainMenu/UI/WBP_LoadingScreen.WBP_LoadingScreen_C" null 5.0))
    (`UserWidget.AddToViewport` _returnvalue 0)
    (`|LoadAsset` (`self.Level`)
      (:`then`
        (add `/Game/ThirdPerson/MainMenu/UI/WBP_LoadingScreen.OnLoadingCompleted` _returnvalue (delegate `On Loading Completed`))))))

(event `On Loading Completed`
  (bind _level (`self.Level`))
  (bind _myplayercharacter (`/Game/ThirdPerson/CommonFunctionLibrary.GetMyPlayerCharacter`))
  (bind _returnvalue (`self.GetComponentByClass` _myplayercharacter "/Game/ThirdPerson/QuestSYstem/QuestLog_Component.QuestLog_Component_C"))
  (if (`KismetArrayLibrary.Array_Contains` (`/Game/ThirdPerson/QuestSYstem/QuestLog_Component.CurrentActiveQuests` _returnvalue) "IntroQuest00")
    (bind _asbp_game_instance (cast `/Game/BP_GameInstance` (`GameplayStatics.GetGameInstance`)))
    (bind _myplayercharacter_2 (`/Game/ThirdPerson/CommonFunctionLibrary.GetMyPlayerCharacter`))
    (set `/Game/BP_GameInstance.Saved_KnowledgePoints` (`/Game/ThirdPerson/Blueprints/BP_ThirdPersonCharacter.KnowledgePoints` _myplayercharacter_2) _asbp_game_instance)
    (set `/Game/BP_GameInstance.Saved_PlayerLevel` (`/Game/ThirdPerson/Blueprints/BP_ThirdPersonCharacter.PlayerLevel` _myplayercharacter_2) _asbp_game_instance)
    (set `/Game/BP_GameInstance.Saved_CurrentXP` (`/Game/ThirdPerson/Blueprints/BP_ThirdPersonCharacter.CurrentXP` _myplayercharacter_2) _asbp_game_instance)
    (set `/Game/BP_GameInstance.Saved_XPToNextLevel` (`/Game/ThirdPerson/Blueprints/BP_ThirdPersonCharacter.XPToNextLevel` _myplayercharacter_2) _asbp_game_instance)
    (set `/Game/BP_GameInstance.Saved_MaxKnowledgePoints` (`/Game/ThirdPerson/Blueprints/BP_ThirdPersonCharacter.MaxKnowledgePoints` _myplayercharacter_2) _asbp_game_instance)
    (bind _returnvalue_2 (`self.GetComponentByClass` _myplayercharacter_2 "/Game/ThirdPerson/QuestSYstem/QuestLog_Component.QuestLog_Component_C"))
    (set `/Game/BP_GameInstance.Saved_CompletedQuests` (`/Game/ThirdPerson/QuestSYstem/QuestLog_Component.Completed` _returnvalue_2) _asbp_game_instance)
    (set `/Game/BP_GameInstance.Saved_ActiveQuests` (`/Game/ThirdPerson/QuestSYstem/QuestLog_Component.CurrentActiveQuests` _returnvalue_2) _asbp_game_instance)
    (set `/Game/BP_GameInstance.Saved_InventoryItems` (`/Game/ThirdPerson/Inventory/BP_InventoryComponent.CollectedItems` (`self.GetComponentByClass` "/Game/ThirdPerson/Inventory/BP_InventoryComponent.BP_InventoryComponent_C")) _asbp_game_instance)
    (set `/Game/BP_GameInstance.Saved_UnlockedCodexEntries` (`/Game/ThirdPerson/Codex/BP_CodexSystem.UnlockedEntries` (`self.GetComponentByClass` "/Game/ThirdPerson/Codex/BP_CodexSystem.BP_CodexSystem_C")) _asbp_game_instance)
    (set `/Game/BP_GameInstance.Saved_GreeceToVoidQuest` (`/Game/ThirdPerson/Blueprints/BP_ThirdPersonCharacter.bIsGreeceDone` _myplayercharacter_2) _asbp_game_instance)
    (set `/Game/BP_GameInstance.Saved_PetraToVoidQuest` (`/Game/ThirdPerson/Blueprints/BP_ThirdPersonCharacter.bIsPetraDone` _myplayercharacter_2) _asbp_game_instance)
    (`GameplayStatics.OpenLevelBySoftObjectPtr` _level)
    (else
      (`KismetSystemLibrary.PrintString` "If Current Active Quest is False as IntroQuest00 adding introquest")
      (`/Game/ThirdPerson/QuestSYstem/QuestLog_Component.AddNewQuest` _returnvalue "IntroQuest00")
      (bind _asbp_game_instance_2 (cast `/Game/BP_GameInstance` (`GameplayStatics.GetGameInstance`)))
      (bind _myplayercharacter_3 (`/Game/ThirdPerson/CommonFunctionLibrary.GetMyPlayerCharacter`))
      (set `/Game/BP_GameInstance.Saved_KnowledgePoints` (`/Game/ThirdPerson/Blueprints/BP_ThirdPersonCharacter.KnowledgePoints` _myplayercharacter_3) _asbp_game_instance_2)
      (set `/Game/BP_GameInstance.Saved_PlayerLevel` (`/Game/ThirdPerson/Blueprints/BP_ThirdPersonCharacter.PlayerLevel` _myplayercharacter_3) _asbp_game_instance_2)
      (set `/Game/BP_GameInstance.Saved_CurrentXP` (`/Game/ThirdPerson/Blueprints/BP_ThirdPersonCharacter.CurrentXP` _myplayercharacter_3) _asbp_game_instance_2)
      (set `/Game/BP_GameInstance.Saved_XPToNextLevel` (`/Game/ThirdPerson/Blueprints/BP_ThirdPersonCharacter.XPToNextLevel` _myplayercharacter_3) _asbp_game_instance_2)
      (set `/Game/BP_GameInstance.Saved_MaxKnowledgePoints` (`/Game/ThirdPerson/Blueprints/BP_ThirdPersonCharacter.MaxKnowledgePoints` _myplayercharacter_3) _asbp_game_instance_2)
      (bind _returnvalue_3 (`self.GetComponentByClass` _myplayercharacter_3 "/Game/ThirdPerson/QuestSYstem/QuestLog_Component.QuestLog_Component_C"))
      (set `/Game/BP_GameInstance.Saved_ActiveQuests` (`/Game/ThirdPerson/QuestSYstem/QuestLog_Component.CurrentActiveQuests` _returnvalue_3) _asbp_game_instance_2)
      (set `/Game/BP_GameInstance.Saved_CompletedQuests` (`/Game/ThirdPerson/QuestSYstem/QuestLog_Component.Completed` _returnvalue_3) _asbp_game_instance_2)
      (set `/Game/BP_GameInstance.Saved_InventoryItems` (`/Game/ThirdPerson/Inventory/BP_InventoryComponent.CollectedItems` (`self.GetComponentByClass` _myplayercharacter_3 "/Game/ThirdPerson/Inventory/BP_InventoryComponent.BP_InventoryComponent_C")) _asbp_game_instance_2)
      (set `/Game/BP_GameInstance.Saved_UnlockedCodexEntries` (`/Game/ThirdPerson/Codex/BP_CodexSystem.UnlockedEntries` (`self.GetComponentByClass` _myplayercharacter_3 "/Game/ThirdPerson/Codex/BP_CodexSystem.BP_CodexSystem_C")) _asbp_game_instance_2)
      (set `/Game/BP_GameInstance.Saved_GreeceToVoidQuest` (`/Game/ThirdPerson/Blueprints/BP_ThirdPersonCharacter.bIsGreeceDone` _myplayercharacter_3) _asbp_game_instance_2)
      (set `/Game/BP_GameInstance.Saved_PetraToVoidQuest` (`/Game/ThirdPerson/Blueprints/BP_ThirdPersonCharacter.bIsPetraDone` _myplayercharacter_3) _asbp_game_instance_2)
      (`GameplayStatics.OpenLevelBySoftObjectPtr` _level))))

(fn `UserConstructionScript`)