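; Dialogue NPC Blueprint for Abu, a local guide who tells the player about Petra's history and sights.
; Talk opens WB_Dialogue with options matching DialogueStage, or free-text input from stage 3.
; PlayerInput string-matches scripted questions to set replies, stage and next options.
; "Ask me anything..." sets UseAIDialogue, passing unmatched input to the parent's handler; stage 3 re-entry does not set this flag.
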(event `self.ReceiveBeginPlay`
  (`parent.ReceiveBeginPlay`))

(event `self.ReceivePlayerInput`
  (params (InputText :type String))
  (bind _ui (`self.UI`))
  (bind _ui_2 (`self.UI`))
  (bind _ui_3 (`self.UI`))
  (`/Game/Dialogue/WB_Dialogue.AddChatLine` _ui_3 (`KismetTextLibrary.Conv_StringToText` InputText) true)
  (if (`KismetStringLibrary.EqualEqual_StrStr` InputText "What is Petra?")
    (`/Game/Dialogue/WB_Dialogue.AddChatLine` _ui_3 "Petra was the capital of the Nabataean Kingdom, carved directly into rose-red sandstone cliffs. It controlled the trade routes between Arabia and the Mediterranean for centuries. At its peak, over 30,000 people lived here." false)
    (set `self.DialogueStage` 1)
    (`/Game/Dialogue/WB_Dialogue.SetDialogueOptions` _ui "Tell me about the water systems" "What about the carved tombs?" "Ask me anything...")
    (elif (`KismetStringLibrary.EqualEqual_StrStr` "Who lives here?" InputText)
      (`/Game/Dialogue/WB_Dialogue.AddChatLine` _ui_2 "The Nabataeans — an ancient Arab people. They were not just traders but brilliant engineers. They carved channels into the rock to capture every drop of rain. In a desert where water means life, they became the wealthiest people in the region." false)
      (set `self.DialogueStage` 1)
      (`/Game/Dialogue/WB_Dialogue.SetDialogueOptions` _ui "Tell me about the water systems" "What about the carved tombs?" "Ask me anything...")
      (elif (`KismetStringLibrary.EqualEqual_StrStr` InputText "What should I do first?")
        (`/Game/Dialogue/WB_Dialogue.AddChatLine` _ui_2 "Start at the bazaar - find a merchant named Amina near the entrance, she knows everyone. Then seek out Obodas, he is the keeper of trade knowledge. And be careful near the Treasury... the guard Khalil does not let strangers pass easily." false)
        (set `self.DialogueStage` 1)
        (`/Game/Dialogue/WB_Dialogue.SetDialogueOptions` _ui "Tell me about the water systems" "What about the carved tombs?" "Ask me anything...")
        (elif (`KismetStringLibrary.EqualEqual_StrStr` InputText "Tell me about the water systems")
          (`/Game/Dialogue/WB_Dialogue.AddChatLine` (`self.UI`) "The Nabataeans built an incredible network of dams, cisterns, and channels carved into the rock. They could capture flash flood water and store it for months. That is their greatest secret — they turned the driest desert into a thriving city. Some of those cisterns are still hidden in the cliffs." false)
          (set `self.DialogueStage` 2)
          (`/Game/Dialogue/WB_Dialogue.SetDialogueOptions` (`self.UI`) "How did the Nabataeans disappear?" "Any hidden places to explore?" "Ask me anything...")
          (elif (`KismetStringLibrary.EqualEqual_StrStr` InputText "What about the carved tombs?")
            (`/Game/Dialogue/WB_Dialogue.AddChatLine` (`self.UI`) "The facades you see carved into the cliffs are tombs of Nabataean kings and nobles. The most famous is Al-Khazneh, the Treasury. But do not be fooled by the name — it was never a treasury. It is a royal tomb, though many believe something precious is still hidden inside." false)
            (set `self.DialogueStage` 2)
            (`/Game/Dialogue/WB_Dialogue.SetDialogueOptions` (`self.UI`) "How did the Nabataeans disappear?" "Any hidden places to explore?" "Ask me anything...")
            (elif (`KismetStringLibrary.EqualEqual_StrStr` InputText "How did the Nabataeans disappear?")
              (`/Game/Dialogue/WB_Dialogue.AddChatLine` (`self.UI`) "They did not disappear suddenly. Rome annexed the kingdom in 106 AD. Over time, trade routes shifted to sea lanes, and Petra lost its purpose. Earthquakes damaged the water systems. The people drifted away. But their knowledge, their carvings, their engineering — that remains in every stone." false)
              (set `self.DialogueStage` 3)
              (`/Game/Dialogue/WB_Dialogue.SetDialogueOptions` (`self.UI`) "Any hidden places to explore?" "GoodBye..." "Ask me anything...")
              (elif (`KismetStringLibrary.EqualEqual_StrStr` InputText "Any hidden places to explore?")
                (`/Game/Dialogue/WB_Dialogue.AddChatLine` (`self.UI`) "Oh, many! There are hidden paths above the Treasury that lead to stunning views. The monastery Ad-Deir on the mountain top. Secret cisterns in narrow side canyons. And they say there are chambers beneath Al-Khazneh that no one has entered in centuries..." false)
                (set `self.DialogueStage` 3)
                (`/Game/Dialogue/WB_Dialogue.SetDialogueOptions` (`self.UI`) "How did the Nabataeans disappear?" "Any hidden places to explore?" "Ask me anything...")
                (elif (`KismetStringLibrary.EqualEqual_StrStr` InputText "Ask me anything...")
                  (set `self.Use AI Dialogue` true)
                  (`/Game/Dialogue/WB_Dialogue.AddChatLine` (`self.UI`) "Of course! Ask me whatever is on your mind. Type your question below." false)
                  (`/Game/Dialogue/WB_Dialogue.ShowCustomInput` (`self.UI`))
                  (elif (`self.Use AI Dialogue`)
                    (`parent.ReceivePlayerInput` InputText)
                    (`/Game/Dialogue/WB_Dialogue.ShowCustomInput` (`self.UI`))))))))))))

(event `/Game/Dialogue/BPI_Dialogue.Talk`
  (bind _returnvalue (`GameplayStatics.GetPlayerController` 0))
  (bind _returnvalue_2 (`GameplayStatics.GetPlayerController` 0))
  (bind _ui (`self.UI`))
  (bind _ui_2 (`self.UI`))
  ; Event Talk
  (if (`self.CanTalk?`)
    (set `self.CanTalk?` true)
    (if (>= (`self.DialogueStage`) 3)
      (bind _returnvalue_3 (`|CreateWidget` "/Game/Dialogue/WB_Dialogue.WB_Dialogue_C" _returnvalue_2 self))
      (bind _output_get (set `self.UI` _returnvalue_3))
      (`UserWidget.AddToViewport` _output_get 0)
      (`WidgetBlueprintLibrary.SetInputMode_GameAndUIEx` _returnvalue_2 null)
      (set `PlayerController.bShowMouseCursor` true _returnvalue_2)
      (`/Game/Dialogue/WB_Dialogue.AddChatLine` (`self.UI`) "What else would you like to know, friend? Ask me anything" false)
      (`/Game/Dialogue/WB_Dialogue.ShowCustomInput` _ui_2)
      (else
        (bind _returnvalue_4 (`|CreateWidget` "/Game/Dialogue/WB_Dialogue.WB_Dialogue_C" _returnvalue self))
        (bind _output_get_2 (set `self.UI` _returnvalue_4))
        (`UserWidget.AddToViewport` _output_get_2 0)
        (`WidgetBlueprintLibrary.SetInputMode_GameAndUIEx` _returnvalue null)
        (set `PlayerController.bShowMouseCursor` true _returnvalue)
        (switch `int` (`self.DialogueStage`)
          (:`0`
            (`/Game/Dialogue/WB_Dialogue.AddChatLine` _ui_2 "Ah, you must be the traveler! I am Abu, a local guide. I have lived in these canyons my whole life. Welcome to Petra!\"" false)
            (`/Game/Dialogue/WB_Dialogue.SetDialogueOptions` _ui "What is Petra?" "Who lives here?" "What should I do first?"))
          (:`1`
            (`/Game/Dialogue/WB_Dialogue.AddChatLine` _ui_2 "Good to see you again, friend! What would you like to know?" false)
            (`/Game/Dialogue/WB_Dialogue.SetDialogueOptions` _ui "Tell me about the water systems" "What about the carved tombs?" "Ask me anything..."))
          (:`2`
            (`/Game/Dialogue/WB_Dialogue.AddChatLine` _ui_2 "You are learning quickly! Anything else on your mind?" false)
            (`/Game/Dialogue/WB_Dialogue.SetDialogueOptions` _ui "How did the Nabataeans disappear?" "Any hidden places to explore?" "Ask me anything...")))))))

(fn `UserConstructionScript`
  (`parent.UserConstructionScript`))