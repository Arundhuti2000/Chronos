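; Khalil, the Al-Khazneh guard NPC, takes a honey cake bribe, gives a voiced history lesson, then quizzes the player.
; A DialogueStage counter drives WB_Dialogue options, with choices matched by text.
; Answers add or deduct KP, with game over possible, while typed hint requests go to an AI through BPHttpClientComponent at a KP cost.
; Progress updates quest objectives, and EndDialogue destroys TreasuryDoor actors once MainQuest02's bribe or quiz objective is complete.
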(event `self.OnAIResponseReceived_Event`
  (params (ResponseText :type String))
  (`self.AddToHistory` ResponseText "AI")
  (`/Game/Dialogue/WB_Dialogue.AddChatLine` (`self.UI`) (`KismetTextLibrary.Conv_StringToText` ResponseText) false)
  (if (`self.IsHintResponse`)
    (set `self.IsHintResponse` false)
    (bind _myplayercharacter (`/Game/ThirdPerson/CommonFunctionLibrary.GetMyPlayerCharacter`))
    (bind _bgameover (`/Game/ThirdPerson/Blueprints/BP_ThirdPersonCharacter.DeductKP` _myplayercharacter 5))
    (if _bgameover
      (bind _returnvalue (`|CreateWidget` "/Game/ThirdPerson/QuestSYstem/UI/WBP_GameOver.WBP_GameOver_C"))
      (`UserWidget.AddToViewport` _returnvalue 0)
      (else
        (`self.ShowCurrentDialogueStage`)))
    (else
      (`KismetSystemLibrary.Delay` 6.0)
      (`self.ShowCurrentDialogueStage`))))

(event `self.ReceiveBeginPlay`
  (`parent.ReceiveBeginPlay`)
  (add `/Game/Blueprints/BP_HttpClient_Component.OnAIResponseReceived` (`self.BP_HttpClient_Component`) (delegate `self.OnAIResponseReceived_Event`)))

(event `/Game/Dialogue/BPI_Dialogue.Talk`
  (bind _returnvalue (`GameplayStatics.GetPlayerController` 0))
  (bind _ui (`self.UI`))
  (bind _ui_2 (`self.UI`))
  (if (`self.CanTalk?`)
    (set `self.CanTalk?` false)
    (bind _returnvalue_2 (`|CreateWidget` "/Game/Dialogue/WB_Dialogue.WB_Dialogue_C" _returnvalue self))
    (bind _output_get (set `self.UI` _returnvalue_2))
    (`UserWidget.AddToViewport` _output_get 0)
    (set `PlayerController.bShowMouseCursor` true _returnvalue)
    (if (== (`self.DialogueStage`) 0)
      (`/Game/Dialogue/WB_Dialogue.AddChatLine` _ui_2 "Halt. You cannot pass. Al-Khazneh is sealed by order of King Aretas IV. None enter without purpose or permission." false)
      (bind _returnvalue_3 (`GameplayStatics.SpawnSound2D` "/Game/Audio/khalil/khalilHalt.khalilHalt" 1.0 1.0 0.0 null))
      (set `self.CurrentAudioComponent` _returnvalue_3)
      (`/Game/Dialogue/WB_Dialogue.SetDialogueOptions` _ui_2 "I have honey cakes for you" "What is this place?" "I will be on my way")
      (`/Game/Dialogue/WB_Dialogue.ShowOptionsPanel` _ui_2)
      (elif (== (`self.DialogueStage`) 1)
        (`/Game/Dialogue/WB_Dialogue.AddChatLine` _ui "Welcome back. Are you ready to try the quiz again?" false)
        (`/Game/Dialogue/WB_Dialogue.SetDialogueOptions` _ui "I am ready for the quiz" "What is this place?" "I will be on my way")
        (`/Game/Dialogue/WB_Dialogue.ShowOptionsPanel` _ui)))))

(event `self.ReceivePlayerInput`
  (params (InputText :type String))
  (bind _currentaudiocomponent (`self.CurrentAudioComponent`))
  (bind _ui (`self.UI`))
  (bind _ui_2 (`self.UI`))
  (bind _ui_3 (`self.UI`))
  (bind _ui_4 (`self.UI`))
  (bind _ui_5 (`self.UI`))
  (bind _bp_httpclient_component (`self.BP_HttpClient_Component`))
  (`/Engine/EditorBlueprintResources/StandardMacros.IsValid` _currentaudiocomponent
    (:`Is Valid`
      (`AudioComponent.Stop` _currentaudiocomponent))
    (:`Is Not Valid`
      _))
  (`/Game/Dialogue/WB_Dialogue.AddChatLine` _ui_3 (`KismetTextLibrary.Conv_StringToText` InputText) true)
  (if (`self.IsAwaitingHintInput`)
    (set `self.IsAwaitingHintInput` false)
    (`Widget.SetVisibility` (`/Game/Dialogue/WB_Dialogue.InputBox_Border` _ui_3) "Collapsed")
    (bind _full_prompt (`/Game/Blueprints/BP_HttpClient_Component.Build_Followup_Prompt` _bp_httpclient_component "khalil" (`KismetStringLibrary.Concat_StrStr` (`KismetStringLibrary.Concat_StrStr` "The player is asking for a hint during a quiz about: " (`self.CurrentQuizQuestion`)) InputText) ""))
    (`/Game/Blueprints/BP_HttpClient_Component.Send AI Request` _bp_httpclient_component _full_prompt "" "")
    (elif (`KismetStringLibrary.EqualEqual_StrStr` "What is this place?" InputText)
      (if (`self.HasCompletedTeaching`)
        (`/Game/Dialogue/WB_Dialogue.AddChatLine` _ui_2 "You have already heard my account, traveler. Move along." false)
        (else
          (`/Game/Dialogue/WB_Dialogue.AddChatLine` _ui_2 "This is Al-Khazneh — The Treasury. Though do not let the name fool you. No gold lies within these walls. It was carved as a royal tomb, a mausoleum fit for a king. The Bedouins named it 'The Treasury' from foolish legends about an urn near the top. They even shot at it with rifles hoping coins would fall. Solid stone, all of it." false)
          (bind _returnvalue (`GameplayStatics.SpawnSound2D` "/Game/Audio/khalil/khalilTreasyry.khalilTreasyry" 2.0 1.0 0.0 null))
          (set `self.CurrentAudioComponent` _returnvalue)
          (set `self.DialogueStage` 0)
          (`/Game/Dialogue/WB_Dialogue.SetDialogueOptions` _ui_5 "I have honey cakes for you" "What is this place?" "I will be on my way")
          (`/Game/Dialogue/WB_Dialogue.ShowOptionsPanel` _ui_5)))
      (elif (`KismetStringLibrary.EqualEqual_StrStr` "I will be on my way" InputText)
        (`/Game/Dialogue/WB_Dialogue.AddChatLine` (`self.UI`) "Safe Travels." false)
        (`self.EndDialogue`)
        (elif (`KismetStringLibrary.EqualEqual_StrStr` "I have honey cakes for you" InputText)
          (bind _myplayercharacter (`/Game/ThirdPerson/CommonFunctionLibrary.GetMyPlayerCharacter`))
          (bind _iscollected (`/Game/ThirdPerson/Inventory/BP_InventoryComponent.IsItemCollected` (`self.GetComponentByClass` _myplayercharacter "/Game/ThirdPerson/Inventory/BP_InventoryComponent.BP_InventoryComponent_C") "honeycake"))
          (if _iscollected
            (`/Game/Dialogue/WB_Dialogue.AddChatLine` (`self.UI`) "Hm. Fresh ones too. You have good taste. Very well — I am a fair man. But I do not open these doors for just anyone. Tell me — do you even know what you seek to enter?" false)
            (bind _returnvalue_2 (`GameplayStatics.SpawnSound2D` "/Game/Audio/khalil/khalilfreshones.khalilfreshones" 1.0 1.0 0.0 null))
            (set `self.CurrentAudioComponent` _returnvalue_2)
            (set `self.DialogueStage` 1)
            (for _array_element (`/Game/ThirdPerson/QuestSYstem/QuestLog_Component.CurrentQuests` (`self.GetComponentByClass` _myplayercharacter "/Game/ThirdPerson/QuestSYstem/QuestLog_Component.QuestLog_Component_C"))
              (`/Game/ThirdPerson/QuestSYstem/BP_QuestBase.UpdateObjectiveProgress` _array_element "obj_guard_bribe" 1))
            (`KismetSystemLibrary.Delay` 14.0)
            (`/Game/Dialogue/WB_Dialogue.AddChatLine` _ui "Al-Khazneh stands 39 metres tall, carved top-to-bottom from a single rose-red sandstone cliff. Builders were lowered on ropes the summit — they carved each level downward. No scaffolding from the ground. They worked from the sky." false)
            (bind _returnvalue_3 (`GameplayStatics.SpawnSound2D` "/Game/Audio/khalil/khalil39metre.khalil39metre" 1.0 1.0 0.0 null))
            (set `self.CurrentAudioComponent` _returnvalue_3)
            (`KismetSystemLibrary.Delay` 18.0)
            (`/Game/Dialogue/WB_Dialogue.AddChatLine` _ui "Every figure on the facade carries meaning. Isis stands at the centre of the upper level — goddess of the dead. Castor and Pollux flank the entrance below, the twin gods who guide souls to the afterlife. This is a tomb, not a treasury." false)
            (bind _returnvalue_4 (`GameplayStatics.SpawnSound2D` "/Game/Audio/khalil/khalilIsis.khalilIsis" 1.0 1.0 0.0 null))
            (set `self.CurrentAudioComponent` _returnvalue_4)
            (`KismetSystemLibrary.Delay` 19.0)
            (`/Game/Dialogue/WB_Dialogue.AddChatLine` _ui "Beneath this forecourt, archaeologists found three more Nabataean royal tombs buried underground. Petra keeps its secrets well. Now — let us see if you were paying attention." false)
            (bind _returnvalue_5 (`GameplayStatics.SpawnSound2D` "/Game/Audio/khalil/khalilquiz.khalilquiz" 1.0 1.0 0.0 null))
            (set `self.CurrentAudioComponent` _returnvalue_5)
            (set `self.HasCompletedTeaching` true)
            (`/Game/Dialogue/WB_Dialogue.SetDialogueOptions` _ui "I am ready for the quiz" "" "")
            (`Widget.SetVisibility` (`/Game/Dialogue/WB_Dialogue.BTN_Option2` _ui) "Hidden")
            (`Widget.SetVisibility` (`/Game/Dialogue/WB_Dialogue.BTN_Option3` _ui) "Hidden")
            (`/Game/Dialogue/WB_Dialogue.ShowOptionsPanel` _ui)
            (else
              (`/Game/Dialogue/WB_Dialogue.AddChatLine` (`self.UI`) "Show me first, then we talk." false)))
          (elif (`KismetStringLibrary.EqualEqual_StrStr` "I am ready for the quiz" InputText)
            (set `self.DialogueStage` 2)
            (`self.ShowCurrentDialogueStage`)
            (elif (`KismetStringLibrary.EqualEqual_StrStr` "Ask Khalil for a Hint" InputText)
              (`Widget.SetVisibility` (`/Game/Dialogue/WB_Dialogue.BTN_Option4` _ui_4) "Collapsed")
              (`Widget.SetVisibility` (`/Game/Dialogue/WB_Dialogue.InputBox_Border` _ui_4) "Visible")
              (set `self.IsAwaitingHintInput` true)
              (set `self.IsHintResponse` true)
              (elif (`KismetArrayLibrary.Array_Contains` (`self.QuizOptions`) InputText)
                (`self.HandleQuizAnswer` InputText)))))))))

(event `ShowCurrentDialogueStage`
  (bind _ui (`self.UI`))
  (bind _ui_2 (`self.UI`))
  (bind _ui_3 (`self.UI`))
  (bind _ui_4 (`self.UI`))
  (`Widget.SetVisibility` (`/Game/Dialogue/WB_Dialogue.BTN_Option2` _ui) "Visible")
  (`Widget.SetVisibility` (`/Game/Dialogue/WB_Dialogue.BTN_Option3` _ui) "Visible")
  (if (== (`self.DialogueStage`) 2)
    (`/Game/Dialogue/WB_Dialogue.AddChatLine` _ui_3 "First question. What was Al-Khazneh truly built for?" false)
    (set `self.CurrentQuizQuestion` "What was Al-Khazneh truly built for?")
    (`/Game/Dialogue/WB_Dialogue.SetDialogueOptions` _ui_3 "A treasury to store the King's gold" "A royal tomb for King Aretas IV" "Ask Khalil for a Hint")
    (`/Game/Dialogue/WB_Dialogue.ShowOptionsPanel` _ui_3)
    (elif (== (`self.DialogueStage`) 3)
      (`/Game/Dialogue/WB_Dialogue.AddChatLine` _ui_4 "Second. The goddess carved at the top of the facade — who is she?" false)
      (set `self.CurrentQuizQuestion` "The goddess carved at the top of the treasury facade — who is she?")
      (`/Game/Dialogue/WB_Dialogue.SetDialogueOptions` _ui_4 "Al-Uzza, the Nabataean goddess" "Ask Khalil for a Hint" "Isis, goddess of the dead")
      (`/Game/Dialogue/WB_Dialogue.ShowOptionsPanel` _ui_4)
      (elif (== (`self.DialogueStage`) 4)
        (`/Game/Dialogue/WB_Dialogue.AddChatLine` _ui_2 "Last question. How did the builders carve Al-Khazneh?" false)
        (set `self.CurrentQuizQuestion` "How did the builders carve Al-Khazneh? From top or bottom")
        (`/Game/Dialogue/WB_Dialogue.SetDialogueOptions` _ui_2 "From the ground up with scaffolding" "From the top down, lowered by ropes" "Ask Khalil for a Hint")
        (`/Game/Dialogue/WB_Dialogue.ShowOptionsPanel` _ui_2)
        (elif (== (`self.DialogueStage`) 5)
          (`/Game/Dialogue/WB_Dialogue.AddChatLine` _ui_2 "You know this place better than most who live beside it.Enter — but disturb nothing. The dead deserve their peace." false)
          (bind _returnvalue (`GameplayStatics.SpawnSound2D` "/Game/Audio/khalil/khalil39metre.khalil39metre" 1.0 1.0 0.0 null))
          (set `self.CurrentAudioComponent` _returnvalue)
          (`KismetSystemLibrary.Delay` 7.0)
          (`self.EndDialogue`))))))

(event `self.EndDialogue`
  (`parent.EndDialogue`)
  (bind _myplayercharacter (`/Game/ThirdPerson/CommonFunctionLibrary.GetMyPlayerCharacter`))
  (`/Engine/EditorBlueprintResources/StandardMacros.IsValid` _myplayercharacter
    (:`Is Valid`
      (bind _questlog_component (`/Game/ThirdPerson/Blueprints/BP_ThirdPersonCharacter.QuestLog_Component` _myplayercharacter))
      (`/Engine/EditorBlueprintResources/StandardMacros.IsValid` _questlog_component
        (:`Is Valid`
          (for _array_element (`/Game/ThirdPerson/QuestSYstem/QuestLog_Component.CurrentQuests` _questlog_component)
            (`/Engine/EditorBlueprintResources/StandardMacros.IsValid` _array_element
              (:`Is Valid`
                (`/Game/ThirdPerson/QuestSYstem/BP_QuestBase.UpdateObjectiveProgress` _array_element "obj_confront_guard" 1)
                (bind _myplayercharacter_2 (`/Game/ThirdPerson/CommonFunctionLibrary.GetMyPlayerCharacter`))
                (`/Engine/EditorBlueprintResources/StandardMacros.IsValid` _myplayercharacter_2
                  (:`Is Valid`
                    (bind _questlog_component_2 (`/Game/ThirdPerson/Blueprints/BP_ThirdPersonCharacter.QuestLog_Component` _myplayercharacter_2))
                    (`/Engine/EditorBlueprintResources/StandardMacros.IsValid` _questlog_component_2
                      (:`Is Valid`
                        (for _array_element_2 (`/Game/ThirdPerson/QuestSYstem/QuestLog_Component.CurrentQuests` _questlog_component_2)
                          (bind _iscomplete (`/Game/ThirdPerson/QuestSYstem/BP_QuestBase.IsObjectiveComplete` _array_element_2 "obj_guard_bribe"))
                          (bind _iscomplete_2 (`/Game/ThirdPerson/QuestSYstem/BP_QuestBase.IsObjectiveComplete` _array_element_2 "obj_complete_quiz"))
                          (if (or _iscomplete _iscomplete_2)
                            (if (== (`/Game/ThirdPerson/QuestSYstem/BP_QuestBase.QuestID` _array_element_2) "MainQuest02")
                              (bind _outactors (`GameplayStatics.GetAllActorsWithTag` "TreasuryDoor"))
                              (for _array_element_3 _outactors
                                (`self.K2_DestroyActor` _array_element_3)))))))))))))))))

(fn `CompleteSpecificObjective`
  (params (ObjectiveID :type String))
  (bind _myplayercharacter (`/Game/ThirdPerson/CommonFunctionLibrary.GetMyPlayerCharacter`))
  (for _array_element (`/Game/ThirdPerson/QuestSYstem/QuestLog_Component.CurrentQuests` (`self.GetComponentByClass` _myplayercharacter "/Game/ThirdPerson/QuestSYstem/QuestLog_Component.QuestLog_Component_C"))
    (`/Game/ThirdPerson/QuestSYstem/BP_QuestBase.UpdateObjectiveProgress` _array_element ObjectiveID 1)))

(fn `HandleQuizAnswer`
  (params (AnswerText :type String))
  (bind _ui (`self.UI`))
  (bind _ui_2 (`self.UI`))
  (if (== (`self.DialogueStage`) 2)
    (if (`KismetStringLibrary.EqualEqual_StrStr` AnswerText "A royal tomb for King Aretas IV")
      (bind _myplayercharacter (`/Game/ThirdPerson/CommonFunctionLibrary.GetMyPlayerCharacter`))
      (`/Game/ThirdPerson/Blueprints/BP_ThirdPersonCharacter.AddKP` _myplayercharacter 10)
      (`/Game/Dialogue/WB_Dialogue.AddChatLine` _ui_2 "Correct. A mausoleum, not a treasury. The Bedouin legend of coins in that urn solid stone." false)
      (set `self.DialogueStage` (+ (`self.DialogueStage`) 1))
      (`self.ShowCurrentDialogueStage`)
      (elif (`KismetStringLibrary.EqualEqual_StrStr` AnswerText "A treasury to store the King's gold")
        (bind _myplayercharacter_2 (`/Game/ThirdPerson/CommonFunctionLibrary.GetMyPlayerCharacter`))
        (`/Game/ThirdPerson/Blueprints/BP_ThirdPersonCharacter.DeductKP` _myplayercharacter_2 10 :!label _label)
        (bind _bgameover (`/Game/ThirdPerson/Blueprints/BP_ThirdPersonCharacter.DeductKP` (stale _myplayercharacter_3) 10))
        (if _bgameover
          (bind _returnvalue (`|CreateWidget` "/Game/ThirdPerson/QuestSYstem/UI/WBP_GameOver.WBP_GameOver_C"))
          (`UserWidget.AddToViewport` _returnvalue 0)
          (else
            (`/Game/Dialogue/WB_Dialogue.AddChatLine` _ui_2 "Wrong. No gold was ever found inside. Three empty chambers, nothing more." false)
            (`self.ShowCurrentDialogueStage`)))
        (elif (`KismetStringLibrary.EqualEqual_StrStr` AnswerText "A temple to the god Dushara")
          (bind _myplayercharacter_3 (`/Game/ThirdPerson/CommonFunctionLibrary.GetMyPlayerCharacter`))
          (goto _label))))
    (elif (== (`self.DialogueStage`) 3)
      (if (`KismetStringLibrary.EqualEqual_StrStr` AnswerText "Isis, goddess of the dead")
        (bind _myplayercharacter_4 (`/Game/ThirdPerson/CommonFunctionLibrary.GetMyPlayerCharacter`))
        (`/Game/ThirdPerson/Blueprints/BP_ThirdPersonCharacter.AddKP` _myplayercharacter_4 10)
        (`/Game/Dialogue/WB_Dialogue.AddChatLine` _ui "Yes. The Nabataeans adopted the cult of Isis from Egypt. The basileion crown marks her on the pediment." false)
        (set `self.DialogueStage` (+ (`self.DialogueStage`) 1))
        (`self.ShowCurrentDialogueStage`)
        (elif (`KismetStringLibrary.EqualEqual_StrStr` AnswerText "Tyche, goddess of fortune")
          (bind _myplayercharacter_5 (`/Game/ThirdPerson/CommonFunctionLibrary.GetMyPlayerCharacter`))
          (`/Game/ThirdPerson/Blueprints/BP_ThirdPersonCharacter.DeductKP` _myplayercharacter_5 10 :!label _label_2)
          (bind _bgameover_2 (`/Game/ThirdPerson/Blueprints/BP_ThirdPersonCharacter.DeductKP` (stale _myplayercharacter_6) 10))
          (if _bgameover_2
            (bind _returnvalue_2 (`|CreateWidget` "/Game/ThirdPerson/QuestSYstem/UI/WBP_GameOver.WBP_GameOver_C"))
            (`UserWidget.AddToViewport` _returnvalue_2 0)
            (else
              (`/Game/Dialogue/WB_Dialogue.AddChatLine` _ui "Not quite. The central figure bears the mark of Isis — look for the basileion crown next time." false)
              (`self.ShowCurrentDialogueStage`)))
          (elif (`KismetStringLibrary.EqualEqual_StrStr` AnswerText "Al-Uzza, the Nabataean goddess")
            (bind _myplayercharacter_6 (`/Game/ThirdPerson/CommonFunctionLibrary.GetMyPlayerCharacter`))
            (goto _label_2))))
      (elif (== (`self.DialogueStage`) 4)
        (if (`KismetStringLibrary.EqualEqual_StrStr` AnswerText "From the top down, lowered by ropes")
          (bind _myplayercharacter_7 (`/Game/ThirdPerson/CommonFunctionLibrary.GetMyPlayerCharacter`))
          (`/Game/ThirdPerson/Blueprints/BP_ThirdPersonCharacter.AddKP` _myplayercharacter_7 10)
          (`/Game/Dialogue/WB_Dialogue.AddChatLine` (`self.UI`) "Exactly right. They carved a ledge at the summit and worked downward. Remarkable, is it not?" false)
          (`self.CompleteSpecificObjective` "obj_complete_quiz")
          (set `self.DialogueStage` (+ (`self.DialogueStage`) 1))
          (`self.ShowCurrentDialogueStage`)
          (elif (`KismetStringLibrary.EqualEqual_StrStr` AnswerText "From the ground up with scaffolding")
            (bind _myplayercharacter_8 (`/Game/ThirdPerson/CommonFunctionLibrary.GetMyPlayerCharacter`))
            (`/Game/ThirdPerson/Blueprints/BP_ThirdPersonCharacter.DeductKP` _myplayercharacter_8 10 :!label _label_3)
            (bind _bgameover_3 (`/Game/ThirdPerson/Blueprints/BP_ThirdPersonCharacter.DeductKP` (stale _myplayercharacter_9) 10))
            (if _bgameover_3
              (bind _returnvalue_3 (`|CreateWidget` "/Game/ThirdPerson/QuestSYstem/UI/WBP_GameOver.WBP_GameOver_C"))
              (`UserWidget.AddToViewport` _returnvalue_3 0)
              (else
                (`/Game/Dialogue/WB_Dialogue.AddChatLine` (`self.UI`) "Wrong. The Nabataeans began and descended level by level — no scaffolding from below." false)
                (`self.ShowCurrentDialogueStage`)))
            (elif (`KismetStringLibrary.EqualEqual_StrStr` AnswerText "They carved from inside outward")
              (bind _myplayercharacter_9 (`/Game/ThirdPerson/CommonFunctionLibrary.GetMyPlayerCharacter`))
              (goto _label_3))))))))

(fn `UserConstructionScript`
  (`parent.UserConstructionScript`))