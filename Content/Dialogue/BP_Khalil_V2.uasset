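; Khalil is the NPC guard of Al-Khazneh, who takes honey cakes as a bribe, then offers a three-question history quiz.
; A DialogueStage integer and option-text matching drive the WB_Dialogue chat and update quest objectives.
; HandleQuizAnswer adds or deducts KP and can open Game Over, but its ShowCurrentDialogueStage calls are unreachable.
; Hints come from an AI request through BPHttpClientComponent and cost KP when the response arrives.
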(event `self.ReceiveActorBeginOverlap`
  (params (OtherActor :type "Actor Object Reference")))

(event `ShowCurrentDialogueStage`
  (bind _ui (`self.UI`))
  (bind _ui_2 (`self.UI`))
  (bind _ui_3 (`self.UI`))
  (if (== (`self.DialogueStage`) 2)
    (`/Game/Dialogue/WB_Dialogue.AddChatLine` _ui "Correct. A mausoleum, not a treasury. The Bedouin legend of coins in that urn solid stone." false)
    (set `self.CurrentQuizQuestion` "What was Al-Khazneh truly built for?")
    (`/Game/Dialogue/WB_Dialogue.SetDialogueOptions` _ui "A royal tomb for King Aretas IV" "A treasury to store the King's gold" "Ask Khalil for a Hint")
    (`/Game/Dialogue/WB_Dialogue.ShowOptionsPanel` _ui)
    (elif (== (`self.DialogueStage`) 3)
      (`/Game/Dialogue/WB_Dialogue.AddChatLine` _ui_2 "Correct. A mausoleum, not a treasury. The Bedouin legend of coins in that urn solid stone." false)
      (set `self.CurrentQuizQuestion` "The goddess carved at the top of the treasury facade — who is she?")
      (`/Game/Dialogue/WB_Dialogue.SetDialogueOptions` _ui_2 "Isis, goddess of the dead" "Ask Khalil for a Hint" "Al-Uzza, the Nabataean goddess")
      (`/Game/Dialogue/WB_Dialogue.ShowOptionsPanel` _ui_2)
      (elif (== (`self.DialogueStage`) 4)
        (`/Game/Dialogue/WB_Dialogue.AddChatLine` _ui_3 "Correct. A mausoleum, not a treasury. The Bedouin legend of coins in that urn solid stone." false)
        (set `self.CurrentQuizQuestion` "How did the builders carve Al-Khazneh? From top or bottom")
        (`/Game/Dialogue/WB_Dialogue.SetDialogueOptions` _ui_3 "From the top down, lowered by ropes" "From the ground up with scaffolding" "Ask Khalil for a Hint")
        (`/Game/Dialogue/WB_Dialogue.ShowOptionsPanel` _ui_3)
        (elif (== (`self.DialogueStage`) 5)
          (`/Game/Dialogue/WB_Dialogue.AddChatLine` (`self.UI`) "Correct. A mausoleum, not a treasury. The Bedouin legend of coins in that urn solid stone." false)
          (bind _myplayercharacter (`/Game/ThirdPerson/CommonFunctionLibrary.GetMyPlayerCharacter`))
          (for _array_element (`/Game/ThirdPerson/QuestSYstem/QuestLog_Component.CurrentQuests` (`self.GetComponentByClass` _myplayercharacter "/Game/ThirdPerson/QuestSYstem/QuestLog_Component.QuestLog_Component_C"))
            (`/Game/ThirdPerson/QuestSYstem/BP_QuestBase.UpdateObjectiveProgress` _array_element "obj_inspect_artifact" 1))
          (`/Game/ThirdPerson/QuestSYstem/BP_QuestBase.AdvanceStage` _array_element)
          (`self.EndDialogue`))))))

(event `self.ReceivePlayerInput`
  (params (InputText :type String))
  (bind _bp_httpclient_component (`self.BP_HttpClient_Component`))
  (bind _ui (`self.UI`))
  (bind _ui_2 (`self.UI`))
  (`KismetSystemLibrary.PrintString` (`KismetStringLibrary.Concat_StrStr` (`KismetStringLibrary.Concat_StrStr` (`KismetStringLibrary.Concat_StrStr` "RPI CALLED: " InputText) " | Stage: ") (`KismetStringLibrary.Conv_IntToString` (`self.DialogueStage`))) true true (struct :`R` 1.0 :`G` 1.0 :`A` 1.0) 5.0)
  (if (`KismetStringLibrary.EqualEqual_StrStr` "What is this place?" InputText)
    (if (`self.HasCompletedTeaching`)
      (`/Game/Dialogue/WB_Dialogue.AddChatLine` (`self.UI`) "Correct. A mausoleum, not a treasury. The Bedouin legend of coins in that urn solid stone." false)
      (else
        (`/Game/Dialogue/WB_Dialogue.AddChatLine` (`self.UI`) "Correct. A mausoleum, not a treasury. The Bedouin legend of coins in that urn solid stone." false)
        (set `self.DialogueStage` 0)
        (`/Game/Dialogue/WB_Dialogue.SetDialogueOptions` _ui "I have honey cakes for you" "What is this place?" "I will be on my way")
        (`/Game/Dialogue/WB_Dialogue.ShowOptionsPanel` _ui)))
    (elif (`KismetStringLibrary.EqualEqual_StrStr` "I will be on my way" InputText)
      (`/Game/Dialogue/WB_Dialogue.AddChatLine` (`self.UI`) "Correct. A mausoleum, not a treasury. The Bedouin legend of coins in that urn solid stone." false)
      (`self.EndDialogue`)
      (elif (`KismetStringLibrary.EqualEqual_StrStr` "I have honey cakes for you" InputText)
        (bind _myplayercharacter (`/Game/ThirdPerson/CommonFunctionLibrary.GetMyPlayerCharacter`))
        (`KismetSystemLibrary.PrintString` "HONEY CAKE BRANCH ENTERED" true true (struct :`G` 1.0 :`A` 1.0) 5.0)
        (bind _iscollected (`/Game/ThirdPerson/Inventory/BP_InventoryComponent.IsItemCollected` (`self.GetComponentByClass` _myplayercharacter "/Game/ThirdPerson/Inventory/BP_InventoryComponent.BP_InventoryComponent_C") "honeycake"))
        (if _iscollected
          (`KismetSystemLibrary.PrintString` "ITEM COLLECTED = TRUE" true true (struct :`G` 0.5 :`B` 1.0 :`A` 1.0) 5.0)
          (`/Game/Dialogue/WB_Dialogue.AddChatLine` (`self.UI`) "Correct. A mausoleum, not a treasury. The Bedouin legend of coins in that urn solid stone." false)
          (set `self.DialogueStage` 1)
          (bind _myplayercharacter_2 (`/Game/ThirdPerson/CommonFunctionLibrary.GetMyPlayerCharacter`))
          (for _array_element (`/Game/ThirdPerson/QuestSYstem/QuestLog_Component.CurrentQuests` (`self.GetComponentByClass` _myplayercharacter_2 "/Game/ThirdPerson/QuestSYstem/QuestLog_Component.QuestLog_Component_C"))
            (`/Game/ThirdPerson/QuestSYstem/BP_QuestBase.UpdateObjectiveProgress` _array_element "obj_guard_bribe" 1))
          (`/Game/Dialogue/WB_Dialogue.AddChatLine` _ui_2 "Correct. A mausoleum, not a treasury. The Bedouin legend of coins in that urn solid stone." false)
          (`/Game/Dialogue/WB_Dialogue.AddChatLine` _ui_2 "Correct. A mausoleum, not a treasury. The Bedouin legend of coins in that urn solid stone." false)
          (`/Game/Dialogue/WB_Dialogue.AddChatLine` _ui_2 "Correct. A mausoleum, not a treasury. The Bedouin legend of coins in that urn solid stone." false)
          (`KismetSystemLibrary.Delay` 0.5)
          (set `self.HasCompletedTeaching` true)
          (`/Game/Dialogue/WB_Dialogue.SetDialogueOptions` _ui_2 "I am ready for the quiz" "" "")
          (`/Game/Dialogue/WB_Dialogue.ShowOptionsPanel` _ui_2)
          (else
            (`KismetSystemLibrary.PrintString` "ITEM COLLECTED = FALSE" true true (struct :`R` 1.0 :`A` 1.0) 5.0)
            (`/Game/Dialogue/WB_Dialogue.AddChatLine` (`self.UI`) "Correct. A mausoleum, not a treasury. The Bedouin legend of coins in that urn solid stone." false)))
        (elif (`KismetStringLibrary.EqualEqual_StrStr` "I am ready for the quiz" InputText)
          (set `self.DialogueStage` 2)
          (`self.ShowCurrentDialogueStage`)
          (elif (`KismetStringLibrary.EqualEqual_StrStr` "Ask Khalil for a Hint" InputText)
            (set `self.IsAwaitingHintInput` true)
            (set `self.IsHintResponse` true)
            (bind _full_prompt (`/Game/Blueprints/BP_HttpClient_Component.Build_Followup_Prompt` _bp_httpclient_component "khalil" (`KismetStringLibrary.Concat_StrStr` (`KismetStringLibrary.Concat_StrStr` "The player is asking for a hint during a quiz about: " (`self.CurrentQuizQuestion`)) InputText) ""))
            (`/Game/Blueprints/BP_HttpClient_Component.Send AI Request` _bp_httpclient_component _full_prompt "" "")
            (else
              (`KismetSystemLibrary.PrintString` (`KismetStringLibrary.Concat_StrStr` "FALLBACK TO HANDLEQUIZANSWER: " InputText) true true (struct :`R` 1.0 :`B` 1.0 :`A` 1.0) 5.0)
              (`self.HandleQuizAnswer` InputText))))))))

(event `/Game/Dialogue/BPI_Dialogue.Talk`
  (bind _returnvalue (`GameplayStatics.GetPlayerController` 0))
  (bind _dialoguestage (`self.DialogueStage`))
  (if (`self.CanTalk?`)
    (set `self.CanTalk?` false)
    (bind _returnvalue_2 (`|CreateWidget` "/Game/Dialogue/WB_Dialogue.WB_Dialogue_C" _returnvalue self))
    (bind _output_get (set `self.UI` _returnvalue_2))
    (`UserWidget.AddToViewport` _output_get 0)
    (set `PlayerController.bShowMouseCursor` true _returnvalue)
    (if (== _dialoguestage 0)
      (`/Game/Dialogue/WB_Dialogue.AddChatLine` _output_get (`KismetTextLibrary.Conv_StringToText` "Halt. You cannot pass. Al-Khazneh is sealed by order of King Aretas IV. None enter without purpose or permission.") false)
      (`/Game/Dialogue/WB_Dialogue.SetDialogueOptions` _output_get "I have honey cakes for you" "What is this place?" "I will be on my way")
      (`/Game/Dialogue/WB_Dialogue.ShowOptionsPanel` _output_get)
      (elif (== _dialoguestage 1)
        (`/Game/Dialogue/WB_Dialogue.AddChatLine` _output_get (`KismetTextLibrary.Conv_StringToText` "Welcome back. Are you ready to try the quiz again?") false)
        (`/Game/Dialogue/WB_Dialogue.SetDialogueOptions` _output_get "I am ready for the quiz" "What is this place?" "I will be on my way")
        (`/Game/Dialogue/WB_Dialogue.ShowOptionsPanel` _output_get)))))

(event `self.ReceiveBeginPlay`
  (bind _bp_httpclient_component (`self.BP_HttpClient_Component`))
  (`parent.ReceiveBeginPlay`)
  (`/Engine/EditorBlueprintResources/StandardMacros.IsValid` _bp_httpclient_component
    (:`Is Valid`
      (add `/Game/Blueprints/BP_HttpClient_Component.OnAIResponseReceived` _bp_httpclient_component (delegate `self.OnAIResponseReceived_Event`)))
    (:`Is Not Valid`
      (`KismetSystemLibrary.PrintString` "HTTP Client component not found on NPC" true true (struct :`R` 1.0 :`A` 1.0)))))

(event `self.OnAIResponseReceived_Event`
  (params (ResponseText :type String))
  (`self.AddToHistory` ResponseText "AI")
  (`/Game/Dialogue/WB_Dialogue.AddChatLine` (`self.UI`) (`KismetTextLibrary.Conv_StringToText` ResponseText) false)
  (if (`self.IsHintResponse`)
    (set `self.IsHintResponse` false)
    (bind _myplayercharacter (`/Game/ThirdPerson/CommonFunctionLibrary.GetMyPlayerCharacter`))
    (`/Game/ThirdPerson/Blueprints/BP_ThirdPersonCharacter.DeductKP` _myplayercharacter 5)))

(event `self.EndDialogue`
  (`parent.EndDialogue`)
  (bind _myplayercharacter (`/Game/ThirdPerson/CommonFunctionLibrary.GetMyPlayerCharacter`))
  (`/Engine/EditorBlueprintResources/StandardMacros.IsValid` _myplayercharacter
    (:`Is Valid`
      (bind _questlog_component (`/Game/ThirdPerson/Blueprints/BP_ThirdPersonCharacter.QuestLog_Component` _myplayercharacter))
      (`/Engine/EditorBlueprintResources/StandardMacros.IsValid` _questlog_component
        (:`Is Valid`
          (for _array_element (`/Game/ThirdPerson/QuestSYstem/QuestLog_Component.CurrentQuests` _questlog_component)
            (`/Engine/EditorBlueprintResources/StandardMacros.IsValid` _array_element
              (:`Is Valid`
                (`/Game/ThirdPerson/QuestSYstem/BP_QuestBase.UpdateObjectiveProgress` _array_element "obj_confront_guard" 1)
                (bind _myplayercharacter_2 (`/Game/ThirdPerson/CommonFunctionLibrary.GetMyPlayerCharacter`))
                (`/Engine/EditorBlueprintResources/StandardMacros.IsValid` _myplayercharacter_2
                  (:`Is Valid`
                    (bind _questlog_component_2 (`/Game/ThirdPerson/Blueprints/BP_ThirdPersonCharacter.QuestLog_Component` _myplayercharacter_2))
                    (`/Engine/EditorBlueprintResources/StandardMacros.IsValid` _questlog_component_2
                      (:`Is Valid`
                        (for _array_element_2 (`/Game/ThirdPerson/QuestSYstem/QuestLog_Component.CurrentQuests` _questlog_component_2)
                          (bind _iscomplete (`/Game/ThirdPerson/QuestSYstem/BP_QuestBase.IsObjectiveComplete` _array_element_2 "obj_guard_bribe"))
                          (bind _iscomplete_2 (`/Game/ThirdPerson/QuestSYstem/BP_QuestBase.IsObjectiveComplete` _array_element_2 "obj_guard_persuade"))
                          (if (or _iscomplete _iscomplete_2)
                            (`/Game/ThirdPerson/QuestSYstem/BP_QuestBase.AdvanceStage` _array_element_2)))))))))))))))

(event `self.ReceiveTick`
  (params (DeltaSeconds :type "Float (single-precision)")))

(fn `HandleQuizAnswer`
  (params (AnswerText :type String))
  (bind _ui (`self.UI`))
  (bind _ui_2 (`self.UI`))
  (bind _ui_3 (`self.UI`))
  (if (== (`self.DialogueStage`) 2)
    (if (`KismetStringLibrary.EqualEqual_StrStr` AnswerText "A royal tomb for King Aretas IV")
      (bind _myplayercharacter (`/Game/ThirdPerson/CommonFunctionLibrary.GetMyPlayerCharacter`))
      (`/Game/ThirdPerson/Blueprints/BP_ThirdPersonCharacter.AddKP` _myplayercharacter 10)
      (`/Game/Dialogue/WB_Dialogue.AddChatLine` _ui_3 "Correct. A mausoleum, not a treasury. The Bedouin legend of coins in that urn solid stone." false)
      (set `self.DialogueStage` (+ (`self.DialogueStage`) 1))
      (elif (`KismetStringLibrary.EqualEqual_StrStr` AnswerText "A treasury to store the King's gold")
        (bind _myplayercharacter_2 (`/Game/ThirdPerson/CommonFunctionLibrary.GetMyPlayerCharacter`))
        (bind _bgameover (`/Game/ThirdPerson/Blueprints/BP_ThirdPersonCharacter.DeductKP` _myplayercharacter_2 10 :!label _label))
        (if _bgameover
          (bind _returnvalue (`|CreateWidget` "/Game/ThirdPerson/QuestSYstem/UI/WBP_GameOver.WBP_GameOver_C"))
          (`UserWidget.AddToViewport` _returnvalue 0)
          (`/Game/Dialogue/WB_Dialogue.AddChatLine` _ui_3 "Wrong. No gold was ever found inside. Three empty chambers, nothing more." false)
          (set `self.DialogueStage` (+ (`self.DialogueStage`) 1)))
        (elif (`KismetStringLibrary.EqualEqual_StrStr` AnswerText "A temple to the god Dushara")
          (goto _label))))
    (elif (== (`self.DialogueStage`) 3)
      (if (`KismetStringLibrary.EqualEqual_StrStr` AnswerText "Isis, goddess of the dead")
        (bind _myplayercharacter_3 (`/Game/ThirdPerson/CommonFunctionLibrary.GetMyPlayerCharacter`))
        (`/Game/ThirdPerson/Blueprints/BP_ThirdPersonCharacter.AddKP` _myplayercharacter_3 10)
        (`/Game/Dialogue/WB_Dialogue.AddChatLine` _ui_2 "Yes. The Nabataeans adopted the cult of Isis from Egypt. The basileion crown marks her on the pediment." false)
        (set `self.DialogueStage` (+ (`self.DialogueStage`) 1))
        (elif (`KismetStringLibrary.EqualEqual_StrStr` AnswerText "Tyche, goddess of fortune")
          (bind _bgameover_2 (`/Game/ThirdPerson/Blueprints/BP_ThirdPersonCharacter.DeductKP` _myplayercharacter_2 10 :!label _label_2))
          (if _bgameover_2
            (bind _returnvalue_2 (`|CreateWidget` "/Game/ThirdPerson/QuestSYstem/UI/WBP_GameOver.WBP_GameOver_C"))
            (`UserWidget.AddToViewport` _returnvalue_2 0)
            (`/Game/Dialogue/WB_Dialogue.AddChatLine` _ui_2 "Not quite. The central figure bears the mark of Isis — look for the basileion crown next time." false)
            (set `self.DialogueStage` (+ (`self.DialogueStage`) 1)))
          (elif (`KismetStringLibrary.EqualEqual_StrStr` AnswerText "Al-Uzza, the Nabataean goddess")
            (goto _label_2))))
      (elif (== (`self.DialogueStage`) 4)
        (if (`KismetStringLibrary.EqualEqual_StrStr` "" "From the top down, lowered by ropes")
          (bind _myplayercharacter_4 (`/Game/ThirdPerson/CommonFunctionLibrary.GetMyPlayerCharacter`))
          (`/Game/ThirdPerson/Blueprints/BP_ThirdPersonCharacter.AddKP` _myplayercharacter_4 10)
          (`/Game/Dialogue/WB_Dialogue.AddChatLine` _ui "Exactly right. They carved a ledge at the summit and worked downward. Remarkable, is it not?" false)
          (set `self.DialogueStage` (+ (`self.DialogueStage`) 1))
          (elif (`KismetStringLibrary.EqualEqual_StrStr` "" "From the ground up with scaffolding")
            (bind _bgameover_3 (`/Game/ThirdPerson/Blueprints/BP_ThirdPersonCharacter.DeductKP` _myplayercharacter_2 10 :!label _label_3))
            (if _bgameover_3
              (bind _returnvalue_3 (`|CreateWidget` "/Game/ThirdPerson/QuestSYstem/UI/WBP_GameOver.WBP_GameOver_C"))
              (`UserWidget.AddToViewport` _returnvalue_3 0)
              (`/Game/Dialogue/WB_Dialogue.AddChatLine` _ui "Wrong. The Nabataeans began and descended level by level — no scaffolding from below." false)
              (set `self.DialogueStage` (+ (`self.DialogueStage`) 1)))
            (elif (`KismetStringLibrary.EqualEqual_StrStr` "" "They carved from inside outward")
              (goto _label_3))))))))

(fn `UserConstructionScript`
  (`parent.UserConstructionScript`))