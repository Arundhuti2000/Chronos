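; Amina is a merchant NPC who introduces the player to Petra through voiced, option-based dialogue and advances intro quest objectives.
; Talk opens a WB_Dialogue widget linked to her and picks a greeting from DialogueStage, guarded by CanTalk.
; PlayerInput matches option text in a hardcoded branch chain to set replies, sounds, next options and stage.
; CompleteSpecificObjective pushes progress to every current quest in the player's QuestLog_Component.
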(event `self.ReceiveBeginPlay`
  (`parent.ReceiveBeginPlay`))

(event `self.ReceivePlayerInput`
  (params (InputText :type String))
  (bind _ui (`self.UI`))
  (`/Game/Dialogue/WB_Dialogue.AddChatLine` _ui (`KismetTextLibrary.Conv_StringToText` InputText) true)
  (if (`KismetStringLibrary.EqualEqual_StrStr` InputText "What is this place?")
    (`/Game/Dialogue/WB_Dialogue.AddChatLine` _ui (`KismetTextLibrary.Conv_StringToText` "This is Petra — carved into the rose-red cliffs by the Nabataeans over two thousand years ago. It sits at the crossroads of ancient trade routes connecting Arabia, Egypt, and the Mediterranean. Caravans carrying incense, spices, silk, and precious stones all pass through here.") false)
    (`GameplayStatics.PlaySound2D` "/Game/Audio/Amina/this_is_petra_amina.this_is_petra_amina" 1.0 1.0 0.0 null null)
    (`self.CompleteSpecificObjective` "obj_intro_learn_petra")
    (set `self.DialogueStage` 1)
    (`/Game/Dialogue/WB_Dialogue.SetDialogueOptions` _ui "Tell me about the trade routes" "What dangers should I watch for?" "I think I'm ready to explore")
    (`/Game/Dialogue/WB_Dialogue.ShowOptionsPanel` _ui)
    (elif (`KismetStringLibrary.EqualEqual_StrStr` InputText "Who are the Nabataeans?")
      (`/Game/Dialogue/WB_Dialogue.AddChatLine` _ui (`KismetTextLibrary.Conv_StringToText` "The Nabataeans were master traders and engineers. They controlled the water in this desert — hidden cisterns, secret channels carved into rock. That is how they built their wealth. They turned this barren canyon into the richest city on the trade routes.") false)
      (`GameplayStatics.PlaySound2D` "/Game/Audio/Amina/Who_are_Nabateans.Who_are_Nabateans" 1.0 1.0 0.0 null null)
      (`self.CompleteSpecificObjective` "obj_intro_learn_petra")
      (set `self.DialogueStage` 1)
      (`/Game/Dialogue/WB_Dialogue.SetDialogueOptions` _ui "Tell me about the trade routes" "What dangers should I watch for?" "I think I'm ready to explore")
      (`/Game/Dialogue/WB_Dialogue.ShowOptionsPanel` _ui)
      (elif (`KismetStringLibrary.EqualEqual_StrStr` InputText "What can I do here?")
        (`/Game/Dialogue/WB_Dialogue.AddChatLine` _ui (`KismetTextLibrary.Conv_StringToText` "There is much to discover! The merchant Obodas in the bazaar knows everything about the incense trade. The Treasury of Al-Khazneh holds ancient secrets, but a guard blocks the entrance. And if you need a guide, old Abu near the entrance knows every path in these canyons.") false)
        (`GameplayStatics.PlaySound2D` "/Game/Audio/Amina/What_to_explore.What_to_explore" 1.0 1.0 0.0 null null)
        (`self.CompleteSpecificObjective` "obj_intro_learn_petra")
        (set `self.DialogueStage` 1)
        (`/Game/Dialogue/WB_Dialogue.SetDialogueOptions` _ui "Tell me about the trade routes" "What dangers should I watch for?" "I think I'm ready to explore")
        (`/Game/Dialogue/WB_Dialogue.ShowOptionsPanel` _ui)
        (elif (`KismetStringLibrary.EqualEqual_StrStr` InputText "Tell me about the trade routes")
          (`/Game/Dialogue/WB_Dialogue.AddChatLine` _ui (`KismetTextLibrary.Conv_StringToText` "Caravans travel from the heart of Arabia through Petra to the ports of Gaza on the Mediterranean. Frankincense and myrrh from Yemen, silk from the East, spices from India — they all flow through this city. The Nabataeans charge tolls and offer safe passage. That is how Petra grew wealthy beyond imagination.") false)
          (`GameplayStatics.PlaySound2D` "/Game/Audio/Amina/caravans_travel.caravans_travel" 1.0 1.0 0.0 null null)
          (`self.CompleteSpecificObjective` "obj_intro_learn_trade")
          (`/Game/Dialogue/WB_Dialogue.SetDialogueOptions` _ui "What dangers should I watch for?" "I think I'm ready to explore" "Tell me more about the goods")
          (`/Game/Dialogue/WB_Dialogue.ShowOptionsPanel` _ui)
          (elif (`KismetStringLibrary.EqualEqual_StrStr` InputText "What dangers should I watch for?")
            (`/Game/Dialogue/WB_Dialogue.AddChatLine` _ui (`KismetTextLibrary.Conv_StringToText` "The desert is unforgiving, traveler. Bandits prey on lone travelers, and sandstorms can swallow a caravan whole. But inside Petra, the greatest danger is ignorance. Speak to the locals, learn the customs, and you will be safe. The people here respect knowledge and courtesy.") false)
            (`GameplayStatics.PlaySound2D` "/Game/Audio/Amina/dangers_of_desert.dangers_of_desert" 1.0 1.0 0.0 null null)
            (`self.CompleteSpecificObjective` "obj_intro_learn_tasks")
            (`/Game/Dialogue/WB_Dialogue.SetDialogueOptions` _ui "Tell me about the trade routes" "I think I'm ready to explore" "Any advice for a newcomer?")
            (`/Game/Dialogue/WB_Dialogue.ShowOptionsPanel` _ui)
            (elif (`KismetStringLibrary.EqualEqual_StrStr` InputText "I think I'm ready to explore")
              (`/Game/Dialogue/WB_Dialogue.AddChatLine` _ui (`KismetTextLibrary.Conv_StringToText` "Then go with confidence, traveler! Speak to Obodas in the bazaar — he is the best place to start. And remember, in Petra, knowledge is the most valuable currency. May fortune smile upon you!") false)
              (`GameplayStatics.PlaySound2D` "/Game/Audio/Amina/explore_the_bazaar.explore_the_bazaar" 1.0 1.0 0.0 null null)
              (`self.CompleteSpecificObjective` "obj_intro_complete")
              (set `self.HasCompletedIntro` true)
              (set `self.DialogueStage` 2)
              (set `self.CanTalk?` true)
              (else
                (`/Game/Dialogue/WB_Dialogue.AddChatLine` _ui (`KismetTextLibrary.Conv_StringToText` "There is always more to learn! Explore the bazaar, talk to the locals. Every person here has a story to tell.") false)
                (`GameplayStatics.PlaySound2D` "/Game/Audio/Amina/explore_there_is_more.explore_there_is_more" 1.0 1.0 0.0 null null)
                (`/Game/Dialogue/WB_Dialogue.SetDialogueOptions` _ui "Tell me about the trade routes" "What dangers should I watch for?" "I think I'm ready to explore")
                (`/Game/Dialogue/WB_Dialogue.ShowOptionsPanel` _ui)))))))))

(event `/Game/Dialogue/BPI_Dialogue.Talk`
  (bind _returnvalue (`GameplayStatics.GetPlayerController` 0))
  (bind _dialoguestage (`self.DialogueStage`))
  (if (`self.CanTalk?`)
    (set `self.CanTalk?` false)
    (bind _returnvalue_2 (`|CreateWidget` "/Game/Dialogue/WB_Dialogue.WB_Dialogue_C" _returnvalue self))
    (bind _output_get (set `self.UI` _returnvalue_2))
    (`UserWidget.AddToViewport` _output_get 0)
    (`WidgetBlueprintLibrary.SetInputMode_GameAndUIEx` _returnvalue _output_get "DoNotLock" false)
    (set `PlayerController.bShowMouseCursor` true _returnvalue)
    (if (== _dialoguestage 0)
      (`/Game/Dialogue/WB_Dialogue.AddChatLine` _output_get (`KismetTextLibrary.Conv_StringToText` "Peace be upon you, traveler! Welcome to Petra, the Rose City of the Nabataeans. I am Amina, a merchant of spices and precious goods.") false)
      (`GameplayStatics.PlaySound2D` "/Game/Audio/Amina/amina_line1.amina_line1" 1.0 1.0 0.0 null null)
      (`/Game/Dialogue/WB_Dialogue.SetDialogueOptions` _output_get "What is this place?" "Who are the Nabataeans?" "What can I do here?")
      (`/Game/Dialogue/WB_Dialogue.ShowOptionsPanel` _output_get)
      (elif (== _dialoguestage 1)
        (`/Game/Dialogue/WB_Dialogue.AddChatLine` _output_get (`KismetTextLibrary.Conv_StringToText` "Welcome back, traveler! What else would you like to know?") false)
        (`GameplayStatics.PlaySound2D` "/Game/Audio/Amina/welcome_back_traveler.welcome_back_traveler" 1.0 1.0 0.0 null null)
        (`/Game/Dialogue/WB_Dialogue.SetDialogueOptions` _output_get "Tell me about the trade routes" "What dangers should I watch for?" "I think I'm ready to explore")
        (`/Game/Dialogue/WB_Dialogue.ShowOptionsPanel` _output_get)
        (elif (== _dialoguestage 2)
          (`/Game/Dialogue/WB_Dialogue.AddChatLine` _output_get (`KismetTextLibrary.Conv_StringToText` "Good to see you again! You seem well on your way. May the winds carry you safely.") false)
          (`GameplayStatics.PlaySound2D` "/Game/Audio/Amina/good_to_see_you.good_to_see_you" 1.0 1.0 0.0 null null)
          (set `self.CanTalk?` true))))))

(fn `CompleteQuestObjectives`
  (bind _myplayercharacter (`/Game/ThirdPerson/CommonFunctionLibrary.GetMyPlayerCharacter`))
  (for _array_element (`/Game/ThirdPerson/QuestSYstem/QuestLog_Component.CurrentQuests` (`self.GetComponentByClass` _myplayercharacter "/Game/ThirdPerson/QuestSYstem/QuestLog_Component.QuestLog_Component_C"))
    (for _array_element_2 (`self.ObjectivesToComplete`)
      (bind _iscomplete (`/Game/ThirdPerson/QuestSYstem/BP_QuestBase.IsObjectiveComplete` _array_element _array_element_2))
      (if (not _iscomplete)
        (`/Game/ThirdPerson/QuestSYstem/BP_QuestBase.UpdateObjectiveProgress` _array_element _array_element_2 1)
        (break)))))

(fn `CompleteSpecificObjective`
  (params (ObjectiveID :type String))
  (bind _myplayercharacter (`/Game/ThirdPerson/CommonFunctionLibrary.GetMyPlayerCharacter`))
  (for _array_element (`/Game/ThirdPerson/QuestSYstem/QuestLog_Component.CurrentQuests` (`self.GetComponentByClass` _myplayercharacter "/Game/ThirdPerson/QuestSYstem/QuestLog_Component.QuestLog_Component_C"))
    (`/Game/ThirdPerson/QuestSYstem/BP_QuestBase.UpdateObjectiveProgress` _array_element ObjectiveID 1)))

(fn `UserConstructionScript`
  (`parent.UserConstructionScript`))