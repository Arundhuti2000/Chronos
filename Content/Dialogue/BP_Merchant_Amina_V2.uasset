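; Amina, the merchant NPC who introduces Petra through scripted, voiced dialogue in WB_Dialogue, then quizzes the player before exploration.
; PlayerInput matches option text, completing quest objectives and unlocking codex entries.
; A DialogueStage counter drives the four-question quiz, where answers add or deduct KP and a failed deduction can show Game Over.
; Typed hint requests go to an AI HTTP component, and each hint response costs KP.
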(event `ShowCurrentDialogueStage`
  (bind _returnvalue (`KismetTextLibrary.Conv_StringToText` "What connects Arabia, Egypt, and the Mediterranean through Petra?"))
  (bind _returnvalue_2 (`KismetTextLibrary.Conv_StringToText` "What is the greatest danger in the desert outside Petra?"))
  (bind _returnvalue_3 (`KismetTextLibrary.Conv_StringToText` "What goods flow through Petra's trade routes?"))
  (bind _returnvalue_4 (`KismetTextLibrary.Conv_StringToText` "What is Petra also known as?"))
  (bind _returnvalue_5 (`GameplayStatics.GetPlayerController` 0))
  (bind _dialoguestage (`self.DialogueStage`))
  (bind _ui (`self.UI`))
  (bind _currentaudiocomponent (`self.CurrentAudioComponent`))
  (bind _ui_2 (`self.UI`))
  (bind _ui_3 (`self.UI`))
  (bind _ui_4 (`self.UI`))
  (if (== _dialoguestage 2)
    (`/Game/Dialogue/WB_Dialogue.AddChatLine` _ui _returnvalue_4 false)
    (`/Game/Dialogue/WB_Dialogue.SetDialogueOptions` _ui "The Green City" "The Rose City" "The City of Columns")
    (`/Game/Dialogue/WB_Dialogue.ShowOptionsPanel` _ui)
    (set `self.Current Quiz Question` (`KismetTextLibrary.Conv_TextToString` _returnvalue_4))
    (`Widget.SetVisibility` (`/Game/Dialogue/WB_Dialogue.InputBox_Border` (`self.UI`)) "SelfHitTestInvisible")
    (`Widget.SetVisibility` (`/Game/Dialogue/WB_Dialogue.BTN_Option4` (`self.UI`)) "Visible")
    (`TextBlock.SetText` (`/Game/Dialogue/WB_Dialogue.Txt_Option4` (`self.UI`)) (`KismetTextLibrary.Conv_StringToText` "Ask Amina for a hint"))
    (elif (== _dialoguestage 3)
      (`/Game/Dialogue/WB_Dialogue.AddChatLine` _ui_2 _returnvalue_3 false)
      (`/Game/Dialogue/WB_Dialogue.SetDialogueOptions` _ui_2 "Timber and stone" "Incense, spices, and silk" "Weapons and iron")
      (`/Game/Dialogue/WB_Dialogue.ShowOptionsPanel` _ui_2)
      (set `self.Current Quiz Question` (`KismetTextLibrary.Conv_TextToString` _returnvalue_3))
      (`Widget.SetVisibility` (`/Game/Dialogue/WB_Dialogue.InputBox_Border` (`self.UI`)) "SelfHitTestInvisible")
      (`Widget.SetVisibility` (`/Game/Dialogue/WB_Dialogue.BTN_Option4` (`self.UI`)) "Visible")
      (`TextBlock.SetText` (`/Game/Dialogue/WB_Dialogue.Txt_Option4` (`self.UI`)) (`KismetTextLibrary.Conv_StringToText` "Ask Amina for a hint"))
      (elif (== _dialoguestage 4)
        (`/Game/Dialogue/WB_Dialogue.AddChatLine` _ui_3 _returnvalue_2 false)
        (`/Game/Dialogue/WB_Dialogue.SetDialogueOptions` _ui_3 "Flooding rivers" "Wild animals" "Bandits and sandstorms")
        (`/Game/Dialogue/WB_Dialogue.ShowOptionsPanel` _ui_3)
        (set `self.Current Quiz Question` (`KismetTextLibrary.Conv_TextToString` _returnvalue_2))
        (`Widget.SetVisibility` (`/Game/Dialogue/WB_Dialogue.InputBox_Border` (`self.UI`)) "SelfHitTestInvisible")
        (`Widget.SetVisibility` (`/Game/Dialogue/WB_Dialogue.BTN_Option4` (`self.UI`)) "Visible")
        (`TextBlock.SetText` (`/Game/Dialogue/WB_Dialogue.Txt_Option4` (`self.UI`)) (`KismetTextLibrary.Conv_StringToText` "Ask Amina for a hint"))
        (elif (== _dialoguestage 5)
          (`/Game/Dialogue/WB_Dialogue.AddChatLine` _ui_4 _returnvalue false)
          (`/Game/Dialogue/WB_Dialogue.SetDialogueOptions` _ui_4 "Ancient trade routes" "A great river" "A mountain pass")
          (`/Game/Dialogue/WB_Dialogue.ShowOptionsPanel` _ui_4)
          (set `self.Current Quiz Question` (`KismetTextLibrary.Conv_TextToString` _returnvalue))
          (`Widget.SetVisibility` (`/Game/Dialogue/WB_Dialogue.InputBox_Border` (`self.UI`)) "SelfHitTestInvisible")
          (`Widget.SetVisibility` (`/Game/Dialogue/WB_Dialogue.BTN_Option4` (`self.UI`)) "Visible")
          (`TextBlock.SetText` (`/Game/Dialogue/WB_Dialogue.Txt_Option4` (`self.UI`)) (`KismetTextLibrary.Conv_StringToText` "Ask Amina for a hint"))
          (else
            (`/Game/Dialogue/WB_Dialogue.AddChatLine` (`self.UI`) (`KismetTextLibrary.Conv_StringToText` "Wonderful! You have a sharp mind, traveler. Speak to Obodas in the bazaar — he is the best place to start. And remember, in Petra, knowledge is the most valuable currency. May fortune smile upon you!") false)
            (bind _returnvalue_6 (`GameplayStatics.SpawnSound2D` "/Game/Audio/Amina/wonderful.wonderful" 1.0 1.0 0.0 null))
            (set `self.CurrentAudioComponent` _returnvalue_6)
            (bind _myplayercharacter (`/Game/ThirdPerson/CommonFunctionLibrary.GetMyPlayerCharacter`))
            (`/Game/ThirdPerson/Blueprints/BP_ThirdPersonCharacter.AddKP` _myplayercharacter 20)
            (`self.CompleteSpecificObjective` "obj_intro_complete")
            (set `self.HasCompletedIntro` true)
            (set `self.CanTalk?` true)
            (set `self.DialogueStage` 1)
            (`Widget.RemoveFromParent` (`self.UI`))
            (`WidgetBlueprintLibrary.SetInputMode_GameOnly` _returnvalue_5)
            (set `PlayerController.bShowMouseCursor` false _returnvalue_5)
            (`/Engine/EditorBlueprintResources/StandardMacros.IsValid` _currentaudiocomponent
              (:`Is Valid`
                (`AudioComponent.Stop` _currentaudiocomponent)))))))))

(event `/Game/Dialogue/BPI_Dialogue.Talk`
  (bind _returnvalue (`GameplayStatics.GetPlayerController` 0))
  (bind _dialoguestage (`self.DialogueStage`))
  ; Event Talk
  (if (`self.CanTalk?`)
    (set `self.CanTalk?` false)
    (bind _returnvalue_2 (`|CreateWidget` "/Game/Dialogue/WB_Dialogue.WB_Dialogue_C" _returnvalue self))
    (bind _output_get (set `self.UI` _returnvalue_2))
    (`UserWidget.AddToViewport` _output_get 0)
    (`WidgetBlueprintLibrary.SetInputMode_GameAndUIEx` _returnvalue _output_get "DoNotLock" false)
    (set `PlayerController.bShowMouseCursor` true _returnvalue)
    (if (== _dialoguestage 0)
      (`/Game/Dialogue/WB_Dialogue.AddChatLine` _output_get (`KismetTextLibrary.Conv_StringToText` "Peace be upon you, traveler! Welcome to Petra, the Rose City of the Nabataeans. I am Amina, a merchant of spices and precious goods.") false)
      (bind _returnvalue_3 (`GameplayStatics.SpawnSound2D` "/Game/Audio/Amina/amina_line1.amina_line1" 1.0 1.0 0.0 null))
      (set `self.CurrentAudioComponent` _returnvalue_3)
      (`/Game/Dialogue/WB_Dialogue.SetDialogueOptions` _output_get "What is this place?" "Who are the Nabataeans?" "What can I do here?")
      (`/Game/Dialogue/WB_Dialogue.ShowOptionsPanel` _output_get)
      (elif (== _dialoguestage 1)
        (`/Game/Dialogue/WB_Dialogue.AddChatLine` _output_get (`KismetTextLibrary.Conv_StringToText` "Welcome back, traveler! What else would you like to know?") false)
        (bind _returnvalue_4 (`GameplayStatics.SpawnSound2D` "/Game/Audio/Amina/welcome_back_traveler.welcome_back_traveler" 1.0 1.0 0.0 null))
        (set `self.CurrentAudioComponent` _returnvalue_4)
        (if (`self.HasCompletedIntro`)
          (`/Game/Dialogue/WB_Dialogue.SetDialogueOptions` _output_get "Tell me about the trade routes" "What dangers should I watch for?" "Tell me more about the goods")
          (`/Game/Dialogue/WB_Dialogue.ShowOptionsPanel` _output_get)
          (else
            (`/Game/Dialogue/WB_Dialogue.SetDialogueOptions` _output_get "Tell me about the trade routes" "What dangers should I watch for?" "I think I'm ready to explore")
            (`/Game/Dialogue/WB_Dialogue.ShowOptionsPanel` _output_get)))
        (elif (== _dialoguestage 2)
          (`self.ShowCurrentDialogueStage`)
          (elif (`self.HasCompletedIntro`)
            (`/Game/Dialogue/WB_Dialogue.AddChatLine` _output_get "Good to see you again! You seem well on your way. May the winds carry you safely." false)
            (bind _returnvalue_5 (`GameplayStatics.SpawnSound2D` "/Game/Audio/Amina/good_to_see_you.good_to_see_you" 1.0 1.0 0.0 null))
            (set `self.CurrentAudioComponent` _returnvalue_5)))))))

(event `self.ReceivePlayerInput`
  (params (InputText :type String))
  (bind _returnvalue (`GameplayStatics.GetPlayerController` 0))
  (bind _currentaudiocomponent (`self.CurrentAudioComponent`))
  (bind _ui (`self.UI`))
  (bind _currentaudiocomponent_2 (`self.CurrentAudioComponent`))
  (bind _ui_2 (`self.UI`))
  (bind _bp_httpclient_component (`self.BP_HttpClient_Component`))
  ; ReceivePlayerInput
  (`/Engine/EditorBlueprintResources/StandardMacros.IsValid` _currentaudiocomponent
    (:`Is Valid`
      (`AudioComponent.Stop` _currentaudiocomponent))
    (:`Is Not Valid`
      _))
  (`/Game/Dialogue/WB_Dialogue.AddChatLine` _ui_2 (`KismetTextLibrary.Conv_StringToText` InputText) true)
  (if (`self.Is Awaiting Hint Input`)
    (set `self.Is Awaiting Hint Input` false)
    (`Widget.SetVisibility` (`/Game/Dialogue/WB_Dialogue.InputBox_Border` (`self.UI`)) "Collapsed")
    (bind _full_prompt (`/Game/Blueprints/BP_HttpClient_Component.Build_Followup_Prompt` _bp_httpclient_component "amina" (`KismetStringLibrary.Concat_StrStr` (`KismetStringLibrary.Concat_StrStr` "The player is asking for a hint during a quiz about: " (`self.Current Quiz Question`)) InputText) ""))
    (`/Game/Blueprints/BP_HttpClient_Component.Send AI Request` _bp_httpclient_component _full_prompt "" "")
    (elif (`KismetStringLibrary.EqualEqual_StrStr` InputText "What is this place?")
      (`/Game/Dialogue/WB_Dialogue.AddChatLine` _ui_2 (`KismetTextLibrary.Conv_StringToText` "This is Petra — carved into the rose-red cliffs by the Nabataeans over two thousand years ago. It sits at the crossroads of ancient trade routes connecting Arabia, Egypt, and the Mediterranean. Caravans carrying incense, spices, silk, and precious stones all pass through here.") false)
      (bind _returnvalue_2 (`GameplayStatics.SpawnSound2D` "/Game/Audio/Amina/this_is_petra_amina.this_is_petra_amina" 1.0 1.0 0.0 null))
      (set `self.CurrentAudioComponent` _returnvalue_2)
      (`self.CompleteSpecificObjective` "obj_intro_learn_petra")
      (bind _myplayercharacter (`/Game/ThirdPerson/CommonFunctionLibrary.GetMyPlayerCharacter`))
      (`/Game/ThirdPerson/Codex/BP_CodexSystem.UnlockEntry` (`self.GetComponentByClass` _myplayercharacter "/Game/ThirdPerson/Codex/BP_CodexSystem.BP_CodexSystem_C") "codex_trade_routes")
      (if (< (`self.DialogueStage`) 2)
        (set `self.DialogueStage` 1))
      (if (`self.HasCompletedIntro`)
        (`/Game/Dialogue/WB_Dialogue.SetDialogueOptions` _ui_2 "Tell me about the trade routes" "What dangers should I watch for?" "Tell me more about the goods")
        (`/Game/Dialogue/WB_Dialogue.ShowOptionsPanel` _ui_2)
        (else
          (`/Game/Dialogue/WB_Dialogue.SetDialogueOptions` _ui_2 "Tell me about the trade routes" "What dangers should I watch for?" "I think I'm ready to explore")
          (`/Game/Dialogue/WB_Dialogue.ShowOptionsPanel` _ui_2)))
      (elif (`KismetStringLibrary.EqualEqual_StrStr` InputText "Who are the Nabataeans?")
        (`/Game/Dialogue/WB_Dialogue.AddChatLine` _ui_2 (`KismetTextLibrary.Conv_StringToText` "The Nabataeans were master traders and engineers. They controlled the water in this desert — hidden cisterns, secret channels carved into rock. That is how they built their wealth. They turned this barren canyon into the richest city on the trade routes.") false)
        (bind _returnvalue_3 (`GameplayStatics.SpawnSound2D` "/Game/Audio/Amina/Who_are_Nabateans.Who_are_Nabateans" 1.0 1.0 0.0 null))
        (set `self.CurrentAudioComponent` _returnvalue_3)
        (`self.CompleteSpecificObjective` "obj_intro_learn_petra")
        (bind _myplayercharacter_2 (`/Game/ThirdPerson/CommonFunctionLibrary.GetMyPlayerCharacter`))
        (`/Game/ThirdPerson/Codex/BP_CodexSystem.UnlockEntry` (`self.GetComponentByClass` _myplayercharacter_2 "/Game/ThirdPerson/Codex/BP_CodexSystem.BP_CodexSystem_C") "codex_nabataean_advantage")
        (if (< (`self.DialogueStage`) 2)
          (set `self.DialogueStage` 1))
        (if (`self.HasCompletedIntro`)
          (`/Game/Dialogue/WB_Dialogue.SetDialogueOptions` _ui_2 "Tell me about the trade routes" "What dangers should I watch for?" "Tell me more about the goods")
          (`/Game/Dialogue/WB_Dialogue.ShowOptionsPanel` _ui_2)
          (else
            (`/Game/Dialogue/WB_Dialogue.SetDialogueOptions` _ui_2 "Tell me about the trade routes" "What dangers should I watch for?" "I think I'm ready to explore")
            (`/Game/Dialogue/WB_Dialogue.ShowOptionsPanel` _ui_2)))
        (elif (`KismetStringLibrary.EqualEqual_StrStr` InputText "What can I do here?")
          (`/Game/Dialogue/WB_Dialogue.AddChatLine` _ui_2 (`KismetTextLibrary.Conv_StringToText` "There is much to discover! The merchant Obodas in the bazaar knows everything about the incense trade. The Treasury of Al-Khazneh holds ancient secrets, but a guard blocks the entrance. And if you need a guide, old Abu near the entrance knows every path in these canyons.") false)
          (bind _returnvalue_4 (`GameplayStatics.SpawnSound2D` "/Game/Audio/Amina/What_to_explore.What_to_explore" 1.0 1.0 0.0 null))
          (set `self.CurrentAudioComponent` _returnvalue_4)
          (`self.CompleteSpecificObjective` "obj_intro_learn_petra")
          (if (< (`self.DialogueStage`) 2)
            (set `self.DialogueStage` 1))
          (if (`self.HasCompletedIntro`)
            (`/Game/Dialogue/WB_Dialogue.SetDialogueOptions` _ui_2 "Tell me about the trade routes" "What dangers should I watch for?" "Tell me more about the goods")
            (`/Game/Dialogue/WB_Dialogue.ShowOptionsPanel` _ui_2)
            (else
              (`/Game/Dialogue/WB_Dialogue.SetDialogueOptions` _ui_2 "Tell me about the trade routes" "What dangers should I watch for?" "I think I'm ready to explore")
              (`/Game/Dialogue/WB_Dialogue.ShowOptionsPanel` _ui_2)))
          (elif (`KismetStringLibrary.EqualEqual_StrStr` InputText "Tell me about the trade routes")
            (`/Game/Dialogue/WB_Dialogue.AddChatLine` _ui_2 (`KismetTextLibrary.Conv_StringToText` "Caravans travel from the heart of Arabia through Petra to the ports of Gaza on the Mediterranean. Frankincense and myrrh from Yemen, silk from the East, spices from India — they all flow through this city. The Nabataeans charge tolls and offer safe passage. That is how Petra grew wealthy beyond imagination.") false)
            (bind _returnvalue_5 (`GameplayStatics.SpawnSound2D` "/Game/Audio/Amina/caravans_travel.caravans_travel" 1.0 1.0 0.0 null))
            (set `self.CurrentAudioComponent` _returnvalue_5)
            (`self.CompleteSpecificObjective` "obj_intro_learn_trade")
            (bind _myplayercharacter_3 (`/Game/ThirdPerson/CommonFunctionLibrary.GetMyPlayerCharacter`))
            (`/Game/ThirdPerson/Codex/BP_CodexSystem.UnlockEntry` (`self.GetComponentByClass` _myplayercharacter_3 "/Game/ThirdPerson/Codex/BP_CodexSystem.BP_CodexSystem_C") "codex_incense_trade")
            (if (`self.HasCompletedIntro`)
              (`/Game/Dialogue/WB_Dialogue.SetDialogueOptions` _ui_2 "Tell me about the trade routes" "What dangers should I watch for?" "Tell me more about the goods")
              (`/Game/Dialogue/WB_Dialogue.ShowOptionsPanel` _ui_2)
              (else
                (`/Game/Dialogue/WB_Dialogue.SetDialogueOptions` _ui_2 "What dangers should I watch for?" "I think I'm ready to explore" "Tell me more about the goods")
                (`/Game/Dialogue/WB_Dialogue.ShowOptionsPanel` _ui_2)))
            (elif (`KismetStringLibrary.EqualEqual_StrStr` InputText "What dangers should I watch for?")
              (`/Game/Dialogue/WB_Dialogue.AddChatLine` _ui_2 (`KismetTextLibrary.Conv_StringToText` "The desert is unforgiving, traveler. Bandits prey on lone travelers, and sandstorms can swallow a caravan whole. But inside Petra, the greatest danger is ignorance. Speak to the locals, learn the customs, and you will be safe. The people here respect knowledge and courtesy.") false)
              (bind _returnvalue_6 (`GameplayStatics.SpawnSound2D` "/Game/Audio/Amina/dangers_of_desert.dangers_of_desert" 1.0 1.0 0.0 null))
              (set `self.CurrentAudioComponent` _returnvalue_6)
              (`self.CompleteSpecificObjective` "obj_intro_learn_tasks")
              (bind _myplayercharacter_4 (`/Game/ThirdPerson/CommonFunctionLibrary.GetMyPlayerCharacter`))
              (`/Game/ThirdPerson/Codex/BP_CodexSystem.UnlockEntry` (`self.GetComponentByClass` _myplayercharacter_4 "/Game/ThirdPerson/Codex/BP_CodexSystem.BP_CodexSystem_C") "codex_desert_dangers")
              (if (`self.HasCompletedIntro`)
                (`/Game/Dialogue/WB_Dialogue.SetDialogueOptions` _ui_2 "Tell me about the trade routes" "What dangers should I watch for?" "Tell me more about the goods")
                (`/Game/Dialogue/WB_Dialogue.ShowOptionsPanel` _ui_2)
                (else
                  (`/Game/Dialogue/WB_Dialogue.SetDialogueOptions` _ui_2 "Tell me about the trade routes" "I think I'm ready to explore" "Any advice for a newcomer?")
                  (`/Game/Dialogue/WB_Dialogue.ShowOptionsPanel` _ui_2)))
              (elif (`KismetStringLibrary.EqualEqual_StrStr` InputText "I think I'm ready to explore")
                (if (`self.HasCompletedIntro`)
                  (`/Game/Dialogue/WB_Dialogue.AddChatLine` _ui_2 "You've already proven yourself, traveler! Go explore Petra — Obodas awaits you in the bazaar." false)
                  (`Widget.RemoveFromParent` _ui_2)
                  (`WidgetBlueprintLibrary.SetInputMode_GameOnly` _returnvalue)
                  (set `PlayerController.bShowMouseCursor` false _returnvalue)
                  (`/Engine/EditorBlueprintResources/StandardMacros.IsValid` _currentaudiocomponent_2
                    (:`Is Valid`
                      (`AudioComponent.Stop` _currentaudiocomponent_2)))
                  (else
                    (`/Game/Dialogue/WB_Dialogue.AddChatLine` _ui_2 (`KismetTextLibrary.Conv_StringToText` "Before you go, let me test your memory! A good traveler always remembers what they've learned.") false)
                    (bind _returnvalue_7 (`GameplayStatics.SpawnSound2D` "/Game/Audio/Amina/Before_you_go.Before_you_go" 1.0 1.0 0.0 null))
                    (set `self.CurrentAudioComponent` _returnvalue_7)
                    (`KismetSystemLibrary.Delay` 3.0)
                    (set `self.DialogueStage` 2)
                    (`self.ShowCurrentDialogueStage`)))
                (elif (`KismetArrayLibrary.Array_Contains` (`self.QuizOptions`) InputText)
                  (`self.HandleQuizAnswer` InputText)
                  (elif (`KismetStringLibrary.EqualEqual_StrStr` InputText "Ask Amina for a hint")
                    (`Widget.SetVisibility` (`/Game/Dialogue/WB_Dialogue.BTN_Option4` _ui) "Collapsed")
                    (`Widget.SetVisibility` (`/Game/Dialogue/WB_Dialogue.InputBox_Border` _ui) "Visible")
                    (set `self.Is Awaiting Hint Input` true)
                    (set `self.Is Hint Response` true)
                    (else
                      (`/Game/Dialogue/WB_Dialogue.AddChatLine` _ui_2 (`KismetTextLibrary.Conv_StringToText` "There is always more to learn! Explore the bazaar, talk to the locals. Every person here has a story to tell.") false)
                      (bind _returnvalue_8 (`GameplayStatics.SpawnSound2D` "/Game/Audio/Amina/explore_there_is_more.explore_there_is_more" 1.0 1.0 0.0 null))
                      (set `self.CurrentAudioComponent` _returnvalue_8)
                      (if (`self.HasCompletedIntro`)
                        (`/Game/Dialogue/WB_Dialogue.SetDialogueOptions` _ui_2 "Tell me about the trade routes" "What dangers should I watch for?" "Tell me more about the goods")
                        (`/Game/Dialogue/WB_Dialogue.ShowOptionsPanel` _ui_2)
                        (else
                          (`/Game/Dialogue/WB_Dialogue.SetDialogueOptions` _ui_2 "Tell me about the trade routes" "What dangers should I watch for?" "I think I'm ready to explore")
                          (`/Game/Dialogue/WB_Dialogue.ShowOptionsPanel` _ui_2))))))))))))))

(event `self.OnAIResponseReceived_Event`
  (params (ResponseText :type String))
  (`self.AddToHistory` "" "AI")
  (`/Game/Dialogue/WB_Dialogue.AddChatLine` (`self.UI`) (`KismetTextLibrary.Conv_StringToText` ResponseText) false)
  (if (`self.Is Hint Response`)
    (set `self.Is Hint Response` false)
    (bind _myplayercharacter (`/Game/ThirdPerson/CommonFunctionLibrary.GetMyPlayerCharacter`))
    (`/Game/ThirdPerson/Blueprints/BP_ThirdPersonCharacter.DeductKP` _myplayercharacter 5))
  (`self.CheckQuestKeywords` ResponseText)
  (bind _myplayercharacter_2 (`/Game/ThirdPerson/CommonFunctionLibrary.GetMyPlayerCharacter`))
  (bind _returnvalue (`self.GetComponentByClass` _myplayercharacter_2 "/Game/ThirdPerson/QuestSYstem/QuestLog_Component.QuestLog_Component_C"))
  (for _array_element (`/Game/ThirdPerson/QuestSYstem/QuestLog_Component.CurrentQuests` _returnvalue)
    (`/Engine/EditorBlueprintResources/StandardMacros.IsValid` _array_element
      (:`Is Valid`
        (for _array_element_2 (`.Objectives_21_75F1BA2A457170AB65DED5B45FFC78A1` (break `/Game/ThirdPerson/QuestSYstem/StageDetails` (`/Game/ThirdPerson/QuestSYstem/BP_QuestBase.CurrentStageDetails` _array_element)))
          (bind (_objectivename _description _type _objectiveid) (break `/Game/ThirdPerson/QuestSYstem/ObjectiveDetails` _array_element_2))
          (bind _iscomplete (`/Game/ThirdPerson/QuestSYstem/BP_QuestBase.IsObjectiveComplete` _array_element _objectiveid))
          (if (not _iscomplete)
            (if (`KismetArrayLibrary.Array_Contains` (`self.ObjectivesToComplete`) _objectiveid)
              (`/Game/ThirdPerson/QuestSYstem/BP_QuestBase.UpdateObjectiveProgress` _array_element _objectiveid 1)
              (`self.ProcessQuestForCodex` _array_element)
              (break)))))))
  (for _ (`/Game/ThirdPerson/QuestSYstem/QuestLog_Component.CompletedQuestActors` _returnvalue)
    _)
  (`KismetSystemLibrary.Delay` 6.0)
  (`self.ShowCurrentDialogueStage`))

(event `BeginPlay`
  (`parent.ReceiveBeginPlay`)
  (add `/Game/Blueprints/BP_HttpClient_Component.OnAIResponseReceived` (`self.BP_HttpClient_Component`) (delegate `self.OnAIResponseReceived_Event`)))

(fn `CompleteSpecificObjective`
  (params (ObjectiveID :type String))
  (bind _myplayercharacter (`/Game/ThirdPerson/CommonFunctionLibrary.GetMyPlayerCharacter`))
  (for _array_element (`/Game/ThirdPerson/QuestSYstem/QuestLog_Component.CurrentQuests` (`self.GetComponentByClass` _myplayercharacter "/Game/ThirdPerson/QuestSYstem/QuestLog_Component.QuestLog_Component_C"))
    (`/Game/ThirdPerson/QuestSYstem/BP_QuestBase.UpdateObjectiveProgress` _array_element ObjectiveID 1)))

(fn `HandleQuizAnswer`
  (params (AnswerText :type String))
  (bind _dialoguestage (`self.DialogueStage`))
  (bind _ui (`self.UI`))
  (bind _kprewardpercorrect (`self.KPRewardPerCorrect`))
  (bind _kppenaltyperwrong (`self.KPPenaltyPerWrong`))
  (if (== _dialoguestage 2)
    (`|ExecutionSequence`
      (:`then_0`
        (if (`KismetStringLibrary.EqualEqual_StrStr` AnswerText "The Rose City")
          (bind _myplayercharacter (`/Game/ThirdPerson/CommonFunctionLibrary.GetMyPlayerCharacter`))
          (`/Game/ThirdPerson/Blueprints/BP_ThirdPersonCharacter.AddKP` _myplayercharacter _kprewardpercorrect)
          (set `self.DialogueStage` (+ (`self.DialogueStage`) 1))
          (`self.CompleteSpecificObjective` self "obj_intro_learn_petra")
          (bind _myplayercharacter_2 (`/Game/ThirdPerson/CommonFunctionLibrary.GetMyPlayerCharacter`))
          (`/Game/ThirdPerson/Codex/BP_CodexSystem.UnlockEntry` (`self.GetComponentByClass` _myplayercharacter_2 "/Game/ThirdPerson/Codex/BP_CodexSystem.BP_CodexSystem_C") "codex_petra_exports")
          (`/Game/Dialogue/WB_Dialogue.AddChatLine` _ui (`KismetTextLibrary.Conv_StringToText` "Correct! Petra is carved from rose-red sandstone, giving it the name The Rose City. +10 KP!") false)
          (`self.ShowCurrentDialogueStage` self)
          (else
            (bind _myplayercharacter_3 (`/Game/ThirdPerson/CommonFunctionLibrary.GetMyPlayerCharacter`))
            (bind _bgameover (`/Game/ThirdPerson/Blueprints/BP_ThirdPersonCharacter.DeductKP` _myplayercharacter_3 _kppenaltyperwrong))
            (if _bgameover
              (bind _returnvalue (`|CreateWidget` "/Game/ThirdPerson/QuestSYstem/UI/WBP_GameOver.WBP_GameOver_C"))
              (`UserWidget.AddToViewport` _returnvalue 0)
              (else
                (`/Game/Dialogue/WB_Dialogue.AddChatLine` _ui (`KismetTextLibrary.Conv_StringToText` "Not quite... Petra is known as The Rose City for its rose-red cliffs. -3 KP!") false)
                (`self.ShowCurrentDialogueStage` self)))))))
    (elif (== _dialoguestage 3)
      (`|ExecutionSequence`
        (:`then_0`
          (if (`KismetStringLibrary.EqualEqual_StrStr` AnswerText "Incense, spices, and silk")
            (bind _myplayercharacter_4 (`/Game/ThirdPerson/CommonFunctionLibrary.GetMyPlayerCharacter`))
            (`/Game/ThirdPerson/Blueprints/BP_ThirdPersonCharacter.AddKP` _myplayercharacter_4 _kprewardpercorrect)
            (set `self.DialogueStage` (+ (`self.DialogueStage`) 1))
            (`self.CompleteSpecificObjective` self "obj_intro_learn_trade")
            (bind _myplayercharacter_5 (`/Game/ThirdPerson/CommonFunctionLibrary.GetMyPlayerCharacter`))
            (`/Game/ThirdPerson/Codex/BP_CodexSystem.UnlockEntry` (`self.GetComponentByClass` _myplayercharacter_5 "/Game/ThirdPerson/Codex/BP_CodexSystem.BP_CodexSystem_C") "codex_incense_trade")
            (`/Game/Dialogue/WB_Dialogue.AddChatLine` _ui (`KismetTextLibrary.Conv_StringToText` "Correct! These precious goods made Petra fabulously wealthy. +10 KP!") false)
            (`self.ShowCurrentDialogueStage` self)
            (else
              (bind _myplayercharacter_6 (`/Game/ThirdPerson/CommonFunctionLibrary.GetMyPlayerCharacter`))
              (bind _bgameover_2 (`/Game/ThirdPerson/Blueprints/BP_ThirdPersonCharacter.DeductKP` _myplayercharacter_6 _kppenaltyperwrong))
              (if _bgameover_2
                (bind _returnvalue_2 (`|CreateWidget` "/Game/ThirdPerson/QuestSYstem/UI/WBP_GameOver.WBP_GameOver_C"))
                (`UserWidget.AddToViewport` _returnvalue_2 0)
                (else
                  (`/Game/Dialogue/WB_Dialogue.AddChatLine` _ui (`KismetTextLibrary.Conv_StringToText` "Not quite... Incense, spices, and silk all flowed through Petra's trade routes. -3 KP!") false)
                  (`self.ShowCurrentDialogueStage` self)))))))
      (elif (== _dialoguestage 4)
        (`|ExecutionSequence`
          (:`then_0`
            (if (`KismetStringLibrary.EqualEqual_StrStr` AnswerText "Bandits and sandstorms")
              (bind _myplayercharacter_7 (`/Game/ThirdPerson/CommonFunctionLibrary.GetMyPlayerCharacter`))
              (`/Game/ThirdPerson/Blueprints/BP_ThirdPersonCharacter.AddKP` _myplayercharacter_7 _kprewardpercorrect)
              (set `self.DialogueStage` (+ (`self.DialogueStage`) 1))
              (`self.CompleteSpecificObjective` self "obj_intro_learn_tasks")
              (bind _myplayercharacter_8 (`/Game/ThirdPerson/CommonFunctionLibrary.GetMyPlayerCharacter`))
              (`/Game/ThirdPerson/Codex/BP_CodexSystem.UnlockEntry` (`self.GetComponentByClass` _myplayercharacter_8 "/Game/ThirdPerson/Codex/BP_CodexSystem.BP_CodexSystem_C") "codex_desert_dangers")
              (`/Game/Dialogue/WB_Dialogue.AddChatLine` _ui (`KismetTextLibrary.Conv_StringToText` "Correct! The desert is full of perils for travelers. +10 KP!") false)
              (`self.ShowCurrentDialogueStage` self)
              (else
                (bind _myplayercharacter_9 (`/Game/ThirdPerson/CommonFunctionLibrary.GetMyPlayerCharacter`))
                (bind _bgameover_3 (`/Game/ThirdPerson/Blueprints/BP_ThirdPersonCharacter.DeductKP` _myplayercharacter_9 _kppenaltyperwrong))
                (if _bgameover_3
                  (bind _returnvalue_3 (`|CreateWidget` "/Game/ThirdPerson/QuestSYstem/UI/WBP_GameOver.WBP_GameOver_C"))
                  (`UserWidget.AddToViewport` _returnvalue_3 0)
                  (else
                    (`/Game/Dialogue/WB_Dialogue.AddChatLine` _ui (`KismetTextLibrary.Conv_StringToText` "Not quite... Bandits and sandstorms are the greatest threats outside Petra. -3 KP!") false)
                    (`self.ShowCurrentDialogueStage` self)))))))
        (elif (== _dialoguestage 5)
          (`|ExecutionSequence`
            (:`then_0`
              (if (`KismetStringLibrary.EqualEqual_StrStr` AnswerText "Ancient trade routes")
                (bind _myplayercharacter_10 (`/Game/ThirdPerson/CommonFunctionLibrary.GetMyPlayerCharacter`))
                (`/Game/ThirdPerson/Blueprints/BP_ThirdPersonCharacter.AddKP` _myplayercharacter_10 _kprewardpercorrect)
                (set `self.DialogueStage` (+ (`self.DialogueStage`) 1))
                (`self.CompleteSpecificObjective` self "obj_intro_learn_tasks")
                (bind _myplayercharacter_11 (`/Game/ThirdPerson/CommonFunctionLibrary.GetMyPlayerCharacter`))
                (`/Game/ThirdPerson/Codex/BP_CodexSystem.UnlockEntry` (`self.GetComponentByClass` _myplayercharacter_11 "/Game/ThirdPerson/Codex/BP_CodexSystem.BP_CodexSystem_C") "codex_trade_routes")
                (`/Game/Dialogue/WB_Dialogue.AddChatLine` _ui (`KismetTextLibrary.Conv_StringToText` "Correct! Petra sits at the crossroads of ancient trade routes spanning three continents. +10 KP!") false)
                (`self.ShowCurrentDialogueStage` self)
                (else
                  (bind _myplayercharacter_12 (`/Game/ThirdPerson/CommonFunctionLibrary.GetMyPlayerCharacter`))
                  (bind _bgameover_4 (`/Game/ThirdPerson/Blueprints/BP_ThirdPersonCharacter.DeductKP` _myplayercharacter_12 _kppenaltyperwrong))
                  (if _bgameover_4
                    (bind _returnvalue_4 (`|CreateWidget` "/Game/ThirdPerson/QuestSYstem/UI/WBP_GameOver.WBP_GameOver_C"))
                    (`UserWidget.AddToViewport` _returnvalue_4 0)
                    (else
                      (`/Game/Dialogue/WB_Dialogue.AddChatLine` _ui (`KismetTextLibrary.Conv_StringToText` "Not quite... Ancient trade routes connecting Arabia, Egypt, and the Mediterranean all pass through Petra. -3 KP!") false)
                      (`self.ShowCurrentDialogueStage` self))))))))))))

(fn `ProcessQuestForCodex`
  (params (QUEST :type "/Game/ThirdPerson/QuestSYstem/BP_QuestBase Object Reference"))
  (bind _returnvalue (`self.GetComponentByClass` (`GameplayStatics.GetPlayerCharacter` 0) "/Game/ThirdPerson/Codex/BP_CodexSystem.BP_CodexSystem_C"))
  (bind (_value _returnvalue_2) (`BlueprintMapLibrary.Map_Find` (`self.QuestToCodexMap`) "obj_bonus"))
  (set `self.CompletedCount` 0)
  (for _array_element (`self.ObjectivesToComplete`)
    (bind _iscomplete (`/Game/ThirdPerson/QuestSYstem/BP_QuestBase.IsObjectiveComplete` QUEST _array_element))
    (if _iscomplete
      (set `self.CompletedCount` (+ (`self.CompletedCount`) 1))
      (bind (_value_2 _returnvalue_3) (`BlueprintMapLibrary.Map_Find` (`self.QuestToCodexMap`) _array_element))
      (if _returnvalue_3
        (`/Engine/EditorBlueprintResources/StandardMacros.IsValid` _returnvalue
          (:`Is Valid`
            (`/Game/ThirdPerson/Codex/BP_CodexSystem.UnlockEntry` _returnvalue (`KismetStringLibrary.Conv_StringToName` _value_2)))))))
  (if (== (`self.CompletedCount`) (`KismetArrayLibrary.Array_Length` (`self.ObjectivesToComplete`)))
    (if _returnvalue_2
      (`/Game/ThirdPerson/Codex/BP_CodexSystem.UnlockEntry` (`self.GetComponentByClass` (`GameplayStatics.GetPlayerCharacter` 0) "/Game/ThirdPerson/Codex/BP_CodexSystem.BP_CodexSystem_C") (`KismetStringLibrary.Conv_StringToName` _value)))))

(fn `UserConstructionScript`
  (`parent.UserConstructionScript`))