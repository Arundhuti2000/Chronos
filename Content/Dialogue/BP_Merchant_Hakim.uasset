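; Dialogue NPC Hakim, a Petra merchant who hints at guard Khalil's weakness for honey cakes and sells one for knowledge points.
; Talk, gated by CanTalk, opens WB_Dialogue with a greeting chosen by DialogueStage.
; PlayerInput matches option text through nested branches to set replies and options, usually with voice audio.
; Specific answers unlock BP_CodexSystem entries, advance QuestLog_Component objectives, or exchange KP for the inventory item.
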(event `/Game/Dialogue/BPI_Dialogue.Talk`
  (bind _returnvalue (`GameplayStatics.GetPlayerController` 0))
  (bind _ui (`self.UI`))
  (bind _ui_2 (`self.UI`))
  (if (`self.CanTalk?`)
    (set `self.CanTalk?` false)
    (bind _returnvalue_2 (`|CreateWidget` "/Game/Dialogue/WB_Dialogue.WB_Dialogue_C" _returnvalue self))
    (bind _output_get (set `self.UI` _returnvalue_2))
    (`UserWidget.AddToViewport` _output_get 0)
    (set `PlayerController.bShowMouseCursor` true _returnvalue)
    (if (== (`self.Dialogue Stage`) 0)
      (`/Game/Dialogue/WB_Dialogue.AddChatLine` _ui_2 "Peace be upon you! I am Hakim, baker and trader of fine goods." false)
      (bind _returnvalue_3 (`GameplayStatics.SpawnSound2D` "/Game/Audio/hakim/hakimIntro.hakimIntro" 1.0 1.0 0.0 null))
      (set `self.Current Audio Component` _returnvalue_3)
      (`/Game/Dialogue/WB_Dialogue.SetDialogueOptions` _ui_2 "What foods do people eat here?" "Do you know Khalil?" "")
      (`/Game/Dialogue/WB_Dialogue.ShowOptionsPanel` _ui_2)
      (elif (== (`self.Dialogue Stage`) 1)
        (`/Game/Dialogue/WB_Dialogue.AddChatLine` _ui "Welcome back, friend! What else can I tell you?" false)
        (`/Game/Dialogue/WB_Dialogue.SetDialogueOptions` _ui "What foods do people eat here?" "Do you know Khalil?" "")
        (`/Game/Dialogue/WB_Dialogue.ShowOptionsPanel` _ui)))))

(event `self.ReceivePlayerInput`
  (params (InputText :type String))
  (bind _ui (`self.UI`))
  (bind _ui_2 (`self.UI`))
  (bind _ui_3 (`self.UI`))
  (bind _current_audio_component (`self.Current Audio Component`))
  (bind _ui_4 (`self.UI`))
  (`/Engine/EditorBlueprintResources/StandardMacros.IsValid` _current_audio_component
    (:`Is Valid`
      (`AudioComponent.Stop` _current_audio_component))
    (:`Is Not Valid`
      _))
  (if (`KismetStringLibrary.EqualEqual_StrStr` "What foods do people eat here?" InputText)
    (`/Game/Dialogue/WB_Dialogue.AddChatLine` (`self.UI`) "Ah, the finest food in Petra! Every day we eat flatbread, lentils, dates, figs and olives. Honey sweetens everything here - it is worth its weight in silver on the trade routes!" false)
    (bind _returnvalue (`GameplayStatics.SpawnSound2D` "/Game/Audio/hakim/hakimfinestfood.hakimfinestfood" 1.0 1.0 0.0 null))
    (set `self.Current Audio Component` _returnvalue)
    (bind _myplayercharacter (`/Game/ThirdPerson/CommonFunctionLibrary.GetMyPlayerCharacter`))
    (`/Game/ThirdPerson/Codex/BP_CodexSystem.UnlockEntry` (`self.GetComponentByClass` _myplayercharacter "/Game/ThirdPerson/Codex/BP_CodexSystem.BP_CodexSystem_C") "codex_petra_foods")
    (set `self.Has Talked About Food` true)
    (set `self.Dialogue Stage` 1)
    (`/Game/Dialogue/WB_Dialogue.SetDialogueOptions` (`self.UI`) "Do you know Khalil?" "Tell me more about honey" "")
    (elif (`KismetStringLibrary.EqualEqual_StrStr` "Do you know Khalil?" InputText)
      (`/Game/Dialogue/WB_Dialogue.AddChatLine` (`self.UI`) "Ah yes... Khalil! The guard at the treasury gate. A good man, very loyal. Very... hungry." false)
      (bind _returnvalue_2 (`GameplayStatics.SpawnSound2D` "/Game/Audio/hakim/hakim_khlil_hungry.hakim_khlil_hungry" 1.0 1.0 0.0 null))
      (set `self.Current Audio Component` _returnvalue_2)
      (set `self.Has Talked About Khalil` true)
      (set `self.Dialogue Stage` 1)
      (`/Game/Dialogue/WB_Dialogue.SetDialogueOptions` _ui_4 "What is his weakness?" "What foods do people eat here?" "")
      (`/Game/Dialogue/WB_Dialogue.ShowOptionsPanel` _ui_4)
      (elif (`KismetStringLibrary.EqualEqual_StrStr` "What is his weakness?" InputText)
        (`/Game/Dialogue/WB_Dialogue.AddChatLine` (`self.UI`) "Ha! My friend, Khalil cannot resist honey cakes. Fresh from the oven, warm with honey — he would open any gate for one! and let you take the artifact in the Tresury \nHoney cakes are the pride of our bakers here in Petra." false)
        (bind _returnvalue_3 (`GameplayStatics.SpawnSound2D` "/Game/Audio/hakim/hakim_honeycakes.hakim_honeycakes" 1.0 1.0 0.0 null))
        (set `self.Current Audio Component` _returnvalue_3)
        (bind _myplayercharacter_2 (`/Game/ThirdPerson/CommonFunctionLibrary.GetMyPlayerCharacter`))
        (`/Game/ThirdPerson/Codex/BP_CodexSystem.UnlockEntry` (`self.GetComponentByClass` _myplayercharacter_2 "/Game/ThirdPerson/Codex/BP_CodexSystem.BP_CodexSystem_C") "codex_honey_cake")
        (bind _myplayercharacter_3 (`/Game/ThirdPerson/CommonFunctionLibrary.GetMyPlayerCharacter`))
        (for _array_element (`/Game/ThirdPerson/QuestSYstem/QuestLog_Component.CurrentQuests` (`self.GetComponentByClass` _myplayercharacter_3 "/Game/ThirdPerson/QuestSYstem/QuestLog_Component.QuestLog_Component_C"))
          (`/Game/ThirdPerson/QuestSYstem/BP_QuestBase.UpdateObjectiveProgress` _array_element "obj_merchant_intel" 1)
          (`/Game/Dialogue/WB_Dialogue.SetDialogueOptions` _ui_2 "Where can I find honey cakes?" "Tell me more about honey" "")
          (`/Game/Dialogue/WB_Dialogue.ShowOptionsPanel` _ui_2))
        (elif (`KismetStringLibrary.EqualEqual_StrStr` "Where can I find honey cakes?" InputText)
          (`/Game/Dialogue/WB_Dialogue.AddChatLine` (`self.UI`) "I have some right here! But good things have a price, friend. Fifty knowledge points and one is yours." false)
          (bind _returnvalue_4 (`GameplayStatics.SpawnSound2D` "/Game/Audio/hakim/hakim_50KP.hakim_50KP" 1.0 1.0 0.0 null))
          (set `self.Current Audio Component` _returnvalue_4)
          (`/Game/Dialogue/WB_Dialogue.SetDialogueOptions` (`self.UI`) "Here are 50 KP, give me a honey cake" "Maybe another time" "")
          (`/Game/Dialogue/WB_Dialogue.ShowOptionsPanel` (`self.UI`))
          (elif (`KismetStringLibrary.EqualEqual_StrStr` "Here are 50 KP, give me a honey cake" InputText)
            (bind _myplayercharacter_4 (`/Game/ThirdPerson/CommonFunctionLibrary.GetMyPlayerCharacter`))
            (bind _currentkp (`/Game/ThirdPerson/Blueprints/BP_ThirdPersonCharacter.GetKP` _myplayercharacter_4))
            (if (> _currentkp 49)
              (`/Game/ThirdPerson/Blueprints/BP_ThirdPersonCharacter.DeductKP` _myplayercharacter_4 50)
              (`/Game/ThirdPerson/Inventory/BP_InventoryComponent.AddItem` (`/Game/ThirdPerson/Blueprints/BP_ThirdPersonCharacter.InventoryComponent` _myplayercharacter_4) "honeycake")
              (set `self.Has Given Honey Cake` true)
              (bind _myplayercharacter_5 (`/Game/ThirdPerson/CommonFunctionLibrary.GetMyPlayerCharacter`))
              (for _array_element_2 (`/Game/ThirdPerson/QuestSYstem/QuestLog_Component.CurrentQuests` (`self.GetComponentByClass` _myplayercharacter_5 "/Game/ThirdPerson/QuestSYstem/QuestLog_Component.QuestLog_Component_C"))
                (`/Game/ThirdPerson/QuestSYstem/BP_QuestBase.UpdateObjectiveProgress` _array_element_2 "obj_find_cakes" 1))
              (`/Game/Dialogue/WB_Dialogue.AddChatLine` (`self.UI`) "Here you go, traveler! Fresh and sweet. \nKhalil will not be able to say no!" false)
              (bind _returnvalue_5 (`GameplayStatics.SpawnSound2D` "/Game/Audio/hakim/hakim_hereItis.hakim_hereItis" 1.0 1.0 0.0 null))
              (set `self.Current Audio Component` _returnvalue_5)
              (else
                (`/Game/Dialogue/WB_Dialogue.AddChatLine` (`self.UI`) "You do not have enough knowledge points yet, friend. Come back when you have learned more!" false)))
            (elif (`KismetStringLibrary.EqualEqual_StrStr` "Maybe another time" InputText)
              (`/Game/Dialogue/WB_Dialogue.AddChatLine` _ui_3 "Of course! My door is always open, friend." false)
              (bind _returnvalue_6 (`GameplayStatics.SpawnSound2D` "/Game/Audio/hakim/hakim_ofcourse.hakim_ofcourse" 1.0 1.0 0.0 null))
              (set `self.Current Audio Component` _returnvalue_6)
              (`/Game/Dialogue/WB_Dialogue.SetDialogueOptions` _ui_3 "Where can I find honey cakes?" "Do you know Khalil?" "")
              (`/Game/Dialogue/WB_Dialogue.ShowOptionsPanel` _ui_3)
              (elif (`KismetStringLibrary.EqualEqual_StrStr` "Tell me more about honey" InputText)
                (`/Game/Dialogue/WB_Dialogue.AddChatLine` _ui "Honey is the treasure of the desert, my friend! We collect it from wild hives in the cliffs above Petra. It never spoils — traders have carried it for months across the desert. The Romans pay a fortune for it, and our bakers use it in everything." false)
                (bind _returnvalue_7 (`GameplayStatics.SpawnSound2D` "/Game/Audio/hakim/hakim_honeyDetails.hakim_honeyDetails" 1.0 1.0 0.0 null))
                (set `self.Current Audio Component` _returnvalue_7)
                (`/Game/Dialogue/WB_Dialogue.SetDialogueOptions` _ui "Where can I find honey cakes?" "Do you know Khalil?" "")
                (`/Game/Dialogue/WB_Dialogue.ShowOptionsPanel` _ui)))))))))

(fn `UserConstructionScript`
  (`parent.UserConstructionScript`))