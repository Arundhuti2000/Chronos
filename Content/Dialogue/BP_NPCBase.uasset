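; Base NPC for dialogue in a Petra adventure, using either AI chat or scripted lines in a WB_Dialogue widget.
; AI prompts go through BPHttpClientComponent with a capped rolling chat history as context.
; Replies award KP via [CORRECT]/[PARTIAL] tags and advance quest objectives through keyword matching, with a honeycake check for guard bribes.
; Player questions deduct KP, and a true DeductKP result pauses into game over.
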(event `self.ReceiveBeginPlay`
  ; On AI Response Received
  (`/Engine/EditorBlueprintResources/StandardMacros.IsValid` (`self.BP_HttpClient_Component`)
    (:`Is Valid`
      (add `/Game/Blueprints/BP_HttpClient_Component.OnAIResponseReceived` (`self.BP_HttpClient_Component`) (delegate `OnAIResponseReceived_Event`)))
    (:`Is Not Valid`
      (`KismetSystemLibrary.PrintString` "HTTP Client component not found on NPC" true true (struct :`R` 1.0 :`A` 1.0)))))

(event `OnAIResponseReceived_Event`
  (params (ResponseText :type String))
  ; On AI Response Received
  (`self.AddToHistory` ResponseText "AI")
  (set `self.IsFirstMessage` false)
  (`/Game/Dialogue/WB_Dialogue.AddChatLine` (`self.UI`) (`KismetTextLibrary.Conv_StringToText` ResponseText) false)
  (`self.CheckQuestKeywords` ResponseText)
  (if (`KismetStringLibrary.Contains` ResponseText "[CORRECT]")
    (bind _myplayercharacter (`/Game/ThirdPerson/CommonFunctionLibrary.GetMyPlayerCharacter`))
    (`/Game/ThirdPerson/Blueprints/BP_ThirdPersonCharacter.AddKP` _myplayercharacter 15)
    (elif (`KismetStringLibrary.Contains` ResponseText "[PARTIAL]")
      (bind _myplayercharacter_2 (`/Game/ThirdPerson/CommonFunctionLibrary.GetMyPlayerCharacter`))
      (`/Game/ThirdPerson/Blueprints/BP_ThirdPersonCharacter.AddKP` _myplayercharacter_2 5))))

(event `/Game/Dialogue/BPI_Dialogue.Talk`
  (bind _returnvalue (`GameplayStatics.GetPlayerController` 0))
  (bind _ui (`self.UI`))
  ; Event Talk Trigger
  (if (`self.CanTalk?`)
    (set `self.CanTalk?` false)
    ; Use Ai Dialogue
    (if (`self.Use AI Dialogue`)
      (bind _returnvalue_2 (`|CreateWidget` "/Game/Dialogue/WB_Dialogue.WB_Dialogue_C" (`GameplayStatics.GetPlayerController` 0) self))
      (bind _output_get (set `self.UI` _returnvalue_2))
      (`UserWidget.AddToViewport` _output_get 0)
      (if (`self.IsFirstMessage`)
        (bind _full_prompt (`/Game/Blueprints/BP_HttpClient_Component.Build_Opening_Prompt` (`self.BP_HttpClient_Component`) (`self.Current Character ID`) "[The player approaches for the first time]"))
        (`/Game/Blueprints/BP_HttpClient_Component.Send AI Request` (`self.BP_HttpClient_Component`) _full_prompt "" "")
        (`KismetSystemLibrary.Delay` 5.0)
        (set `self.CanTalk?` true)
        (else
          ; No AI Default Dialogue Set
          (bind _historystring (`self.GetFormattedHistory`))
          (bind _full_prompt_2 (`/Game/Blueprints/BP_HttpClient_Component.Build_Followup_Prompt` (`self.BP_HttpClient_Component`) (`self.Current Character ID`) (`self.prompt`) (`KismetStringLibrary.Concat_StrStr` "The player is an adventurer visiting Petra. \nChat History:\n" _historystring)))
          (`/Game/Blueprints/BP_HttpClient_Component.Send AI Request` (`self.BP_HttpClient_Component`) _full_prompt_2 "" "")
          (`KismetSystemLibrary.Delay` 5.0)
          (set `self.CanTalk?` true)))
      (else
        (`/Engine/EditorBlueprintResources/StandardMacros.IncrementInt` (`self.talkIndex`)
          (:`  `
            (if (< (`self.talkIndex`) (`KismetArrayLibrary.Array_Length` (`self.dialogue`)))
              (`self.UI`
                (:`then`
                  _)
                (:`else`
                  (bind _returnvalue_3 (`|CreateWidget` "/Game/Dialogue/WB_Dialogue.WB_Dialogue_C" _returnvalue self))
                  (bind _output_get_2 (set `self.UI` _returnvalue_3))
                  (`UserWidget.AddToViewport` _output_get_2 0)
                  (`WidgetBlueprintLibrary.SetInputMode_GameAndUIEx` _returnvalue _output_get_2 "DoNotLock" false)
                  (set `PlayerController.bShowMouseCursor` true _returnvalue)
                  (`self.EnableInput` (`GameplayStatics.GetPlayerController` 0))))
              (`/Game/Dialogue/WB_Dialogue.AddChatLine` (`self.UI`) (`KismetTextLibrary.Conv_StringToText` (`|GetArrayItem` (`self.dialogue`) (`self.talkIndex`))) false)
              (set `self.CanTalk?` true)
              (else
                (`/Engine/EditorBlueprintResources/StandardMacros.IsValid` _ui
                  (:`Is Valid`
                    (`Widget.RemoveFromParent` _ui)
                    (set `self.UI` null))
                  (:`Is Not Valid`
                    _))
                (set `self.CanTalk?` true)
                (set `self.talkIndex` -1)))))))
    (else
      (`KismetSystemLibrary.Delay` 0.2)
      (`KismetSystemLibrary.PrintString` "I'm thinking, give me a moment")
      (set `self.CanTalk?` true))))

(event `EnhancedInput|/Game/Input/Actions/IA_ExitDialogue`
  (params (ActionValue :type Boolean) (ElapsedSeconds :type "Float (double-precision)") (TriggeredSeconds :type "Float (double-precision)") (InputAction :type "InputAction Object Reference" :default "/Game/Input/Actions/IA_ExitDialogue.IA_ExitDialogue"))
  (:`Triggered`
    (`self.EndDialogue`)))

(event `ReceivePlayerInput`
  (params (InputText :type String))
  ; ReceivePlayerInput
  (bind _myplayercharacter (`/Game/ThirdPerson/CommonFunctionLibrary.GetMyPlayerCharacter`))
  (bind _bgameover (`/Game/ThirdPerson/Blueprints/BP_ThirdPersonCharacter.DeductKP` _myplayercharacter (`/Game/ThirdPerson/Blueprints/BP_ThirdPersonCharacter.KPCostPerQuestion` _myplayercharacter)))
  (if _bgameover
    (bind _returnvalue (`|CreateWidget` "/Game/ThirdPerson/QuestSYstem/UI/WBP_GameOver.WBP_GameOver_C"))
    (`UserWidget.AddToViewport` _returnvalue 0)
    (`GameplayStatics.SetGamePaused` true)
    (else
      (`self.AddToHistory` InputText "Player")
      (bind _historystring (`self.GetFormattedHistory`))
      (bind _full_prompt (`/Game/Blueprints/BP_HttpClient_Component.Build_Followup_Prompt` (`self.BP_HttpClient_Component`) (`self.Current Character ID`) InputText (`KismetStringLibrary.Concat_StrStr` "" _historystring)))
      (if (`self.Use AI Dialogue`)
        (`/Game/Blueprints/BP_HttpClient_Component.Send AI Request` (`self.BP_HttpClient_Component`) _full_prompt "" "")
        (`KismetSystemLibrary.Delay` 5.0)
        (set `self.CanTalk?` true)
        (else
          (`KismetSystemLibrary.PrintString` "I cannot answer that"))))))

(event `EndDialogue`
  (bind _returnvalue (`GameplayStatics.GetPlayerController` 0))
  ; End Dialogue
  (bind _ui (`self.UI`)
    (:`then`
      (`Widget.RemoveFromParent` _ui)
      (`WidgetBlueprintLibrary.SetInputMode_GameOnly` _returnvalue)
      (set `PlayerController.bShowMouseCursor` false _returnvalue)
      (`self.DisableInput` _returnvalue)
      (set `self.CanTalk?` true))
    (:`else`)))

(fn `AddToHistory`
  (params (Message :type String) (Role :type String))
  (`KismetArrayLibrary.Array_Add` (`self.ConversationHistory`) (make `/Game/Dialogue/Structs/S_ChatMessage` Message Role))
  (if (> (`KismetArrayLibrary.Array_Length` (`self.ConversationHistory`)) 30)
    (`KismetArrayLibrary.Array_Remove` (`self.ConversationHistory`))))

(fn `CheckQuestKeywords`
  (params (ResponseText :type String))
  (bind (_keypin _valuepin) (`|MapForEach` (`self.DialogueKeywords`))
    (:`then`
      (if (`KismetStringLibrary.Contains` ResponseText _keypin)
        (if (`KismetStringLibrary.EqualEqual_StrStr` _valuepin "obj_guard_bribe")
          (bind _myplayercharacter (`/Game/ThirdPerson/CommonFunctionLibrary.GetMyPlayerCharacter`))
          (bind _returnvalue (`self.GetComponentByClass` _myplayercharacter "/Game/ThirdPerson/Inventory/BP_InventoryComponent.BP_InventoryComponent_C"))
          (bind _iscollected (`/Game/ThirdPerson/Inventory/BP_InventoryComponent.IsItemCollected` _returnvalue "honeycake"))
          (if _iscollected
            (`/Game/ThirdPerson/Inventory/BP_InventoryComponent.RemoveItem` _returnvalue "honeycake")
            (bind _myplayercharacter_2 (`/Game/ThirdPerson/CommonFunctionLibrary.GetMyPlayerCharacter`))
            (for _array_element (`/Game/ThirdPerson/QuestSYstem/QuestLog_Component.CurrentQuests` (`/Game/ThirdPerson/Blueprints/BP_ThirdPersonCharacter.QuestLog_Component` _myplayercharacter_2))
              (`/Game/ThirdPerson/QuestSYstem/BP_QuestBase.UpdateObjectiveProgress` _array_element _valuepin 1)))
          (else
            (bind _myplayercharacter_3 (`/Game/ThirdPerson/CommonFunctionLibrary.GetMyPlayerCharacter`))
            (for _array_element_2 (`/Game/ThirdPerson/QuestSYstem/QuestLog_Component.CurrentQuests` (`/Game/ThirdPerson/Blueprints/BP_ThirdPersonCharacter.QuestLog_Component` _myplayercharacter_3))
              (`/Game/ThirdPerson/QuestSYstem/BP_QuestBase.UpdateObjectiveProgress` _array_element_2 _valuepin 1))))))))

(fn `GetFormattedHistory`
  (returns (HistoryString :type String))
  (locals (TempHistory :type String))
  (for _array_element (`self.ConversationHistory`)
    (bind (_message _role) (break `/Game/Dialogue/Structs/S_ChatMessage` _array_element))
    (set `local.TempHistory` (`KismetStringLibrary.Concat_StrStr` (`local.TempHistory`) (`KismetStringLibrary.Concat_StrStr` _role ": " _message "\\n"))))
  (return (`local.TempHistory`)))

(fn `RepopulateChatFromHistory`
  (for _array_element (`self.ConversationHistory`)
    (bind (_message _role) (break `/Game/Dialogue/Structs/S_ChatMessage` _array_element))
    (`/Game/Dialogue/WB_Dialogue.AddChatLine` (`self.UI`) (`KismetTextLibrary.Conv_StringToText` _message) (`KismetStringLibrary.EqualEqual_StrStr` _role "Player"))))

(fn `UserConstructionScript`
  (cast `/Game/Blueprints/BP_HttpClient_Component` (`self.GetComponentByClass` self "/Game/Blueprints/BP_HttpClient_Component.BP_HttpClient_Component_C")))