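; Obodas dialogue NPC Blueprint whose AI replies from an HTTP client component drive chat, quest progress and codex unlocks.
; Each reply is logged, shown in chat and keyword-checked, then advances the first matching incomplete objective in each current quest, regardless of content.
; ProcessQuestForCodex maps completed objectives to codex entries, rechecks completed quests every reply, and unlocks a bonus entry when all listed objectives are done.
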(event `self.ReceiveBeginPlay`
  (`parent.ReceiveBeginPlay`)
  (add `/Game/Blueprints/BP_HttpClient_Component.OnAIResponseReceived` (`self.BP_HttpClient_Component`) (delegate `self.OnAIResponseReceived_Event`)))

(event `/Game/Dialogue/BPI_Dialogue.Talk`
  (`parent.Talk`))

(event `self.OnAIResponseReceived_Event`
  (params (ResponseText :type String))
  (`self.AddToHistory` ResponseText "AI")
  (`/Game/Dialogue/WB_Dialogue.AddChatLine` (`self.UI`) (`KismetTextLibrary.Conv_StringToText` ResponseText) false)
  (`self.CheckQuestKeywords` ResponseText)
  (bind _myplayercharacter (`/Game/ThirdPerson/CommonFunctionLibrary.GetMyPlayerCharacter`))
  (bind _returnvalue (`self.GetComponentByClass` _myplayercharacter "/Game/ThirdPerson/QuestSYstem/QuestLog_Component.QuestLog_Component_C"))
  (for _array_element (`/Game/ThirdPerson/QuestSYstem/QuestLog_Component.CurrentQuests` _returnvalue)
    (`/Engine/EditorBlueprintResources/StandardMacros.IsValid` _array_element
      (:`Is Valid`
        (for _array_element_2 (`.Objectives_21_75F1BA2A457170AB65DED5B45FFC78A1` (break `/Game/ThirdPerson/QuestSYstem/StageDetails` (`/Game/ThirdPerson/QuestSYstem/BP_QuestBase.CurrentStageDetails` _array_element)))
          (bind (_objectivename _description _type _objectiveid) (break `/Game/ThirdPerson/QuestSYstem/ObjectiveDetails` _array_element_2))
          (bind _iscomplete (`/Game/ThirdPerson/QuestSYstem/BP_QuestBase.IsObjectiveComplete` _array_element _objectiveid))
          (if (not _iscomplete)
            (if (`KismetArrayLibrary.Array_Contains` (`self.ObjectivesToComplete`) _objectiveid)
              (`/Game/ThirdPerson/QuestSYstem/BP_QuestBase.UpdateObjectiveProgress` _array_element _objectiveid 1)
              (`self.ProcessQuestForCodex` _array_element)
              (break)))))))
  (for _array_element_3 (`/Game/ThirdPerson/QuestSYstem/QuestLog_Component.CompletedQuestActors` _returnvalue)
    (`self.ProcessQuestForCodex` _array_element_3)))

(fn `ProcessQuestForCodex`
  (params (QuestActor :type "/Game/ThirdPerson/QuestSYstem/BP_QuestBase Object Reference"))
  (bind _returnvalue (`self.GetComponentByClass` (`GameplayStatics.GetPlayerCharacter` 0) "/Game/ThirdPerson/Codex/BP_CodexSystem.BP_CodexSystem_C"))
  (bind (_value _returnvalue_2) (`BlueprintMapLibrary.Map_Find` (`self.QuestToCodexMap`) "obj_bonus"))
  (set `self.CompletedCount` 0)
  (for _array_element (`self.ObjectivesToComplete`)
    (bind _iscomplete (`/Game/ThirdPerson/QuestSYstem/BP_QuestBase.IsObjectiveComplete` QuestActor _array_element))
    (if _iscomplete
      (set `self.CompletedCount` (+ (`self.CompletedCount`) 1))
      (bind (_value_2 _returnvalue_3) (`BlueprintMapLibrary.Map_Find` (`self.QuestToCodexMap`) _array_element))
      (if _returnvalue_3
        (`/Engine/EditorBlueprintResources/StandardMacros.IsValid` _returnvalue
          (:`Is Valid`
            (`/Game/ThirdPerson/Codex/BP_CodexSystem.UnlockEntry` _returnvalue _value_2))))))
  (if (== (`self.CompletedCount`) (`KismetArrayLibrary.Array_Length` (`self.ObjectivesToComplete`)))
    (if _returnvalue_2
      (`/Game/ThirdPerson/Codex/BP_CodexSystem.UnlockEntry` (`self.GetComponentByClass` (`GameplayStatics.GetPlayerCharacter` 0) "/Game/ThirdPerson/Codex/BP_CodexSystem.BP_CodexSystem_C") _value))))

(fn `UserConstructionScript`
  (`parent.UserConstructionScript`))