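; Obodas, a Petra merchant NPC who teaches Nabataean trade lore, then quizzes the player for Knowledge Points and quest objectives.
; A DialogueStage counter drives WB_Dialogue text and options; quiz answers are string-matched, adjust KP and advance the stage.
; Free-typed quiz questions cost KP (game over if DeductKP returns true) and go to an AI HTTP client with chat history.
; AI responses also advance matching quest objectives and unlock mapped codex entries.
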(event `self.ReceivePlayerInput`
  (params (InputText :type String))
  (bind _ui (`self.UI`))
  (bind _ui_2 (`self.UI`))
  (bind _dialoguestage (`self.DialogueStage`))
  (bind _bp_httpclient_component (`self.BP_HttpClient_Component`))
  ; ReceivePlayerInput
  (`/Game/Dialogue/WB_Dialogue.AddChatLine` _ui_2 (`KismetTextLibrary.Conv_StringToText` InputText) true)
  (if (< _dialoguestage 3)
    (if (or (or (== InputText "I think I understand, test me!") (== InputText "Fascinating! Test my knowledge!")) (== InputText "I'm ready to be tested!"))
      (set `self.DialogueStage` 3)
      (set `self.HasCompletedTeaching` true)
      (`/Game/Dialogue/WB_Dialogue.AddChatLine` _ui_2 (`KismetTextLibrary.Conv_StringToText` "Excellent! You are ready for the quiz!") false)
      (`self.ShowCurrentDialogueStage`)
      (elif (== InputText "I need to hear that again")
        (`self.ShowCurrentDialogueStage`)
        (else
          (set `self.DialogueStage` (+ _dialoguestage 1))
          (`self.ShowCurrentDialogueStage`))))
    (elif (== InputText "Ask Obodas for a hint")
      (`Widget.SetVisibility` (`/Game/Dialogue/WB_Dialogue.InputBox_Border` _ui) "SelfHitTestInvisible")
      (`Widget.SetKeyboardFocus` (`/Game/Dialogue/WB_Dialogue.InputBox` _ui))
      (elif (`KismetArrayLibrary.Array_Contains` (`self.QuizOptions`) InputText)
        (`self.HandleQuizAnswer` InputText)
        (else
          (`/Game/Dialogue/WB_Dialogue.AddChatLine` (`self.UI`) (`KismetTextLibrary.Conv_StringToText` "⚠ Warning: Using AI help costs Knowledge Points!") false)
          (set `self.UsedAIHelp` true)
          (bind _myplayercharacter (`/Game/ThirdPerson/CommonFunctionLibrary.GetMyPlayerCharacter`))
          (bind _bgameover (`/Game/ThirdPerson/Blueprints/BP_ThirdPersonCharacter.DeductKP` _myplayercharacter (`/Game/ThirdPerson/Blueprints/BP_ThirdPersonCharacter.KPCostPerQuestion` _myplayercharacter)))
          (if _bgameover
            (bind _returnvalue (`|CreateWidget` "/Game/ThirdPerson/QuestSYstem/UI/WBP_GameOver.WBP_GameOver_C" (`GameplayStatics.GetPlayerController` 0)))
            (`UserWidget.AddToViewport` _returnvalue 0)
            (`GameplayStatics.SetGamePaused` true)
            (else
              (`self.AddToHistory` InputText "Player")
              (bind _historystring (`self.GetFormattedHistory`))
              (bind _full_prompt (`/Game/Blueprints/BP_HttpClient_Component.Build_Followup_Prompt` _bp_httpclient_component (`self.Current Character ID`) InputText (`KismetStringLibrary.Concat_StrStr` "The player is asking about Petra trade. Chat History:\n" _historystring)))
              (`/Game/Blueprints/BP_HttpClient_Component.Send AI Request` _bp_httpclient_component _full_prompt "OnAIResponseReceived_Event" ""))))))))

(event `self.Talk`
  (bind _returnvalue (`GameplayStatics.GetPlayerController` 0))
  (if (`self.CanTalk?`)
    (set `self.CanTalk?` false)
    (bind _returnvalue_2 (`|CreateWidget` "/Game/Dialogue/WB_Dialogue.WB_Dialogue_C" _returnvalue self))
    (bind _output_get (set `self.UI` _returnvalue_2))
    (`UserWidget.AddToViewport` _output_get 0)
    (`WidgetBlueprintLibrary.SetInputMode_GameAndUIEx` _returnvalue _output_get "DoNotLock" false)
    (set `PlayerController.bShowMouseCursor` true _returnvalue)
    (`self.ShowCurrentDialogueStage`)))

(event `ShowCurrentDialogueStage`
  (bind _ui (`self.UI`))
  (bind _ui_2 (`self.UI`))
  (bind _ui_3 (`self.UI`))
  (bind _ui_4 (`self.UI`))
  (bind _ui_5 (`self.UI`))
  (bind _ui_6 (`self.UI`))
  (bind _dialoguestage (`self.DialogueStage`))
  (bind _ui_7 (`self.UI`))
  (if (== _dialoguestage 0)
    (`/Game/Dialogue/WB_Dialogue.AddChatLine` _ui_7 (`KismetTextLibrary.Conv_StringToText` (`KismetStringLibrary.Concat_StrStr` "Welcome, traveler! I am Obodas, a merchant who has walked every trade road from Yemen to Rome. Let me share secrets that only the wisest traders know..." "Did you know that a single camel load of frankincense was worth enough to buy a house in Rome? he incense trade made Petra wealthier than many kingdoms.")) false)
    (`/Game/Dialogue/WB_Dialogue.SetDialogueOptions` _ui_7 "Tell me about the trade routes" "What about the dangers?" "I need to hear that again")
    (`/Game/Dialogue/WB_Dialogue.ShowOptionsPanel` _ui_7)
    (elif (== _dialoguestage 1)
      (`/Game/Dialogue/WB_Dialogue.AddChatLine` _ui_7 (`KismetTextLibrary.Conv_StringToText` "The Nabataeans had a secret tax — not gold, but knowledge. Every caravan that passed through had to share the location of hidden water springs. This is how the Nabataeans built the greatest water map of the ancient world.") false)
      (`/Game/Dialogue/WB_Dialogue.SetDialogueOptions` _ui_7 "Tell me about Al-Khazneh" "What about Nabataean engineering?" "I need to hear that again")
      (`/Game/Dialogue/WB_Dialogue.ShowOptionsPanel` _ui_7)
      (elif (== _dialoguestage 2)
        (`/Game/Dialogue/WB_Dialogue.AddChatLine` _ui_7 (`KismetTextLibrary.Conv_StringToText` "The Treasury — Al-Khazneh — was never a treasury at all! It was a royal tomb, carved directly into the cliff face. But clever traders used its inner chambers to store contracts and trade agreements, safe from thieves.") false)
        (`/Game/Dialogue/WB_Dialogue.AddChatLine` _ui_7 (`KismetTextLibrary.Conv_StringToText` "The Nabataeans invented an ingenious system of ceramic pipelines — thin clay pipes that carried water across miles of desert. This engineering marvel meant their cities could thrive where no others could survive.") false)
        (`/Game/Dialogue/WB_Dialogue.AddChatLine` _ui_7 (`KismetTextLibrary.Conv_StringToText` "And here is a secret few know: Petra controlled the bitumen trade from the Dead Sea. The Romans desperately needed bitumen to waterproof their mighty warships. Without Petra, Rome's navy would have rotted in the harbors!") false)
        (`/Game/Dialogue/WB_Dialogue.SetDialogueOptions` _ui_7 "Fascinating! Test my knowledge!" "Tell me more about Petra's exports" "I need to hear that again")
        (`/Game/Dialogue/WB_Dialogue.ShowOptionsPanel` _ui_7)
        (`Widget.SetVisibility` (`/Game/Dialogue/WB_Dialogue.BTN_Option4` _ui_6) "Visible")
        (`TextBlock.SetText` (`/Game/Dialogue/WB_Dialogue.Txt_Option4` _ui_6) "Ask Obodas for a hint")
        (elif (== _dialoguestage 3)
          (`/Game/Dialogue/WB_Dialogue.AddChatLine` _ui_7 (`KismetTextLibrary.Conv_StringToText` "Now let us test your knowledge! How valuable was frankincense compared to other goods?") false)
          (`/Game/Dialogue/WB_Dialogue.SetDialogueOptions` _ui_7 "A camel load could buy a house in Rome" "It was cheaper than pottery" "It had no value outside Arabia")
          (`/Game/Dialogue/WB_Dialogue.ShowOptionsPanel` _ui_7)
          (`Widget.SetVisibility` (`/Game/Dialogue/WB_Dialogue.InputBox_Border` _ui_7) "SelfHitTestInvisible")
          (`Widget.SetVisibility` (`/Game/Dialogue/WB_Dialogue.BTN_Option4` _ui) "Visible")
          (`TextBlock.SetText` (`/Game/Dialogue/WB_Dialogue.Txt_Option4` _ui) "Ask Obodas for a hint")
          (elif (== _dialoguestage 4)
            (`/Game/Dialogue/WB_Dialogue.AddChatLine` _ui_7 (`KismetTextLibrary.Conv_StringToText` "What secret 'tax' did the Nabataeans charge caravans passing through?") false)
            (`/Game/Dialogue/WB_Dialogue.SetDialogueOptions` _ui_7 "Knowledge of hidden water sources" "Gold coins" "Spice samples")
            (`/Game/Dialogue/WB_Dialogue.ShowOptionsPanel` _ui_7)
            (`Widget.SetVisibility` (`/Game/Dialogue/WB_Dialogue.InputBox_Border` _ui_7) "SelfHitTestInvisible")
            (`Widget.SetVisibility` (`/Game/Dialogue/WB_Dialogue.BTN_Option4` _ui_2) "Visible")
            (`TextBlock.SetText` (`/Game/Dialogue/WB_Dialogue.Txt_Option4` _ui_2) "Ask Obodas for a hint")
            (elif (== _dialoguestage 5)
              (`/Game/Dialogue/WB_Dialogue.AddChatLine` _ui_7 (`KismetTextLibrary.Conv_StringToText` "What was Al-Khazneh — the famous Treasury — actually built as?") false)
              (`/Game/Dialogue/WB_Dialogue.SetDialogueOptions` _ui_7 "A royal tomb" "A bank vault" "A temple to Zeus")
              (`/Game/Dialogue/WB_Dialogue.ShowOptionsPanel` _ui_7)
              (`Widget.SetVisibility` (`/Game/Dialogue/WB_Dialogue.InputBox_Border` _ui_7) "SelfHitTestInvisible")
              (`Widget.SetVisibility` (`/Game/Dialogue/WB_Dialogue.BTN_Option4` _ui_3) "Visible")
              (`TextBlock.SetText` (`/Game/Dialogue/WB_Dialogue.Txt_Option4` _ui_3) "Ask Obodas for a hint")
              (elif (== _dialoguestage 6)
                (`/Game/Dialogue/WB_Dialogue.AddChatLine` _ui_7 (`KismetTextLibrary.Conv_StringToText` "How did the Nabataeans transport water across miles of desert?") false)
                (`/Game/Dialogue/WB_Dialogue.SetDialogueOptions` _ui_7 "Ceramic pipeline systems" "Underground rivers" "Carried by camels")
                (`/Game/Dialogue/WB_Dialogue.ShowOptionsPanel` _ui_7)
                (`Widget.SetVisibility` (`/Game/Dialogue/WB_Dialogue.InputBox_Border` _ui_7) "SelfHitTestInvisible")
                (`Widget.SetVisibility` (`/Game/Dialogue/WB_Dialogue.BTN_Option4` _ui_4) "Visible")
                (`TextBlock.SetText` (`/Game/Dialogue/WB_Dialogue.Txt_Option4` _ui_4) "Ask Obodas for a hint")
                (elif (== _dialoguestage 7)
                  (`/Game/Dialogue/WB_Dialogue.AddChatLine` _ui_7 (`KismetTextLibrary.Conv_StringToText` "Final question! Why did Rome desperately need Petra's bitumen?") false)
                  (`/Game/Dialogue/WB_Dialogue.SetDialogueOptions` _ui_7 "To waterproof their ships" "To build roads" "To make weapons")
                  (`/Game/Dialogue/WB_Dialogue.ShowOptionsPanel` _ui_7)
                  (`Widget.SetVisibility` (`/Game/Dialogue/WB_Dialogue.InputBox_Border` _ui_7) "SelfHitTestInvisible")
                  (`Widget.SetVisibility` (`/Game/Dialogue/WB_Dialogue.BTN_Option4` _ui_5) "Visible")
                  (`TextBlock.SetText` (`/Game/Dialogue/WB_Dialogue.Txt_Option4` _ui_5) "Ask Obodas for a hint")
                  (else
                    (`/Game/Dialogue/WB_Dialogue.AddChatLine` _ui_7 (`KismetTextLibrary.Conv_StringToText` "Well done, traveler! You have proven your knowledge of Petra's trade. Go forth with wisdom!") false)
                    (bind _myplayercharacter (`/Game/ThirdPerson/CommonFunctionLibrary.GetMyPlayerCharacter`))
                    (`/Game/ThirdPerson/Blueprints/BP_ThirdPersonCharacter.AddKP` _myplayercharacter 25)
                    (`self.CompleteSpecificObjective` "obj_bonus")
                    (set `self.CanTalk?` true)))))))))))

(event `self.OnAIResponseReceived_Event`
  (params (ResponseText :type String))
  (`self.AddToHistory` ResponseText "AI")
  (`/Game/Dialogue/WB_Dialogue.AddChatLine` (`self.UI`) (`KismetTextLibrary.Conv_StringToText` ResponseText) false)
  (`self.CheckQuestKeywords` ResponseText)
  (bind _myplayercharacter (`/Game/ThirdPerson/CommonFunctionLibrary.GetMyPlayerCharacter`))
  (bind _returnvalue (`self.GetComponentByClass` _myplayercharacter "/Game/ThirdPerson/QuestSYstem/QuestLog_Component.QuestLog_Component_C"))
  (for _array_element (`/Game/ThirdPerson/QuestSYstem/QuestLog_Component.CurrentQuests` _returnvalue)
    (`/Engine/EditorBlueprintResources/StandardMacros.IsValid` _array_element
      (:`Is Valid`
        (for _array_element_2 (`.Objectives_21_75F1BA2A457170AB65DED5B45FFC78A1` (break `/Game/ThirdPerson/QuestSYstem/StageDetails` (`/Game/ThirdPerson/QuestSYstem/BP_QuestBase.CurrentStageDetails` _array_element)))
          (bind (_objectivename _description _type _objectiveid) (break `/Game/ThirdPerson/QuestSYstem/ObjectiveDetails` _array_element_2))
          (bind _iscomplete (`/Game/ThirdPerson/QuestSYstem/BP_QuestBase.IsObjectiveComplete` _array_element _objectiveid))
          (if (not _iscomplete)
            (if (`KismetArrayLibrary.Array_Contains` (`self.ObjectivesToComplete`) _objectiveid)
              (`/Game/ThirdPerson/QuestSYstem/BP_QuestBase.UpdateObjectiveProgress` _array_element _objectiveid 1)
              (`self.ProcessQuestForCodex` _array_element)
              (break)))))))
  (for _array_element_3 (`/Game/ThirdPerson/QuestSYstem/QuestLog_Component.CompletedQuestActors` _returnvalue)
    (`self.ProcessQuestForCodex` _array_element_3))
  (`KismetSystemLibrary.Delay` 5.0)
  (`self.ShowCurrentDialogueStage`))

(event `self.ReceiveBeginPlay`
  (`parent.ReceiveBeginPlay`)
  (add `/Game/Blueprints/BP_HttpClient_Component.OnAIResponseReceived` (`self.BP_HttpClient_Component`) (delegate `self.OnAIResponseReceived_Event`)))

(fn `CompleteSpecificObjective`
  (params (ObjectiveID :type String))
  (bind _myplayercharacter (`/Game/ThirdPerson/CommonFunctionLibrary.GetMyPlayerCharacter`))
  (for _array_element (`/Game/ThirdPerson/QuestSYstem/QuestLog_Component.CurrentQuests` (`self.GetComponentByClass` _myplayercharacter "/Game/ThirdPerson/QuestSYstem/QuestLog_Component.QuestLog_Component_C"))
    (`/Game/ThirdPerson/QuestSYstem/BP_QuestBase.UpdateObjectiveProgress` _array_element ObjectiveID 1)))

(fn `HandleQuizAnswer`
  (params (AnswerText :type String))
  (bind _dialoguestage (`self.DialogueStage`))
  (bind _ui (`self.UI`))
  (bind _kprewardpercorrect (`self.KPRewardPerCorrect`))
  (bind _kppenaltyperwrong (`self.KPPenaltyPerWrong`))
  (if (== _dialoguestage 3)
    (`|ExecutionSequence`
      (:`then_0`
        (if (`KismetStringLibrary.EqualEqual_StrStr` AnswerText "A camel load could buy a house in Rome")
          (bind _myplayercharacter (`/Game/ThirdPerson/CommonFunctionLibrary.GetMyPlayerCharacter`))
          (`/Game/ThirdPerson/Blueprints/BP_ThirdPersonCharacter.AddKP` _myplayercharacter _kprewardpercorrect)
          (`self.CompleteSpecificObjective` "obj_01")
          (`/Game/Dialogue/WB_Dialogue.AddChatLine` _ui (`KismetTextLibrary.Conv_StringToText` "Correct! Frankincense was worth more than gold to the Romans. +15 KP!") false)
          (else
            (bind _myplayercharacter_2 (`/Game/ThirdPerson/CommonFunctionLibrary.GetMyPlayerCharacter`))
            (`/Game/ThirdPerson/Blueprints/BP_ThirdPersonCharacter.DeductKP` _myplayercharacter_2 _kppenaltyperwrong)
            (`/Game/Dialogue/WB_Dialogue.AddChatLine` _ui (`KismetTextLibrary.Conv_StringToText` "Not quite... A single camel load could buy a house in Rome! -5 KP!") false))))
      (:`then_1`
        (set `self.DialogueStage` (+ _dialoguestage 1))
        (`self.ShowCurrentDialogueStage`)))
    (elif (== _dialoguestage 4)
      (`|ExecutionSequence`
        (:`then_0`
          (if (`KismetStringLibrary.EqualEqual_StrStr` AnswerText "Knowledge of hidden water sources")
            (bind _myplayercharacter_3 (`/Game/ThirdPerson/CommonFunctionLibrary.GetMyPlayerCharacter`))
            (`/Game/ThirdPerson/Blueprints/BP_ThirdPersonCharacter.AddKP` _myplayercharacter_3 _kprewardpercorrect)
            (`self.CompleteSpecificObjective` "obj_02")
            (`/Game/Dialogue/WB_Dialogue.AddChatLine` _ui (`KismetTextLibrary.Conv_StringToText` "Correct! Water knowledge was the most valuable currency in the desert. +15 KP!") false)
            (else
              (bind _myplayercharacter_4 (`/Game/ThirdPerson/CommonFunctionLibrary.GetMyPlayerCharacter`))
              (`/Game/ThirdPerson/Blueprints/BP_ThirdPersonCharacter.DeductKP` _myplayercharacter_4 _kppenaltyperwrong)
              (`/Game/Dialogue/WB_Dialogue.AddChatLine` _ui (`KismetTextLibrary.Conv_StringToText` "Not quite... The Nabataeans demanded knowledge of hidden water springs. -5 KP!") false))))
        (:`then_1`
          (set `self.DialogueStage` (+ _dialoguestage 1))
          (`self.ShowCurrentDialogueStage`)))
      (elif (== _dialoguestage 5)
        (`|ExecutionSequence`
          (:`then_0`
            (if (`KismetStringLibrary.EqualEqual_StrStr` AnswerText "A royal tomb")
              (bind _myplayercharacter_5 (`/Game/ThirdPerson/CommonFunctionLibrary.GetMyPlayerCharacter`))
              (`/Game/ThirdPerson/Blueprints/BP_ThirdPersonCharacter.AddKP` _myplayercharacter_5 _kprewardpercorrect)
              (`self.CompleteSpecificObjective` "obj_03")
              (`/Game/Dialogue/WB_Dialogue.AddChatLine` _ui (`KismetTextLibrary.Conv_StringToText` "Correct! Al-Khazneh was carved as a royal tomb, not a treasury. +15 KP!") false)
              (else
                (bind _myplayercharacter_6 (`/Game/ThirdPerson/CommonFunctionLibrary.GetMyPlayerCharacter`))
                (`/Game/ThirdPerson/Blueprints/BP_ThirdPersonCharacter.DeductKP` _myplayercharacter_6 _kppenaltyperwrong)
                (`/Game/Dialogue/WB_Dialogue.AddChatLine` _ui (`KismetTextLibrary.Conv_StringToText` "	Not quite... Al-Khazneh was actually a royal tomb. -5 KP!") false))))
          (:`then_1`
            (set `self.DialogueStage` (+ _dialoguestage 1))
            (`self.ShowCurrentDialogueStage`)))
        (elif (== _dialoguestage 6)
          (`|ExecutionSequence`
            (:`then_0`
              (if (`KismetStringLibrary.EqualEqual_StrStr` AnswerText "Ceramic pipeline systems")
                (bind _myplayercharacter_7 (`/Game/ThirdPerson/CommonFunctionLibrary.GetMyPlayerCharacter`))
                (`/Game/ThirdPerson/Blueprints/BP_ThirdPersonCharacter.AddKP` _myplayercharacter_7 _kprewardpercorrect)
                (`self.CompleteSpecificObjective` "obj_04")
                (`/Game/Dialogue/WB_Dialogue.AddChatLine` _ui (`KismetTextLibrary.Conv_StringToText` "Correct! Their ceramic pipes were an engineering marvel. +15 KP!") false)
                (else
                  (bind _myplayercharacter_8 (`/Game/ThirdPerson/CommonFunctionLibrary.GetMyPlayerCharacter`))
                  (`/Game/ThirdPerson/Blueprints/BP_ThirdPersonCharacter.DeductKP` _myplayercharacter_8 _kppenaltyperwrong)
                  (`/Game/Dialogue/WB_Dialogue.AddChatLine` _ui (`KismetTextLibrary.Conv_StringToText` "Not quite... They used ingenious ceramic pipeline systems. -5 KP!") false))))
            (:`then_1`
              (set `self.DialogueStage` (+ _dialoguestage 1))
              (`self.ShowCurrentDialogueStage`)))
          (elif (== _dialoguestage 7)
            (`|ExecutionSequence`
              (:`then_0`
                (if (`KismetStringLibrary.EqualEqual_StrStr` AnswerText "To waterproof their ships")
                  (bind _myplayercharacter_9 (`/Game/ThirdPerson/CommonFunctionLibrary.GetMyPlayerCharacter`))
                  (`/Game/ThirdPerson/Blueprints/BP_ThirdPersonCharacter.AddKP` _myplayercharacter_9 _kprewardpercorrect)
                  (`self.CompleteSpecificObjective` "obj_05")
                  (`/Game/Dialogue/WB_Dialogue.AddChatLine` _ui (`KismetTextLibrary.Conv_StringToText` "Correct! Without Petra's bitumen, Rome's navy would have rotted! +15 KP!") false)
                  (else
                    (bind _myplayercharacter_10 (`/Game/ThirdPerson/CommonFunctionLibrary.GetMyPlayerCharacter`))
                    (`/Game/ThirdPerson/Blueprints/BP_ThirdPersonCharacter.DeductKP` _myplayercharacter_10 _kppenaltyperwrong)
                    (`/Game/Dialogue/WB_Dialogue.AddChatLine` _ui (`KismetTextLibrary.Conv_StringToText` "Not quite... Rome needed bitumen to waterproof their warships. -5 KP!") false))))
              (:`then_1`
                (set `self.DialogueStage` (+ _dialoguestage 1))
                (`self.ShowCurrentDialogueStage`)))))))))

(fn `ProcessQuestForCodex`
  (params (QuestActor :type "/Game/ThirdPerson/QuestSYstem/BP_QuestBase Object Reference"))
  (bind _returnvalue (`self.GetComponentByClass` (`GameplayStatics.GetPlayerCharacter` 0) "/Game/ThirdPerson/Codex/BP_CodexSystem.BP_CodexSystem_C"))
  (bind (_value _returnvalue_2) (`BlueprintMapLibrary.Map_Find` (`self.QuestToCodexMap`) "obj_bonus"))
  (set `self.CompletedCount` 0)
  (for _array_element (`self.ObjectivesToComplete`)
    (bind _iscomplete (`/Game/ThirdPerson/QuestSYstem/BP_QuestBase.IsObjectiveComplete` QuestActor _array_element))
    (if _iscomplete
      (set `self.CompletedCount` (+ (`self.CompletedCount`) 1))
      (bind (_value_2 _returnvalue_3) (`BlueprintMapLibrary.Map_Find` (`self.QuestToCodexMap`) _array_element))
      (if _returnvalue_3
        (`/Engine/EditorBlueprintResources/StandardMacros.IsValid` _returnvalue
          (:`Is Valid`
            (`/Game/ThirdPerson/Codex/BP_CodexSystem.UnlockEntry` _returnvalue _value_2))))))
  (if (== (`self.CompletedCount`) (`KismetArrayLibrary.Array_Length` (`self.ObjectivesToComplete`)))
    (if _returnvalue_2
      (`/Game/ThirdPerson/Codex/BP_CodexSystem.UnlockEntry` (`self.GetComponentByClass` (`GameplayStatics.GetPlayerCharacter` 0) "/Game/ThirdPerson/Codex/BP_CodexSystem.BP_CodexSystem_C") _value))))

(fn `UserConstructionScript`
  (`parent.UserConstructionScript`))