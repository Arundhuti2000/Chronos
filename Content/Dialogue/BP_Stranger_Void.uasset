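; The Stranger NPC in the Void, who hands out main-story quests and triggers the game's ending.
; One second after BeginPlay, it reads the player's completion flags and QuestLog to add the Void intro, remaining-world intro or final quest.
; With the final quest, Talk advances the first current quest's objective and shows the game-complete widget.
; Otherwise parent dialogue runs, restoring game input and crediting the talk objective when finished.
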(event `self.ReceiveBeginPlay`
  (`parent.ReceiveBeginPlay`)
  (bind _myplayercharacter (`/Game/ThirdPerson/CommonFunctionLibrary.GetMyPlayerCharacter`))
  (`KismetSystemLibrary.Delay` 1.0)
  (if (and (`/Game/ThirdPerson/Blueprints/BP_ThirdPersonCharacter.bIsGreeceDone` _myplayercharacter) (`/Game/ThirdPerson/Blueprints/BP_ThirdPersonCharacter.bIsPetraDone` _myplayercharacter))
    (bind _returnvalue (`self.GetComponentByClass` _myplayercharacter "/Game/ThirdPerson/QuestSYstem/QuestLog_Component.QuestLog_Component_C"))
    (`/Game/ThirdPerson/QuestSYstem/QuestLog_Component.AddNewQuest` _returnvalue "MainQuestFinal")
    (set `self.DialogueStage` 1)
    (elif (`/Game/ThirdPerson/QuestSYstem/QuestLog_Component.QueryActiveQuest` _returnvalue "MainQuestFinal")
      (set `self.DialogueStage` 1)
      (else
        (bind _returnvalue_2 (`KismetArrayLibrary.Array_Contains` (`/Game/ThirdPerson/QuestSYstem/QuestLog_Component.Completed` _returnvalue) "GreeceToVoidQuest"))
        (bind _returnvalue_3 (`KismetArrayLibrary.Array_Contains` (`/Game/ThirdPerson/QuestSYstem/QuestLog_Component.Completed` _returnvalue) "PetraToVoidQuest"))
        (if (and _returnvalue_2 _returnvalue_3)
          (`/Game/ThirdPerson/QuestSYstem/QuestLog_Component.AddNewQuest` _returnvalue "MainQuestFinal")
          (set `self.DialogueStage` 1)
          (elif _returnvalue_3
            (`/Game/ThirdPerson/QuestSYstem/QuestLog_Component.AddNewQuest` _returnvalue "GreeceIntroQuest")
            (elif _returnvalue_2
              (`/Game/ThirdPerson/QuestSYstem/QuestLog_Component.AddNewQuest` _returnvalue "IntroQuest00")
              (elif (`/Game/ThirdPerson/QuestSYstem/QuestLog_Component.QueryActiveQuest` _returnvalue "VoidIntroQuest")
                _
                (elif (not (`KismetArrayLibrary.Array_Contains` (`/Game/ThirdPerson/QuestSYstem/QuestLog_Component.Completed` _returnvalue) "VoidIntroQuest"))
                  (`KismetSystemLibrary.PrintString` "Void Intro Quest being added for the firsdt time")
                  (`/Game/ThirdPerson/QuestSYstem/QuestLog_Component.AddNewQuest` _returnvalue "VoidIntroQuest"))))))))))

(event `self.ReceiveActorBeginOverlap`
  (params (OtherActor :type "Actor Object Reference")))

(event `self.Talk`
  (bind _returnvalue (`GameplayStatics.GetPlayerController` 0))
  (bind _returnvalue_2 (`GameplayStatics.GetPlayerController` 0))
  (if (== (`self.DialogueStage`) 1)
    (bind _myplayercharacter (`/Game/ThirdPerson/CommonFunctionLibrary.GetMyPlayerCharacter`))
    (`/Game/ThirdPerson/QuestSYstem/BP_QuestBase.UpdateObjectiveProgress` (`|GetArrayItem` (`/Game/ThirdPerson/QuestSYstem/QuestLog_Component.CurrentQuests` (`/Game/ThirdPerson/Blueprints/BP_ThirdPersonCharacter.QuestLog_Component` _myplayercharacter))) "obj_final_talk_stranger" 1)
    (bind _returnvalue_3 (`|CreateWidget` "/Game/ThirdPerson/QuestSYstem/UI/WBP_GameComplete.WBP_GameComplete_C"))
    (`UserWidget.AddToViewport` _returnvalue_3 0)
    (`WidgetBlueprintLibrary.SetInputMode_UIOnlyEx` _returnvalue_2 null)
    (set `PlayerController.bShowMouseCursor` true _returnvalue_2)
    (set `self.DialogueStage` 2)
    (else
      (`parent.Talk`)
      (if (== (`self.talkIndex`) -1)
        (`WidgetBlueprintLibrary.SetInputMode_GameOnly` _returnvalue)
        (set `PlayerController.bShowMouseCursor` false _returnvalue)
        (set `self.CanTalk?` true)
        (bind _myplayercharacter_2 (`/Game/ThirdPerson/CommonFunctionLibrary.GetMyPlayerCharacter`))
        (for _array_element (`/Game/ThirdPerson/QuestSYstem/QuestLog_Component.CurrentQuests` (`self.GetComponentByClass` _myplayercharacter_2 "/Game/ThirdPerson/QuestSYstem/QuestLog_Component.QuestLog_Component_C"))
          (`/Game/ThirdPerson/QuestSYstem/BP_QuestBase.UpdateObjectiveProgress` _array_element "obj_void_talk_stranger" 1))))))

(fn `UserConstructionScript`
  (`parent.UserConstructionScript`))