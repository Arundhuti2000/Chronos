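; Aspasia, priestess NPC at the Parthenon, who teaches Athenian lore, quizzes the player and takes back the stolen golden owl.
; Talk opens WB_Dialogue by DialogueStage; PlayerInput matches option text to scripted voiced replies, completing quest objectives and unlocking codex entries.
; A staged quiz awards or deducts KP, showing Game Over when a deduction returns true.
; Quiz hints send free-text questions to an AI over HTTP, costing KP.
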(event `self.ReceivePlayerInput`
  (params (InputText :type String))
  (bind _returnvalue (`GameplayStatics.GetPlayerController` 0))
  (bind _bp_httpclient_component (`self.BP_HttpClient_Component`))
  (bind _ui (`self.UI`))
  (bind _ui_2 (`self.UI`))
  (`/Engine/EditorBlueprintResources/StandardMacros.IsValid` (`self.CurrentAudioComponent`)
    (:`Is Valid`
      (`AudioComponent.Stop` (`self.CurrentAudioComponent`)))
    (:`Is Not Valid`
      _))
  (`/Game/Dialogue/WB_Dialogue.AddChatLine` _ui (`KismetTextLibrary.Conv_StringToText` InputText) true)
  (if (`self.IsAwaitingHintInput`)
    (set `self.IsAwaitingHintInput` false)
    (`Widget.SetVisibility` (`/Game/Dialogue/WB_Dialogue.InputBox_Border` _ui) "SelfHitTestInvisible")
    (bind _full_prompt (`/Game/Blueprints/BP_HttpClient_Component.Build_Followup_Prompt` _bp_httpclient_component "aspasia" (`KismetStringLibrary.Concat_StrStr` (`KismetStringLibrary.Concat_StrStr` "The player is asking for a hint during a quiz about: " (`self.Current Quiz Question`)) InputText) ""))
    (`/Game/Blueprints/BP_HttpClient_Component.Send AI Request` _bp_httpclient_component _full_prompt "" "")
    (elif (`KismetStringLibrary.EqualEqual_StrStr` InputText "What is this temple?")
      (`/Game/Dialogue/WB_Dialogue.AddChatLine` _ui (`KismetTextLibrary.Conv_StringToText` "This is the Parthenon — the greatest temple ever built. It was constructed atop the Acropolis by order of Pericles himself, during the golden age of Athens. Every column, every sculpture, was designed to honor Athena Parthenos — the virgin goddess who protects our city.") false)
      (bind _returnvalue_2 (`GameplayStatics.SpawnSound2D` "/Game/Audio/Aspasia/Aspasia_Parthenon.Aspasia_Parthenon" 1.0 1.0 0.0 null))
      (set `self.CurrentAudioComponent` _returnvalue_2)
      (`self.CompleteSpecificObjective` "obj_greece_learn_temple")
      (bind _myplayercharacter (`/Game/ThirdPerson/CommonFunctionLibrary.GetMyPlayerCharacter`))
      (`/Game/ThirdPerson/Codex/BP_CodexSystem.UnlockEntry` (`self.GetComponentByClass` _myplayercharacter "/Game/ThirdPerson/Codex/BP_CodexSystem.BP_CodexSystem_C") (`KismetStringLibrary.Conv_StringToName` (`BlueprintMapLibrary.Map_Find` (`self.QuestToCodexMap`) "obj_greece_learn_temple")))
      (set `self.DialogueStage` 1)
      (`/Game/Dialogue/WB_Dialogue.SetDialogueOptions` _ui "Who is Athena?" "What is the Panathenaic festival?" "Tell me about the golden owl")
      (`/Game/Dialogue/WB_Dialogue.ShowOptionsPanel` _ui)
      (elif (`KismetStringLibrary.EqualEqual_StrStr` InputText "Who is Athena?")
        (`/Game/Dialogue/WB_Dialogue.AddChatLine` _ui (`KismetTextLibrary.Conv_StringToText` "Athena is the patron goddess of Athens — goddess of wisdom, courage, and strategic warfare. She sprang fully armored from the head of Zeus himself. The great statue inside this temple — the Athena Parthenos, built by the sculptor Phidias — stands forty feet tall, covered in gold and ivory.") false)
        (bind _returnvalue_3 (`GameplayStatics.SpawnSound2D` "/Game/Audio/Aspasia/Aspasia_athenaStatue.Aspasia_athenaStatue" 1.0 1.0 0.0 null))
        (set `self.CurrentAudioComponent` _returnvalue_3)
        (`self.CompleteSpecificObjective` "obj_greece_learn_athena")
        (bind _myplayercharacter_2 (`/Game/ThirdPerson/CommonFunctionLibrary.GetMyPlayerCharacter`))
        (`/Game/ThirdPerson/Codex/BP_CodexSystem.UnlockEntry` (`self.GetComponentByClass` _myplayercharacter_2 "/Game/ThirdPerson/Codex/BP_CodexSystem.BP_CodexSystem_C") (`KismetStringLibrary.Conv_StringToName` (`BlueprintMapLibrary.Map_Find` (`self.QuestToCodexMap`) "obj_greece_learn_athena")))
        (set `self.DialogueStage` 1)
        (`/Game/Dialogue/WB_Dialogue.SetDialogueOptions` _ui "What is the Panathenaic festival?" "Tell me about the golden owl" "I think I'm ready to explore")
        (`/Game/Dialogue/WB_Dialogue.ShowOptionsPanel` _ui)
        (elif (`KismetStringLibrary.EqualEqual_StrStr` InputText "What is the Panathenaic festival?")
          (`/Game/Dialogue/WB_Dialogue.AddChatLine` _ui (`KismetTextLibrary.Conv_StringToText` "The Panathenaia is the greatest festival in all of Athens — a celebration of Athena's birthday. Every four years, the Grand Panathenaia brings athletes, poets, and musicians from across Greece. A great procession carries a new sacred robe — the peplos — up to the Acropolis to dress the ancient olive-wood statue of Athena. But this year, the sacred golden owl has vanished. Without it, the festival cannot proceed.") false)
          (bind _returnvalue_4 (`GameplayStatics.SpawnSound2D` "/Game/Audio/Aspasia/Aspasia_pantheic.Aspasia_pantheic" 1.0 1.0 0.0 null))
          (set `self.CurrentAudioComponent` _returnvalue_4)
          (`self.CompleteSpecificObjective` "obj_greece_learn_festival")
          (bind _myplayercharacter_3 (`/Game/ThirdPerson/CommonFunctionLibrary.GetMyPlayerCharacter`))
          (`/Game/ThirdPerson/Codex/BP_CodexSystem.UnlockEntry` (`self.GetComponentByClass` _myplayercharacter_3 "/Game/ThirdPerson/Codex/BP_CodexSystem.BP_CodexSystem_C") (`KismetStringLibrary.Conv_StringToName` (`BlueprintMapLibrary.Map_Find` (`self.QuestToCodexMap`) "obj_greece_learn_festival")))
          (set `self.DialogueStage` 1)
          (`/Game/Dialogue/WB_Dialogue.SetDialogueOptions` _ui "Tell me about the golden owl" "What happened to the owl?" "Tell me more about Athens")
          (`/Game/Dialogue/WB_Dialogue.ShowOptionsPanel` _ui)
          (elif (`KismetStringLibrary.EqualEqual_StrStr` InputText "Tell me about the golden owl")
            (`/Game/Dialogue/WB_Dialogue.AddChatLine` _ui (`KismetTextLibrary.Conv_StringToText` "The golden owl is a sacred ceremonial offering — a small golden sculpture of Athena's sacred bird, the owl of wisdom. It was placed at the feet of the Athena Parthenos statue by the priests during the last Grand Panathenaia. It is said that as long as the owl watches over Athens, the goddess's protection remains. Its disappearance has filled the city with fear.") false)
            (bind _returnvalue_5 (`GameplayStatics.SpawnSound2D` "/Game/Audio/Aspasia/Aspasia_goldenOwl.Aspasia_goldenOwl" 1.0 1.0 0.0 null))
            (set `self.CurrentAudioComponent` _returnvalue_5)
            (`self.CompleteSpecificObjective` "obj_greece_learn_owl")
            (bind _myplayercharacter_4 (`/Game/ThirdPerson/CommonFunctionLibrary.GetMyPlayerCharacter`))
            (`/Game/ThirdPerson/Codex/BP_CodexSystem.UnlockEntry` (`self.GetComponentByClass` _myplayercharacter_4 "/Game/ThirdPerson/Codex/BP_CodexSystem.BP_CodexSystem_C") (`KismetStringLibrary.Conv_StringToName` (`BlueprintMapLibrary.Map_Find` (`self.QuestToCodexMap`) "obj_greece_learn_owl")))
            (`/Game/Dialogue/WB_Dialogue.SetDialogueOptions` _ui "What happened to the owl?" "Tell me more about Athens" "Who might have taken it?")
            (`/Game/Dialogue/WB_Dialogue.ShowOptionsPanel` _ui)
            (elif (`KismetStringLibrary.EqualEqual_StrStr` InputText "What happened to the owl?")
              (`/Game/Dialogue/WB_Dialogue.AddChatLine` _ui (`KismetTextLibrary.Conv_StringToText` "Three nights ago, the temple guards discovered the owl was missing from its place at Athena's feet. No locks were broken, no doors forced. Whoever took it knew the temple well. Some whisper it was the sculptor Phidias's apprentice — a young man named Kleon — but others say Phidias himself may have hidden it to protect it from political enemies. Speak to Sokrates in the agora — he sees everything.") false)
              (bind _returnvalue_6 (`GameplayStatics.SpawnSound2D` "/Game/Audio/Aspasia/Aspasia_whatHappenedtotheOwl.Aspasia_whatHappenedtotheOwl" 1.0 1.0 0.0 null))
              (set `self.CurrentAudioComponent` _returnvalue_6)
              (`self.CompleteSpecificObjective` "obj_greece_learn_theft")
              (bind _myplayercharacter_5 (`/Game/ThirdPerson/CommonFunctionLibrary.GetMyPlayerCharacter`))
              (`/Game/ThirdPerson/Codex/BP_CodexSystem.UnlockEntry` (`self.GetComponentByClass` _myplayercharacter_5 "/Game/ThirdPerson/Codex/BP_CodexSystem.BP_CodexSystem_C") (`KismetStringLibrary.Conv_StringToName` (`BlueprintMapLibrary.Map_Find` (`self.QuestToCodexMap`) "obj_greece_learn_theft")))
              (`/Game/Dialogue/WB_Dialogue.SetDialogueOptions` _ui "What is this temple?" "I think I'm ready to explore" "Who is Athena?")
              (`/Game/Dialogue/WB_Dialogue.ShowOptionsPanel` _ui)
              (elif (`KismetStringLibrary.EqualEqual_StrStr` InputText "I think I'm ready to explore")
                (`/Game/Dialogue/WB_Dialogue.AddChatLine` _ui (`KismetTextLibrary.Conv_StringToText` "Before you go, let me test your memory!") false)
                (bind _returnvalue_7 (`GameplayStatics.SpawnSound2D` "/Game/Audio/Aspasia/Aspasia_LetMeTestYourMemory.Aspasia_LetMeTestYourMemory" 1.0 1.0 0.0 null))
                (set `self.CurrentAudioComponent` _returnvalue_7)
                (`KismetSystemLibrary.Delay` 3.0)
                (set `self.DialogueStage` 2)
                (set `self.CanTalk?` true)
                (bind _myplayercharacter_6 (`/Game/ThirdPerson/CommonFunctionLibrary.GetMyPlayerCharacter`))
                (bind _returnvalue_8 (`self.GetComponentByClass` _myplayercharacter_6 "/Game/ThirdPerson/Codex/BP_CodexSystem.BP_CodexSystem_C"))
                (`/Game/ThirdPerson/Codex/BP_CodexSystem.UnlockEntry` _returnvalue_8 (`KismetStringLibrary.Conv_StringToName` (`BlueprintMapLibrary.Map_Find` (`self.QuestToCodexMap`) "obj_greece_intro_complete")))
                (`self.ShowCurrentDialogueStage`)
                (elif (`KismetStringLibrary.EqualEqual_StrStr` InputText "Ask Aspasia for a hint")
                  (`Widget.SetVisibility` (`/Game/Dialogue/WB_Dialogue.BTN_Option4` _ui_2) "Collapsed")
                  (`Widget.SetVisibility` (`/Game/Dialogue/WB_Dialogue.InputBox_Border` _ui_2) "Visible")
                  (set `self.IsAwaitingHintInput` true)
                  (set `self.IsHintResponse` true)
                  (elif (`KismetArrayLibrary.Array_Contains` (`self.QuizOptions`) InputText)
                    (`self.HandleQuizAnswer` InputText)
                    (elif (`KismetStringLibrary.EqualEqual_StrStr` InputText "I found it! Here, take it back")
                      (bind _myplayercharacter_7 (`/Game/ThirdPerson/CommonFunctionLibrary.GetMyPlayerCharacter`))
                      (bind _returnvalue_9 (`self.GetComponentByClass` _myplayercharacter_7 "/Game/ThirdPerson/Inventory/BP_InventoryComponent.BP_InventoryComponent_C"))
                      (bind _iscollected (`/Game/ThirdPerson/Inventory/BP_InventoryComponent.IsItemCollected` _returnvalue_9 "golden_owl"))
                      (if _iscollected
                        (`/Game/ThirdPerson/Inventory/BP_InventoryComponent.RemoveItem` _returnvalue_9 "golden_owl")
                        (`/Game/Dialogue/WB_Dialogue.AddChatLine` _ui (`KismetTextLibrary.Conv_StringToText` "The owl of Athena! You truly found it behind the statue — Kleon will answer for his treachery. Athens is forever in your debt, traveler.") false)
                        (bind _returnvalue_10 (`GameplayStatics.SpawnSound2D` "/Game/Audio/Aspasia/Aspasia_OwlFOund.Aspasia_OwlFOund" 1.0 1.0 0.0 null))
                        (set `self.CurrentAudioComponent` _returnvalue_10)
                        (`self.CompleteSpecificObjective` "obj_greece_return_owl")
                        (`/Game/ThirdPerson/Codex/BP_CodexSystem.UnlockEntry` _returnvalue_8 "codex_greece_golden_owl")
                        (`KismetSystemLibrary.Delay` 8.0)
                        (`Widget.RemoveFromParent` (`self.UI`))
                        (`WidgetBlueprintLibrary.SetInputMode_GameOnly` _returnvalue)
                        (set `PlayerController.bShowMouseCursor` false _returnvalue)
                        (set `self.CanTalk?` true)
                        (`/Engine/EditorBlueprintResources/StandardMacros.IsValid` (`self.CurrentAudioComponent`)
                          (:`Is Valid`
                            (`AudioComponent.Stop` (`self.CurrentAudioComponent`))))
                        (else
                          (`/Game/Dialogue/WB_Dialogue.AddChatLine` _ui (`KismetTextLibrary.Conv_StringToText` "You say you found it, but I see nothing in your hands. Search the Parthenon more carefully") false)
                          (bind _returnvalue_11 (`GameplayStatics.SpawnSound2D` "/Game/Audio/Aspasia/Aspasia_Showme.Aspasia_Showme" 1.0 1.0 0.0 null))
                          (set `self.CurrentAudioComponent` _returnvalue_11)))
                      (else
                        (`/Game/Dialogue/WB_Dialogue.AddChatLine` _ui (`KismetTextLibrary.Conv_StringToText` "Go with Athena's blessing! Seek out Sokrates in the agora — the philosopher sees and hears everything in this city. And be wary of the sculptor's workshop near the statue. Someone there may know more than they are saying. Remember — in Athens, wisdom is the greatest weapon.") false)
                        (bind _returnvalue_12 (`GameplayStatics.SpawnSound2D` "/Game/Audio/Aspasia/Aspasia_GoSeek.Aspasia_GoSeek" 1.0 1.0 0.0 null))
                        (set `self.CurrentAudioComponent` _returnvalue_12)
                        (`/Game/Dialogue/WB_Dialogue.SetDialogueOptions` _ui "What is this temple?" "Who is Athena?" "I think I'm ready to explore")
                        (`/Game/Dialogue/WB_Dialogue.ShowOptionsPanel` _ui)))))))))))))

(event `self.Talk`
  (bind _returnvalue (`GameplayStatics.GetPlayerController` 0))
  (bind _dialoguestage (`self.DialogueStage`))
  (if (`self.CanTalk?`)
    (set `self.CanTalk?` false)
    (bind _returnvalue_2 (`|CreateWidget` "/Game/Dialogue/WB_Dialogue.WB_Dialogue_C" _returnvalue self))
    (bind _output_get (set `self.UI` _returnvalue_2))
    (`UserWidget.AddToViewport` _output_get 0)
    (`WidgetBlueprintLibrary.SetInputMode_GameAndUIEx` _returnvalue _output_get "DoNotLock" false)
    (set `PlayerController.bShowMouseCursor` true _returnvalue)
    (if (== _dialoguestage 0)
      (`/Game/Dialogue/WB_Dialogue.AddChatLine` _output_get (`KismetTextLibrary.Conv_StringToText` "Welcome, traveler, to the Parthenon — the crown of Athens and the sacred house of Athena. I am Aspasia, priestess of the goddess. But I fear you arrive at a troubled time.") false)
      (bind _returnvalue_3 (`GameplayStatics.SpawnSound2D` "/Game/Audio/Aspasia/Aspasia_Intro.Aspasia_Intro" 1.0 1.0 0.0 null))
      (set `self.CurrentAudioComponent` _returnvalue_3)
      (`/Game/Dialogue/WB_Dialogue.SetDialogueOptions` _output_get "What is this temple?" "Who is Athena?" "What is the Panathenaic festival?")
      (`/Game/Dialogue/WB_Dialogue.ShowOptionsPanel` _output_get)
      (elif (== _dialoguestage 1)
        (`/Game/Dialogue/WB_Dialogue.AddChatLine` _output_get (`KismetTextLibrary.Conv_StringToText` "Welcome back, traveler. The owl is still missing. What else would you like to know?") false)
        (`GameplayStatics.PlaySound2D` null 1.0 1.0 0.0 null null)
        (`/Game/Dialogue/WB_Dialogue.SetDialogueOptions` _output_get "Tell me about the golden owl" "What happened to the owl?" "I think I'm ready to explore")
        (`/Game/Dialogue/WB_Dialogue.ShowOptionsPanel` _output_get)
        (elif (== _dialoguestage 2)
          (`/Game/Dialogue/WB_Dialogue.AddChatLine` _output_get (`KismetTextLibrary.Conv_StringToText` "Athena smiles upon the wise. You have proven your knowledge — go find that owl, traveler!") false)
          (`GameplayStatics.PlaySound2D` null 1.0 1.0 0.0 null null)
          (set `self.CanTalk?` true)
          (elif (== _dialoguestage 3)
            (`/Game/Dialogue/WB_Dialogue.AddChatLine` _output_get "Welcome back, traveler...Do you have any info about the Golden Owl" false)
            (`/Game/Dialogue/WB_Dialogue.SetDialogueOptions` _output_get "I found it! Here, take it back" "Not yet, still searching" "Tell me about the golden owl")
            (`/Game/Dialogue/WB_Dialogue.ShowOptionsPanel` _output_get)))))))

(event `ShowCurrentDialogueStage`
  (bind _returnvalue (`KismetTextLibrary.Conv_StringToText` "What happened to the golden owl?"))
  (bind _returnvalue_2 (`GameplayStatics.GetPlayerController` 0))
  (bind _returnvalue_3 (`KismetTextLibrary.Conv_StringToText` "Now let us test your knowledge! What is the Parthenon?"))
  (bind _returnvalue_4 (`KismetTextLibrary.Conv_StringToText` "What is Athena the goddess of?"))
  (bind _returnvalue_5 (`KismetTextLibrary.Conv_StringToText` "What is the Panathenaic festival?"))
  (bind _ui (`self.UI`))
  (bind _ui_2 (`self.UI`))
  (bind _ui_3 (`self.UI`))
  (bind _ui_4 (`self.UI`))
  (bind _ui_5 (`self.UI`))
  (if (== (`self.DialogueStage`) 2)
    (`/Game/Dialogue/WB_Dialogue.AddChatLine` _ui_4 _returnvalue_3 false)
    (set `self.Current Quiz Question` (`KismetTextLibrary.Conv_TextToString` _returnvalue_3))
    (`/Game/Dialogue/WB_Dialogue.SetDialogueOptions` _ui_4 "The sacred house of Athena" "A marketplace for traders" "A fortress for Athenian soldiers")
    (`/Game/Dialogue/WB_Dialogue.ShowOptionsPanel` _ui_4)
    (`Widget.SetVisibility` (`/Game/Dialogue/WB_Dialogue.InputBox_Border` _ui_4) "SelfHitTestInvisible")
    (`Widget.SetVisibility` (`/Game/Dialogue/WB_Dialogue.BTN_Option4` _ui_4) "Visible")
    (`TextBlock.SetText` (`/Game/Dialogue/WB_Dialogue.Txt_Option4` _ui_4) (`KismetTextLibrary.Conv_StringToText` "Ask Aspasia for a hint"))
    (elif (== (`self.DialogueStage`) 3)
      (`/Game/Dialogue/WB_Dialogue.AddChatLine` _ui_5 _returnvalue_4 false)
      (set `self.Current Quiz Question` (`KismetTextLibrary.Conv_TextToString` _returnvalue_4))
      (`/Game/Dialogue/WB_Dialogue.SetDialogueOptions` _ui_5 "Love, beauty, and the sea" "Wisdom, courage, and strategic warfare" "Fire, harvest, and the underworld")
      (`/Game/Dialogue/WB_Dialogue.ShowOptionsPanel` _ui_5)
      (`Widget.SetVisibility` (`/Game/Dialogue/WB_Dialogue.InputBox_Border` _ui_5) "SelfHitTestInvisible")
      (`Widget.SetVisibility` (`/Game/Dialogue/WB_Dialogue.BTN_Option4` _ui_5) "Visible")
      (`TextBlock.SetText` (`/Game/Dialogue/WB_Dialogue.Txt_Option4` _ui_5) (`KismetTextLibrary.Conv_StringToText` "Ask Aspasia for a hint"))
      (elif (== (`self.DialogueStage`) 4)
        (`/Game/Dialogue/WB_Dialogue.AddChatLine` _ui_2 _returnvalue_5 false)
        (set `self.Current Quiz Question` (`KismetTextLibrary.Conv_TextToString` _returnvalue_5))
        (`/Game/Dialogue/WB_Dialogue.SetDialogueOptions` _ui_2 "A trade fair between Greek city-states" "A funeral ceremony for fallen warriors" "A celebration of Athena's birthday")
        (`/Game/Dialogue/WB_Dialogue.ShowOptionsPanel` _ui_2)
        (`Widget.SetVisibility` (`/Game/Dialogue/WB_Dialogue.InputBox_Border` _ui_2) "SelfHitTestInvisible")
        (`Widget.SetVisibility` (`/Game/Dialogue/WB_Dialogue.BTN_Option4` _ui_2) "Visible")
        (`TextBlock.SetText` (`/Game/Dialogue/WB_Dialogue.Txt_Option4` _ui_2) (`KismetTextLibrary.Conv_StringToText` "Ask Aspasia for a hint"))
        (elif (== (`self.DialogueStage`) 5)
          (`/Game/Dialogue/WB_Dialogue.AddChatLine` _ui _returnvalue false)
          (set `self.Current Quiz Question` (`KismetTextLibrary.Conv_TextToString` _returnvalue))
          (`/Game/Dialogue/WB_Dialogue.SetDialogueOptions` _ui "It was stolen from the Parthenon" "It was melted down for coins" "It was given to Sparta as tribute")
          (`/Game/Dialogue/WB_Dialogue.ShowOptionsPanel` _ui)
          (`Widget.SetVisibility` (`/Game/Dialogue/WB_Dialogue.InputBox_Border` _ui) "SelfHitTestInvisible")
          (`Widget.SetVisibility` (`/Game/Dialogue/WB_Dialogue.BTN_Option4` _ui) "Visible")
          (`TextBlock.SetText` (`/Game/Dialogue/WB_Dialogue.Txt_Option4` _ui) (`KismetTextLibrary.Conv_StringToText` "Ask Aspasia for a hint"))
          (elif (== (`self.DialogueStage`) 6)
            (`/Game/Dialogue/WB_Dialogue.AddChatLine` _ui_3 (`KismetTextLibrary.Conv_StringToText` "Wonderful! You've proven yourself a true student of Athens!") false)
            (`KismetSystemLibrary.Delay` 4.0)
            (`self.CompleteSpecificObjective` "obj_greece_intro_complete")
            (set `self.HasCompletedIntro` true)
            (`Widget.RemoveFromParent` _ui_3)
            (`WidgetBlueprintLibrary.SetInputMode_GameOnly` _returnvalue_2)
            (set `PlayerController.bShowMouseCursor` false _returnvalue_2)
            (`/Engine/EditorBlueprintResources/StandardMacros.IsValid` (`self.CurrentAudioComponent`)
              (:`Is Valid`
                (`AudioComponent.Stop` (`self.CurrentAudioComponent`))))))))))

(event `self.ReceiveBeginPlay`
  (`parent.ReceiveBeginPlay`)
  (add `/Game/Blueprints/BP_HttpClient_Component.OnAIResponseReceived` (`self.BP_HttpClient_Component`) (delegate `self.OnAIResponseReceived_Event`)))

(event `self.OnAIResponseReceived_Event`
  (params (ResponseText :type String))
  (`self.AddToHistory` ResponseText "AI")
  (`/Game/Dialogue/WB_Dialogue.AddChatLine` (`self.UI`) (`KismetTextLibrary.Conv_StringToText` ResponseText) false)
  (if (`self.IsHintResponse`)
    (set `self.IsHintResponse` false)
    (bind _myplayercharacter (`/Game/ThirdPerson/CommonFunctionLibrary.GetMyPlayerCharacter`))
    (`/Game/ThirdPerson/Blueprints/BP_ThirdPersonCharacter.DeductKP` _myplayercharacter 5))
  (`self.CheckQuestKeywords` ResponseText)
  (bind _myplayercharacter_2 (`/Game/ThirdPerson/CommonFunctionLibrary.GetMyPlayerCharacter`))
  (bind _returnvalue (`self.GetComponentByClass` _myplayercharacter_2 "/Game/ThirdPerson/QuestSYstem/QuestLog_Component.QuestLog_Component_C"))
  (for _array_element (`/Game/ThirdPerson/QuestSYstem/QuestLog_Component.CurrentQuests` _returnvalue)
    (`/Engine/EditorBlueprintResources/StandardMacros.IsValid` _array_element
      (:`Is Valid`
        (for _array_element_2 (`.Objectives_21_75F1BA2A457170AB65DED5B45FFC78A1` (break `/Game/ThirdPerson/QuestSYstem/StageDetails` (`/Game/ThirdPerson/QuestSYstem/BP_QuestBase.CurrentStageDetails` _array_element)))
          (bind (_objectivename _description _type _objectiveid) (break `/Game/ThirdPerson/QuestSYstem/ObjectiveDetails` _array_element_2))
          (bind _iscomplete (`/Game/ThirdPerson/QuestSYstem/BP_QuestBase.IsObjectiveComplete` _array_element _objectiveid))
          (if (not _iscomplete)
            (if (`KismetArrayLibrary.Array_Contains` (`self.ObjectivesToComplete`) _objectiveid)
              (`/Game/ThirdPerson/QuestSYstem/BP_QuestBase.UpdateObjectiveProgress` _array_element _objectiveid 1)
              (`self.ProcessQuestForCodex` _array_element)
              (break)))))))
  (for _array_element_3 (`/Game/ThirdPerson/QuestSYstem/QuestLog_Component.CompletedQuestActors` _returnvalue)
    (`self.ProcessQuestForCodex` _array_element_3))
  (`KismetSystemLibrary.Delay` 6.0)
  (`self.ShowCurrentDialogueStage`))

(fn `CompleteQuestObjectives`
  (bind _myplayercharacter (`/Game/ThirdPerson/CommonFunctionLibrary.GetMyPlayerCharacter`))
  (for _array_element (`/Game/ThirdPerson/QuestSYstem/QuestLog_Component.CurrentQuests` (`self.GetComponentByClass` _myplayercharacter "/Game/ThirdPerson/QuestSYstem/QuestLog_Component.QuestLog_Component_C"))
    (for _array_element_2 (`self.ObjectivesToComplete`)
      (bind _iscomplete (`/Game/ThirdPerson/QuestSYstem/BP_QuestBase.IsObjectiveComplete` _array_element _array_element_2))
      (if (not _iscomplete)
        (`/Game/ThirdPerson/QuestSYstem/BP_QuestBase.UpdateObjectiveProgress` _array_element _array_element_2 1)
        (break)))))

(fn `CompleteSpecificObjective`
  (params (ObjectiveID :type String))
  (bind _myplayercharacter (`/Game/ThirdPerson/CommonFunctionLibrary.GetMyPlayerCharacter`))
  (for _array_element (`/Game/ThirdPerson/QuestSYstem/QuestLog_Component.CurrentQuests` (`self.GetComponentByClass` _myplayercharacter "/Game/ThirdPerson/QuestSYstem/QuestLog_Component.QuestLog_Component_C"))
    (`/Game/ThirdPerson/QuestSYstem/BP_QuestBase.UpdateObjectiveProgress` _array_element ObjectiveID 1)))

(fn `HandleQuizAnswer`
  (params (AnswerText :type String))
  (bind _dialoguestage (`self.DialogueStage`))
  (bind _ui (`self.UI`))
  (if (== _dialoguestage 2)
    (if (`KismetStringLibrary.EqualEqual_StrStr` AnswerText "The sacred house of Athena")
      (bind _myplayercharacter (`/Game/ThirdPerson/CommonFunctionLibrary.GetMyPlayerCharacter`))
      (`/Game/ThirdPerson/Blueprints/BP_ThirdPersonCharacter.AddKP` _myplayercharacter 10)
      (`/Game/Dialogue/WB_Dialogue.AddChatLine` _ui (`KismetTextLibrary.Conv_StringToText` "Correct! The Parthenon is Athena's sacred temple!") false)
      (`self.CompleteSpecificObjective` "obj_greece_learn_temple")
      (bind _myplayercharacter_2 (`/Game/ThirdPerson/CommonFunctionLibrary.GetMyPlayerCharacter`))
      (`/Game/ThirdPerson/Codex/BP_CodexSystem.UnlockEntry` (`/Game/ThirdPerson/Blueprints/BP_ThirdPersonCharacter.CodexSystem` _myplayercharacter_2) "codex_greece_parthenon")
      (`|ExecutionSequence`
        (:`then_0`
          (set `self.DialogueStage` (+ _dialoguestage 1))
          (`self.ShowCurrentDialogueStage` self)))
      (else
        (bind _myplayercharacter_3 (`/Game/ThirdPerson/CommonFunctionLibrary.GetMyPlayerCharacter`))
        (bind _bgameover (`/Game/ThirdPerson/Blueprints/BP_ThirdPersonCharacter.DeductKP` _myplayercharacter_3 5))
        (if _bgameover
          (bind _returnvalue (`|CreateWidget` "/Game/ThirdPerson/QuestSYstem/UI/WBP_GameOver.WBP_GameOver_C"))
          (`UserWidget.AddToViewport` _returnvalue 0)
          (else
            (`/Game/Dialogue/WB_Dialogue.AddChatLine` _ui (`KismetTextLibrary.Conv_StringToText` "Not quite. The Parthenon was built as a sacred house for Athena.") false)
            (`self.ShowCurrentDialogueStage`)))))
    (elif (== _dialoguestage 3)
      (if (`KismetStringLibrary.EqualEqual_StrStr` AnswerText "Wisdom, courage, and strategic warfare")
        (bind _myplayercharacter_4 (`/Game/ThirdPerson/CommonFunctionLibrary.GetMyPlayerCharacter`))
        (`/Game/ThirdPerson/Blueprints/BP_ThirdPersonCharacter.AddKP` _myplayercharacter_4 10)
        (`/Game/Dialogue/WB_Dialogue.AddChatLine` _ui (`KismetTextLibrary.Conv_StringToText` "Correct! Athena embodies wisdom and strategic warfare!") false)
        (`self.CompleteSpecificObjective` "obj_greece_learn_athena")
        (bind _myplayercharacter_5 (`/Game/ThirdPerson/CommonFunctionLibrary.GetMyPlayerCharacter`))
        (`/Game/ThirdPerson/Codex/BP_CodexSystem.UnlockEntry` (`/Game/ThirdPerson/Blueprints/BP_ThirdPersonCharacter.CodexSystem` _myplayercharacter_5) "codex_greece_athena")
        (`|ExecutionSequence`
          (:`then_0`
            (set `self.DialogueStage` (+ _dialoguestage 1))
            (`self.ShowCurrentDialogueStage` self)))
        (else
          (bind _myplayercharacter_6 (`/Game/ThirdPerson/CommonFunctionLibrary.GetMyPlayerCharacter`))
          (bind _bgameover_2 (`/Game/ThirdPerson/Blueprints/BP_ThirdPersonCharacter.DeductKP` _myplayercharacter_6 5))
          (if _bgameover_2
            (bind _returnvalue_2 (`|CreateWidget` "/Game/ThirdPerson/QuestSYstem/UI/WBP_GameOver.WBP_GameOver_C"))
            (`UserWidget.AddToViewport` _returnvalue_2 0)
            (else
              (`/Game/Dialogue/WB_Dialogue.AddChatLine` _ui (`KismetTextLibrary.Conv_StringToText` "Not quite. Athena is the goddess of wisdom, courage, and strategic warfare.") false)
              (`self.ShowCurrentDialogueStage`)))))
      (elif (== _dialoguestage 4)
        (if (`KismetStringLibrary.EqualEqual_StrStr` AnswerText "A celebration of Athena's birthday")
          (bind _myplayercharacter_7 (`/Game/ThirdPerson/CommonFunctionLibrary.GetMyPlayerCharacter`))
          (`/Game/ThirdPerson/Blueprints/BP_ThirdPersonCharacter.AddKP` _myplayercharacter_7 10)
          (`/Game/Dialogue/WB_Dialogue.AddChatLine` _ui (`KismetTextLibrary.Conv_StringToText` "Correct! The Panathenaia celebrates Athena's birthday!") false)
          (`self.CompleteSpecificObjective` "obj_greece_learn_festival")
          (bind _myplayercharacter_8 (`/Game/ThirdPerson/CommonFunctionLibrary.GetMyPlayerCharacter`))
          (`/Game/ThirdPerson/Codex/BP_CodexSystem.UnlockEntry` (`/Game/ThirdPerson/Blueprints/BP_ThirdPersonCharacter.CodexSystem` _myplayercharacter_8) "codex_greece_panathenaia")
          (`|ExecutionSequence`
            (:`then_0`
              (set `self.DialogueStage` (+ (`self.DialogueStage`) 1))
              (`self.ShowCurrentDialogueStage` self)))
          (else
            (bind _myplayercharacter_9 (`/Game/ThirdPerson/CommonFunctionLibrary.GetMyPlayerCharacter`))
            (bind _bgameover_3 (`/Game/ThirdPerson/Blueprints/BP_ThirdPersonCharacter.DeductKP` _myplayercharacter_9 5))
            (if _bgameover_3
              (bind _returnvalue_3 (`|CreateWidget` "/Game/ThirdPerson/QuestSYstem/UI/WBP_GameOver.WBP_GameOver_C"))
              (`UserWidget.AddToViewport` _returnvalue_3 0)
              (else
                (`/Game/Dialogue/WB_Dialogue.AddChatLine` _ui (`KismetTextLibrary.Conv_StringToText` "Not quite. The Panathenaia is the great celebration of Athena's birthday.") false)
                (`self.ShowCurrentDialogueStage`)))))
        (elif (== _dialoguestage 5)
          (if (`KismetStringLibrary.EqualEqual_StrStr` AnswerText "It was stolen from the Parthenon")
            (bind _myplayercharacter_10 (`/Game/ThirdPerson/CommonFunctionLibrary.GetMyPlayerCharacter`))
            (`/Game/ThirdPerson/Blueprints/BP_ThirdPersonCharacter.AddKP` _myplayercharacter_10 10)
            (`/Game/Dialogue/WB_Dialogue.AddChatLine` _ui (`KismetTextLibrary.Conv_StringToText` "Correct! The sacred golden owl was stolen from the temple!") false)
            (`self.CompleteSpecificObjective` "obj_greece_learn_owl")
            (`self.CompleteSpecificObjective` "obj_greece_learn_theft")
            (bind _myplayercharacter_11 (`/Game/ThirdPerson/CommonFunctionLibrary.GetMyPlayerCharacter`))
            (`/Game/ThirdPerson/Codex/BP_CodexSystem.UnlockEntry` (`/Game/ThirdPerson/Blueprints/BP_ThirdPersonCharacter.CodexSystem` _myplayercharacter_11) "codex_greece_golden_owl")
            (`|ExecutionSequence`
              (:`then_0`
                (set `self.DialogueStage` (+ (`self.DialogueStage`) 1))
                (`self.ShowCurrentDialogueStage` self)))
            (else
              (bind _myplayercharacter_12 (`/Game/ThirdPerson/CommonFunctionLibrary.GetMyPlayerCharacter`))
              (bind _bgameover_4 (`/Game/ThirdPerson/Blueprints/BP_ThirdPersonCharacter.DeductKP` _myplayercharacter_12 5))
              (if _bgameover_4
                (bind _returnvalue_4 (`|CreateWidget` "/Game/ThirdPerson/QuestSYstem/UI/WBP_GameOver.WBP_GameOver_C"))
                (`UserWidget.AddToViewport` _returnvalue_4 0)
                (else
                  (`/Game/Dialogue/WB_Dialogue.AddChatLine` _ui (`KismetTextLibrary.Conv_StringToText` "Not quite. The golden owl was stolen from its place at Athena's feet.") false)
                  (`self.ShowCurrentDialogueStage`))))))))))

(fn `ProcessQuestForCodex`
  (params (QuestActor :type "/Game/ThirdPerson/QuestSYstem/BP_QuestBase Object Reference"))
  (bind _returnvalue (`self.GetComponentByClass` (`GameplayStatics.GetPlayerCharacter` 0) "/Game/ThirdPerson/Codex/BP_CodexSystem.BP_CodexSystem_C"))
  (bind (_value _returnvalue_2) (`BlueprintMapLibrary.Map_Find` (`self.QuestToCodexMap`) "obj_bonus"))
  (set `self.CompletedCount` 0)
  (for _array_element (`self.ObjectivesToComplete`)
    (bind _iscomplete (`/Game/ThirdPerson/QuestSYstem/BP_QuestBase.IsObjectiveComplete` QuestActor _array_element))
    (if _iscomplete
      (set `self.CompletedCount` (+ (`self.CompletedCount`) 1))
      (bind (_value_2 _returnvalue_3) (`BlueprintMapLibrary.Map_Find` (`self.QuestToCodexMap`) _array_element))
      (if _returnvalue_3
        (`/Engine/EditorBlueprintResources/StandardMacros.IsValid` _returnvalue
          (:`Is Valid`
            (`/Game/ThirdPerson/Codex/BP_CodexSystem.UnlockEntry` _returnvalue (`KismetStringLibrary.Conv_StringToName` _value_2)))))))
  (if (== (`self.CompletedCount`) (`KismetArrayLibrary.Array_Length` (`self.ObjectivesToComplete`)))
    (if _returnvalue_2
      (`/Game/ThirdPerson/Codex/BP_CodexSystem.UnlockEntry` (`self.GetComponentByClass` (`GameplayStatics.GetPlayerCharacter` 0) "/Game/ThirdPerson/Codex/BP_CodexSystem.BP_CodexSystem_C") (`KismetStringLibrary.Conv_StringToName` _value)))))

(fn `UserConstructionScript`
  (`parent.UserConstructionScript`))