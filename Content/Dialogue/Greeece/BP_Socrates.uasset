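; Socrates NPC for the Greece level, running a branching dialogue and knowledge quiz tied to quests and the codex.
; Talk opens WB_Dialogue, and PlayerInput matches option text to scripted, voiced replies that unlock codex entries.
; DialogueStage steps through quiz questions that award or deduct KP, complete objectives and can trigger game over.
; Typed hint requests go through BPHttpClientComponent to an AI, whose replies cost KP and also advance quest objectives.
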(event `self.ReceivePlayerInput`
  (params (InputText :type String))
  (bind _bp_httpclient_component (`self.BP_HttpClient_Component`))
  (bind _ui (`self.UI`))
  (bind _ui_2 (`self.UI`))
  (`/Engine/EditorBlueprintResources/StandardMacros.IsValid` (`self.CurrentAudioComponent`)
    (:`Is Valid`
      (`AudioComponent.Stop` (`self.CurrentAudioComponent`)))
    (:`Is Not Valid`
      _))
  (`/Game/Dialogue/WB_Dialogue.AddChatLine` _ui (`KismetTextLibrary.Conv_StringToText` InputText) true)
  (if (`self.IsAwaitingHintInput`)
    (set `self.IsAwaitingHintInput` false)
    (`Widget.SetVisibility` (`/Game/Dialogue/WB_Dialogue.InputBox_Border` (`self.UI`)) "Collapsed")
    (bind _full_prompt (`/Game/Blueprints/BP_HttpClient_Component.Build_Followup_Prompt` _bp_httpclient_component "socrates" (`KismetStringLibrary.Concat_StrStr` (`KismetStringLibrary.Concat_StrStr` "The player is asking for a hint during a quiz about: " (`self.Current Quiz Question`)) InputText) ""))
    (`/Game/Blueprints/BP_HttpClient_Component.Send AI Request` _bp_httpclient_component _full_prompt "" "")
    (elif (`KismetStringLibrary.EqualEqual_StrStr` InputText "What do you teach about virtue?")
      (`/Game/Dialogue/WB_Dialogue.AddChatLine` _ui (`KismetTextLibrary.Conv_StringToText` "Virtue, my friend, is not something you are born with — it is knowledge. If a person truly understands what is good, they will always choose it. No one does evil willingly — only out of ignorance. Think of it this way: a potter who knows his craft never deliberately makes a crooked pot. So too, a person who truly knows justice will always act justly.") false)
      (bind _returnvalue (`GameplayStatics.SpawnSound2D` "/Game/Audio/Socrates/Socrates_Virtue.Socrates_Virtue" 1.0 1.0 0.0 null))
      (set `self.CurrentAudioComponent` _returnvalue)
      (bind _myplayercharacter (`/Game/ThirdPerson/CommonFunctionLibrary.GetMyPlayerCharacter`))
      (`/Game/ThirdPerson/Codex/BP_CodexSystem.UnlockEntry` (`self.GetComponentByClass` _myplayercharacter "/Game/ThirdPerson/Codex/BP_CodexSystem.BP_CodexSystem_C") (`KismetStringLibrary.Conv_StringToName` (`BlueprintMapLibrary.Map_Find` (`self.QuestToCodexMap`) "obj_greece_learn_ethics")))
      (set `self.DialogueStage` 1)
      (`/Game/Dialogue/WB_Dialogue.SetDialogueOptions` _ui "What is your famous claim about wisdom?" "What do you know about the missing golden owl?" "Tell me about justice and wrongdoing")
      (`/Game/Dialogue/WB_Dialogue.ShowOptionsPanel` _ui)
      (elif (`KismetStringLibrary.EqualEqual_StrStr` InputText "What is your famous claim about wisdom?")
        (`/Game/Dialogue/WB_Dialogue.AddChatLine` _ui (`KismetTextLibrary.Conv_StringToText` "The Oracle at Delphi declared me the wisest man in Athens. I was baffled — so I went to every wise man I could find, every politician, poet, and craftsman. And I discovered something remarkable: they all believed they knew things they did not. I, at least, know that I know nothing. That small difference, it seems, is what the Oracle meant. True wisdom begins with humility.") false)
        (bind _returnvalue_2 (`GameplayStatics.SpawnSound2D` "/Game/Audio/Socrates/Socrates_OracleWisdom.Socrates_OracleWisdom" 1.0 1.0 0.0 null))
        (set `self.CurrentAudioComponent` _returnvalue_2)
        (bind _myplayercharacter_2 (`/Game/ThirdPerson/CommonFunctionLibrary.GetMyPlayerCharacter`))
        (`/Game/ThirdPerson/Codex/BP_CodexSystem.UnlockEntry` (`self.GetComponentByClass` _myplayercharacter_2 "/Game/ThirdPerson/Codex/BP_CodexSystem.BP_CodexSystem_C") (`KismetStringLibrary.Conv_StringToName` (`BlueprintMapLibrary.Map_Find` (`self.QuestToCodexMap`) "obj_greece_learn_knowledge")))
        (set `self.DialogueStage` 1)
        (`/Game/Dialogue/WB_Dialogue.SetDialogueOptions` _ui "What do you know about the missing golden owl?" "Tell me about justice and wrongdoing" "I think I'm ready for the test")
        (`/Game/Dialogue/WB_Dialogue.ShowOptionsPanel` _ui)
        (elif (`KismetStringLibrary.EqualEqual_StrStr` InputText "What do you know about the missing golden owl?")
          (`/Game/Dialogue/WB_Dialogue.AddChatLine` _ui (`KismetTextLibrary.Conv_StringToText` "I observe everything in this agora, and I saw something troubling. Young Kleon — Phidias's apprentice — was carrying something wrapped in cloth near the statue of Athena inside the Parthenon, late at night. He looked over his shoulder three times before disappearing into the shadows. I do not accuse — but the truth often hides where guilt walks.") false)
          (bind _returnvalue_3 (`GameplayStatics.SpawnSound2D` "/Game/Audio/Socrates/Socrates_IObserve.Socrates_IObserve" 1.0 1.0 0.0 null))
          (set `self.CurrentAudioComponent` _returnvalue_3)
          (bind _myplayercharacter_3 (`/Game/ThirdPerson/CommonFunctionLibrary.GetMyPlayerCharacter`))
          (`/Game/ThirdPerson/Codex/BP_CodexSystem.UnlockEntry` (`self.GetComponentByClass` _myplayercharacter_3 "/Game/ThirdPerson/Codex/BP_CodexSystem.BP_CodexSystem_C") (`KismetStringLibrary.Conv_StringToName` (`BlueprintMapLibrary.Map_Find` (`self.QuestToCodexMap`) "codex_greece_socrates")))
          (set `self.DialogueStage` 1)
          (`/Game/Dialogue/WB_Dialogue.SetDialogueOptions` _ui "Tell me about justice and wrongdoing" "What were the charges against you?" "I think I'm ready for the test")
          (`/Game/Dialogue/WB_Dialogue.ShowOptionsPanel` _ui)
          (elif (`KismetStringLibrary.EqualEqual_StrStr` InputText "Tell me about justice and wrongdoing")
            (`/Game/Dialogue/WB_Dialogue.AddChatLine` _ui (`KismetTextLibrary.Conv_StringToText` "Here is what I believe with all my soul: it is better to suffer injustice than to commit it. When someone wrongs you, the damage is to your body, your reputation, your wealth — things that fade. But when YOU commit injustice, the damage is to your soul — and that is permanent. The tyrant who rules through cruelty is the most miserable man alive, though he may not know it.") false)
            (bind _returnvalue_4 (`GameplayStatics.SpawnSound2D` "/Game/Audio/Socrates/Socrates_HereWhat.Socrates_HereWhat" 1.0 1.0 0.0 null))
            (set `self.CurrentAudioComponent` _returnvalue_4)
            (bind _myplayercharacter_4 (`/Game/ThirdPerson/CommonFunctionLibrary.GetMyPlayerCharacter`))
            (`/Game/ThirdPerson/Codex/BP_CodexSystem.UnlockEntry` (`self.GetComponentByClass` _myplayercharacter_4 "/Game/ThirdPerson/Codex/BP_CodexSystem.BP_CodexSystem_C") (`KismetStringLibrary.Conv_StringToName` (`BlueprintMapLibrary.Map_Find` (`self.QuestToCodexMap`) "obj_greece_learn_ethics")))
            (`/Game/Dialogue/WB_Dialogue.SetDialogueOptions` _ui "What were the charges against you?" "Tell me about justice and wrongdoing" "What do you know about the missing golden owl?")
            (`/Game/Dialogue/WB_Dialogue.ShowOptionsPanel` _ui)
            (elif (`KismetStringLibrary.EqualEqual_StrStr` InputText "What were the charges against you?")
              (`/Game/Dialogue/WB_Dialogue.AddChatLine` _ui (`KismetTextLibrary.Conv_StringToText` "The formal charges are corruption of the youth and introducing new gods to Athens. Meletus brought the accusation, but Anytus — a powerful politician — is the true force behind it. They say my questioning undermines respect for tradition. Perhaps it does. But I would rather die than stop seeking truth. If the jury condemns me, I shall drink the hemlock willingly — for an unexamined life is not worth living.") false)
              (bind _returnvalue_5 (`GameplayStatics.SpawnSound2D` "/Game/Audio/Socrates/Socrates_FormalChanges.Socrates_FormalChanges" 1.0 1.0 0.0 null))
              (set `self.CurrentAudioComponent` _returnvalue_5)
              (bind _myplayercharacter_5 (`/Game/ThirdPerson/CommonFunctionLibrary.GetMyPlayerCharacter`))
              (`/Game/ThirdPerson/Codex/BP_CodexSystem.UnlockEntry` (`self.GetComponentByClass` _myplayercharacter_5 "/Game/ThirdPerson/Codex/BP_CodexSystem.BP_CodexSystem_C") (`KismetStringLibrary.Conv_StringToName` (`BlueprintMapLibrary.Map_Find` (`self.QuestToCodexMap`) "obj_greece_learn_trial")))
              (`/Game/Dialogue/WB_Dialogue.SetDialogueOptions` _ui "What is your famous claim about wisdom?" "I think I'm ready for the test" "What do you teach about virtue?")
              (`/Game/Dialogue/WB_Dialogue.ShowOptionsPanel` _ui)
              (elif (`KismetStringLibrary.EqualEqual_StrStr` InputText "I think I'm ready for the test")
                (`/Game/Dialogue/WB_Dialogue.AddChatLine` _ui (`KismetTextLibrary.Conv_StringToText` "Before we part, let me see if you were truly listening!") false)
                (bind _returnvalue_6 (`GameplayStatics.SpawnSound2D` "/Game/Audio/Socrates/Socrates_BeforeYouGo.Socrates_BeforeYouGo" 1.0 1.0 0.0 null))
                (set `self.CurrentAudioComponent` _returnvalue_6)
                (`KismetSystemLibrary.Delay` 3.0)
                (set `self.DialogueStage` 2)
                (set `self.CanTalk?` true)
                (`self.CompleteSpecificObjective` "obj_greece_intro_complete")
                (set `self.HasCompletedIntro` true)
                (bind _myplayercharacter_6 (`/Game/ThirdPerson/CommonFunctionLibrary.GetMyPlayerCharacter`))
                (`/Game/ThirdPerson/Codex/BP_CodexSystem.UnlockEntry` (`self.GetComponentByClass` _myplayercharacter_6 "/Game/ThirdPerson/Codex/BP_CodexSystem.BP_CodexSystem_C") (`KismetStringLibrary.Conv_StringToName` (`BlueprintMapLibrary.Map_Find` (`self.QuestToCodexMap`) "obj_greece_intro_complete")))
                (`self.ShowCurrentDialogueStage`)
                (elif (`KismetStringLibrary.EqualEqual_StrStr` InputText "Ask Socrates for a hint")
                  (`Widget.SetVisibility` (`/Game/Dialogue/WB_Dialogue.BTN_Option4` _ui_2) "Collapsed")
                  (`Widget.SetVisibility` (`/Game/Dialogue/WB_Dialogue.InputBox_Border` _ui_2) "Visible")
                  (set `self.IsAwaitingHintInput` true)
                  (set `self.IsHintResponse` true)
                  (elif (`KismetArrayLibrary.Array_Contains` (`self.QuizOptions`) InputText)
                    (`self.HandleQuizAnswer` InputText)
                    (else
                      (`/Game/Dialogue/WB_Dialogue.AddChatLine` _ui (`KismetTextLibrary.Conv_StringToText` "Excellent! You have truly listened. Go now — carry these ideas with you. Question everything, trust your reason, and remember: the unexamined life is not worth living. Athens needs thinkers like you.") false)
                      (bind _returnvalue_7 (`GameplayStatics.SpawnSound2D` "/Game/Audio/Socrates/Socrates_excellent.Socrates_excellent" 1.0 1.0 0.0 null))
                      (set `self.CurrentAudioComponent` _returnvalue_7)
                      (`/Game/Dialogue/WB_Dialogue.SetDialogueOptions` _ui "What do you teach about virtue?" "What is your famous claim about wisdom?" "I think I'm ready for the test")
                      (`/Game/Dialogue/WB_Dialogue.ShowOptionsPanel` _ui))))))))))))

(event `self.Talk`
  (bind _returnvalue (`GameplayStatics.GetPlayerController` 0))
  (bind _dialoguestage (`self.DialogueStage`))
  (if (`self.CanTalk?`)
    (set `self.CanTalk?` false)
    (bind _returnvalue_2 (`|CreateWidget` "/Game/Dialogue/WB_Dialogue.WB_Dialogue_C" _returnvalue self))
    (bind _output_get (set `self.UI` _returnvalue_2))
    (`UserWidget.AddToViewport` _output_get 0)
    (`WidgetBlueprintLibrary.SetInputMode_GameAndUIEx` _returnvalue _output_get "DoNotLock" false)
    (set `PlayerController.bShowMouseCursor` true _returnvalue)
    (if (== _dialoguestage 0)
      (`/Game/Dialogue/WB_Dialogue.AddChatLine` _output_get (`KismetTextLibrary.Conv_StringToText` "Ah, you approach me willingly? Most people cross to the other side of the agora when they see me coming. I am Socrates — and I have questions for you. But first, tell me what you wish to know.") false)
      (bind _returnvalue_3 (`GameplayStatics.SpawnSound2D` "/Game/Audio/Socrates/Socrates_Intro.Socrates_Intro" 1.0 1.0 0.0 null))
      (set `self.CurrentAudioComponent` _returnvalue_3)
      (`self.CompleteSpecificObjective` "obj_greece_find_socrates")
      (`/Game/Dialogue/WB_Dialogue.SetDialogueOptions` _output_get "What do you teach about virtue?" "What do you know about the missing golden owl?" "What is your famous claim about wisdom?")
      (`/Game/Dialogue/WB_Dialogue.ShowOptionsPanel` _output_get)
      (elif (== _dialoguestage 1)
        (`/Game/Dialogue/WB_Dialogue.AddChatLine` _output_get (`KismetTextLibrary.Conv_StringToText` "You return! Good — a mind that seeks answers twice is worth more than one that never asks at all. What shall we examine today?") false)
        (`GameplayStatics.PlaySound2D` null 1.0 1.0 0.0 null null)
        (`/Game/Dialogue/WB_Dialogue.SetDialogueOptions` _output_get "Tell me about justice and wrongdoing" "What were the charges against you?" "I think I'm ready for the test")
        (`/Game/Dialogue/WB_Dialogue.ShowOptionsPanel` _output_get)
        (elif (== _dialoguestage 2)
          (`/Game/Dialogue/WB_Dialogue.AddChatLine` _output_get (`KismetTextLibrary.Conv_StringToText` "You have proven yourself a true thinker. Go now — carry this wisdom with you, and never stop questioning!") false)
          (`GameplayStatics.PlaySound2D` null 1.0 1.0 0.0 null null)
          (set `self.CanTalk?` true)
          (else
            (`self.ShowCurrentDialogueStage`)
            (set `self.CanTalk?` true)))))))

(event `ShowCurrentDialogueStage`
  (bind _returnvalue (`KismetTextLibrary.Conv_StringToText` "What charges were brought against me at my trial?"))
  (bind _returnvalue_2 (`GameplayStatics.GetPlayerController` 0))
  (bind _returnvalue_3 (`KismetTextLibrary.Conv_StringToText` "Now let us test YOUR knowledge! What did I teach about virtue?"))
  (bind _returnvalue_4 (`KismetTextLibrary.Conv_StringToText` "Where was the golden owl last seen before it went missing?"))
  (bind _returnvalue_5 (`KismetTextLibrary.Conv_StringToText` "Where did I see Kleon last night?"))
  (bind _ui (`self.UI`))
  (bind _ui_2 (`self.UI`))
  (bind _ui_3 (`self.UI`))
  (bind _ui_4 (`self.UI`))
  (bind _ui_5 (`self.UI`))
  (if (== (`self.DialogueStage`) 2)
    (`/Game/Dialogue/WB_Dialogue.AddChatLine` _ui_4 _returnvalue_3 false)
    (set `self.Current Quiz Question` (`KismetTextLibrary.Conv_TextToString` _returnvalue_3))
    (`/Game/Dialogue/WB_Dialogue.SetDialogueOptions` _ui_4 "Virtue is knowledge — no one does wrong willingly" "Virtue is physical strength and wealth" "Virtue cannot be defined by mortals")
    (`/Game/Dialogue/WB_Dialogue.ShowOptionsPanel` _ui_4)
    (`Widget.SetVisibility` (`/Game/Dialogue/WB_Dialogue.InputBox_Border` _ui_4) "SelfHitTestInvisible")
    (`Widget.SetVisibility` (`/Game/Dialogue/WB_Dialogue.BTN_Option4` _ui_4) "Visible")
    (`TextBlock.SetText` (`/Game/Dialogue/WB_Dialogue.Txt_Option4` _ui_4) (`KismetTextLibrary.Conv_StringToText` "Ask Socrates for a hint"))
    (elif (== (`self.DialogueStage`) 3)
      (`/Game/Dialogue/WB_Dialogue.AddChatLine` _ui_5 _returnvalue_4 false)
      (set `self.Current Quiz Question` (`KismetTextLibrary.Conv_TextToString` _returnvalue_4))
      (`/Game/Dialogue/WB_Dialogue.SetDialogueOptions` _ui_5 "At the port of Piraeus" "In the agora marketplace" "At Athena's feet inside the Parthenon")
      (`/Game/Dialogue/WB_Dialogue.ShowOptionsPanel` _ui_5)
      (`Widget.SetVisibility` (`/Game/Dialogue/WB_Dialogue.InputBox_Border` _ui_5) "SelfHitTestInvisible")
      (`Widget.SetVisibility` (`/Game/Dialogue/WB_Dialogue.BTN_Option4` _ui_5) "Visible")
      (`TextBlock.SetText` (`/Game/Dialogue/WB_Dialogue.Txt_Option4` _ui_5) (`KismetTextLibrary.Conv_StringToText` "Ask Socrates for a hint"))
      (elif (== (`self.DialogueStage`) 4)
        (`/Game/Dialogue/WB_Dialogue.AddChatLine` _ui_2 _returnvalue_5 false)
        (set `self.Current Quiz Question` (`KismetTextLibrary.Conv_TextToString` _returnvalue_5))
        (`/Game/Dialogue/WB_Dialogue.SetDialogueOptions` _ui_2 "At the gates of the Acropolis" "Near the docks at Piraeus" "Behind the statue of Athena inside the Parthenon")
        (`/Game/Dialogue/WB_Dialogue.ShowOptionsPanel` _ui_2)
        (`Widget.SetVisibility` (`/Game/Dialogue/WB_Dialogue.InputBox_Border` _ui_2) "SelfHitTestInvisible")
        (`Widget.SetVisibility` (`/Game/Dialogue/WB_Dialogue.BTN_Option4` _ui_2) "Visible")
        (`TextBlock.SetText` (`/Game/Dialogue/WB_Dialogue.Txt_Option4` _ui_2) (`KismetTextLibrary.Conv_StringToText` "Ask Socrates for a hint"))
        (elif (== (`self.DialogueStage`) 5)
          (`/Game/Dialogue/WB_Dialogue.AddChatLine` _ui _returnvalue false)
          (set `self.Current Quiz Question` (`KismetTextLibrary.Conv_TextToString` _returnvalue))
          (`/Game/Dialogue/WB_Dialogue.SetDialogueOptions` _ui "Corrupting the youth and impiety against the gods" "Stealing from the treasury of Athens" "Plotting against Pericles")
          (`/Game/Dialogue/WB_Dialogue.ShowOptionsPanel` _ui)
          (`Widget.SetVisibility` (`/Game/Dialogue/WB_Dialogue.InputBox_Border` _ui) "SelfHitTestInvisible")
          (`Widget.SetVisibility` (`/Game/Dialogue/WB_Dialogue.BTN_Option4` _ui) "Visible")
          (`TextBlock.SetText` (`/Game/Dialogue/WB_Dialogue.Txt_Option4` _ui) (`KismetTextLibrary.Conv_StringToText` "Ask Socrates for a hint"))
          (elif (== (`self.DialogueStage`) 6)
            (`/Game/Dialogue/WB_Dialogue.AddChatLine` _ui_3 (`KismetTextLibrary.Conv_StringToText` "Wonderful! You have proven that you truly listen and think — the mark of a philosopher!") false)
            (`KismetSystemLibrary.Delay` 4.0)
            (`Widget.RemoveFromParent` _ui_3)
            (`WidgetBlueprintLibrary.SetInputMode_GameOnly` _returnvalue_2)
            (set `PlayerController.bShowMouseCursor` false _returnvalue_2)
            (`/Engine/EditorBlueprintResources/StandardMacros.IsValid` (`self.CurrentAudioComponent`)
              (:`Is Valid`
                (`AudioComponent.Stop` (`self.CurrentAudioComponent`))))))))))

(event `self.ReceiveBeginPlay`
  (`parent.ReceiveBeginPlay`)
  (add `/Game/Blueprints/BP_HttpClient_Component.OnAIResponseReceived` (`self.BP_HttpClient_Component`) (delegate `self.OnAIResponseReceived_Event`)))

(event `self.OnAIResponseReceived_Event`
  (params (ResponseText :type String))
  (`self.AddToHistory` ResponseText "AI")
  (`/Game/Dialogue/WB_Dialogue.AddChatLine` (`self.UI`) (`KismetTextLibrary.Conv_StringToText` ResponseText) false)
  (if (`self.IsHintResponse`)
    (set `self.IsHintResponse` false)
    (bind _myplayercharacter (`/Game/ThirdPerson/CommonFunctionLibrary.GetMyPlayerCharacter`))
    (`/Game/ThirdPerson/Blueprints/BP_ThirdPersonCharacter.DeductKP` _myplayercharacter 5))
  (`self.CheckQuestKeywords` ResponseText)
  (bind _myplayercharacter_2 (`/Game/ThirdPerson/CommonFunctionLibrary.GetMyPlayerCharacter`))
  (bind _returnvalue (`self.GetComponentByClass` _myplayercharacter_2 "/Game/ThirdPerson/QuestSYstem/QuestLog_Component.QuestLog_Component_C"))
  (for _array_element (`/Game/ThirdPerson/QuestSYstem/QuestLog_Component.CurrentQuests` _returnvalue)
    (`/Engine/EditorBlueprintResources/StandardMacros.IsValid` _array_element
      (:`Is Valid`
        (for _array_element_2 (`.Objectives_21_75F1BA2A457170AB65DED5B45FFC78A1` (break `/Game/ThirdPerson/QuestSYstem/StageDetails` (`/Game/ThirdPerson/QuestSYstem/BP_QuestBase.CurrentStageDetails` _array_element)))
          (bind (_objectivename _description _type _objectiveid) (break `/Game/ThirdPerson/QuestSYstem/ObjectiveDetails` _array_element_2))
          (bind _iscomplete (`/Game/ThirdPerson/QuestSYstem/BP_QuestBase.IsObjectiveComplete` _array_element _objectiveid))
          (if (not _iscomplete)
            (if (`KismetArrayLibrary.Array_Contains` (`self.ObjectivesToComplete`) _objectiveid)
              (`/Game/ThirdPerson/QuestSYstem/BP_QuestBase.UpdateObjectiveProgress` _array_element _objectiveid 1)
              (`self.ProcessQuestForCodex` _array_element)
              (break)))))))
  (for _array_element_3 (`/Game/ThirdPerson/QuestSYstem/QuestLog_Component.CompletedQuestActors` _returnvalue)
    (`self.ProcessQuestForCodex` _array_element_3))
  (`KismetSystemLibrary.Delay` 6.0)
  (`self.ShowCurrentDialogueStage`))

(fn `CompleteQuestObjectives`
  (bind _myplayercharacter (`/Game/ThirdPerson/CommonFunctionLibrary.GetMyPlayerCharacter`))
  (for _array_element (`/Game/ThirdPerson/QuestSYstem/QuestLog_Component.CurrentQuests` (`self.GetComponentByClass` _myplayercharacter "/Game/ThirdPerson/QuestSYstem/QuestLog_Component.QuestLog_Component_C"))
    (for _array_element_2 (`self.ObjectivesToComplete`)
      (bind _iscomplete (`/Game/ThirdPerson/QuestSYstem/BP_QuestBase.IsObjectiveComplete` _array_element _array_element_2))
      (if (not _iscomplete)
        (`/Game/ThirdPerson/QuestSYstem/BP_QuestBase.UpdateObjectiveProgress` _array_element _array_element_2 1)
        (break)))))

(fn `CompleteSpecificObjective`
  (params (ObjectiveID :type String))
  (bind _myplayercharacter (`/Game/ThirdPerson/CommonFunctionLibrary.GetMyPlayerCharacter`))
  (for _array_element (`/Game/ThirdPerson/QuestSYstem/QuestLog_Component.CurrentQuests` (`self.GetComponentByClass` _myplayercharacter "/Game/ThirdPerson/QuestSYstem/QuestLog_Component.QuestLog_Component_C"))
    (`/Game/ThirdPerson/QuestSYstem/BP_QuestBase.UpdateObjectiveProgress` _array_element ObjectiveID 1)))

(fn `HandleQuizAnswer`
  (params (AnswerText :type String))
  (bind _dialoguestage (`self.DialogueStage`))
  (bind _ui (`self.UI`))
  (if (== _dialoguestage 2)
    (if (`KismetStringLibrary.EqualEqual_StrStr` AnswerText "Virtue is knowledge — no one does wrong willingly")
      (bind _myplayercharacter (`/Game/ThirdPerson/CommonFunctionLibrary.GetMyPlayerCharacter`))
      (`/Game/ThirdPerson/Blueprints/BP_ThirdPersonCharacter.AddKP` _myplayercharacter 10)
      (`/Game/Dialogue/WB_Dialogue.AddChatLine` _ui (`KismetTextLibrary.Conv_StringToText` "Correct! Virtue IS knowledge — those who truly know what is good will always act accordingly.") false)
      (`self.CompleteSpecificObjective` "obj_greece_learn_ethics")
      (bind _myplayercharacter_2 (`/Game/ThirdPerson/CommonFunctionLibrary.GetMyPlayerCharacter`))
      (`/Game/ThirdPerson/Codex/BP_CodexSystem.UnlockEntry` (`/Game/ThirdPerson/Blueprints/BP_ThirdPersonCharacter.CodexSystem` _myplayercharacter_2) "codex_greece_socrates")
      (`|ExecutionSequence`
        (:`then_0`
          (set `self.DialogueStage` (+ _dialoguestage 1))
          (`self.ShowCurrentDialogueStage` self)))
      (else
        (bind _myplayercharacter_3 (`/Game/ThirdPerson/CommonFunctionLibrary.GetMyPlayerCharacter`))
        (bind _bgameover (`/Game/ThirdPerson/Blueprints/BP_ThirdPersonCharacter.DeductKP` _myplayercharacter_3 5))
        (if _bgameover
          (bind _returnvalue (`|CreateWidget` "/Game/ThirdPerson/QuestSYstem/UI/WBP_GameOver.WBP_GameOver_C"))
          (`UserWidget.AddToViewport` _returnvalue 0)
          (else
            (`/Game/Dialogue/WB_Dialogue.AddChatLine` _ui (`KismetTextLibrary.Conv_StringToText` "Not quite. I teach that virtue is knowledge — no one does wrong willingly, only out of ignorance.") false)
            (`self.ShowCurrentDialogueStage`)))))
    (elif (== _dialoguestage 3)
      (if (`KismetStringLibrary.EqualEqual_StrStr` AnswerText "At Athena's feet inside the Parthenon")
        (bind _myplayercharacter_4 (`/Game/ThirdPerson/CommonFunctionLibrary.GetMyPlayerCharacter`))
        (`/Game/ThirdPerson/Blueprints/BP_ThirdPersonCharacter.AddKP` _myplayercharacter_4 10)
        (`/Game/Dialogue/WB_Dialogue.AddChatLine` _ui (`KismetTextLibrary.Conv_StringToText` "Correct! The golden owl was placed at Athena's feet by the priests — and that is where it was taken from.") false)
        (`self.CompleteSpecificObjective` "obj_greece_learn_knowledge")
        (bind _myplayercharacter_5 (`/Game/ThirdPerson/CommonFunctionLibrary.GetMyPlayerCharacter`))
        (`/Game/ThirdPerson/Codex/BP_CodexSystem.UnlockEntry` (`/Game/ThirdPerson/Blueprints/BP_ThirdPersonCharacter.CodexSystem` _myplayercharacter_5) "codex_greece_socrates")
        (`|ExecutionSequence`
          (:`then_0`
            (set `self.DialogueStage` (+ _dialoguestage 1))
            (`self.ShowCurrentDialogueStage` self)))
        (else
          (bind _myplayercharacter_6 (`/Game/ThirdPerson/CommonFunctionLibrary.GetMyPlayerCharacter`))
          (bind _bgameover_2 (`/Game/ThirdPerson/Blueprints/BP_ThirdPersonCharacter.DeductKP` _myplayercharacter_6 5))
          (if _bgameover_2
            (bind _returnvalue_2 (`|CreateWidget` "/Game/ThirdPerson/QuestSYstem/UI/WBP_GameOver.WBP_GameOver_C"))
            (`UserWidget.AddToViewport` _returnvalue_2 0)
            (else
              (`/Game/Dialogue/WB_Dialogue.AddChatLine` _ui (`KismetTextLibrary.Conv_StringToText` "Not quite. The owl stood at the feet of the Athena Parthenos inside the Parthenon before it vanished.") false)
              (`self.ShowCurrentDialogueStage`)))))
      (elif (== _dialoguestage 4)
        (if (`KismetStringLibrary.EqualEqual_StrStr` AnswerText "Behind the statue of Athena inside the Parthenon")
          (bind _myplayercharacter_7 (`/Game/ThirdPerson/CommonFunctionLibrary.GetMyPlayerCharacter`))
          (`/Game/ThirdPerson/Blueprints/BP_ThirdPersonCharacter.AddKP` _myplayercharacter_7 10)
          (`/Game/Dialogue/WB_Dialogue.AddChatLine` _ui (`KismetTextLibrary.Conv_StringToText` "Correct! I saw Kleon crouching behind Athena's great statue, hiding something wrapped in cloth.") false)
          (`self.CompleteSpecificObjective` "obj_greece_learn_kleon")
          (bind _myplayercharacter_8 (`/Game/ThirdPerson/CommonFunctionLibrary.GetMyPlayerCharacter`))
          (`/Game/ThirdPerson/Codex/BP_CodexSystem.UnlockEntry` (`/Game/ThirdPerson/Blueprints/BP_ThirdPersonCharacter.CodexSystem` _myplayercharacter_8) "codex_greece_socrates")
          (`|ExecutionSequence`
            (:`then_0`
              (set `self.DialogueStage` (+ (`self.DialogueStage`) 1))
              (`self.ShowCurrentDialogueStage` self)))
          (else
            (bind _myplayercharacter_9 (`/Game/ThirdPerson/CommonFunctionLibrary.GetMyPlayerCharacter`))
            (bind _bgameover_3 (`/Game/ThirdPerson/Blueprints/BP_ThirdPersonCharacter.DeductKP` _myplayercharacter_9 5))
            (if _bgameover_3
              (bind _returnvalue_3 (`|CreateWidget` "/Game/ThirdPerson/QuestSYstem/UI/WBP_GameOver.WBP_GameOver_C"))
              (`UserWidget.AddToViewport` _returnvalue_3 0)
              (else
                (`/Game/Dialogue/WB_Dialogue.AddChatLine` _ui (`KismetTextLibrary.Conv_StringToText` "Not quite.") false)
                (`self.ShowCurrentDialogueStage`)))))
        (elif (== _dialoguestage 5)
          (if (`KismetStringLibrary.EqualEqual_StrStr` AnswerText "Corrupting the youth and impiety against the gods")
            (bind _myplayercharacter_10 (`/Game/ThirdPerson/CommonFunctionLibrary.GetMyPlayerCharacter`))
            (`/Game/ThirdPerson/Blueprints/BP_ThirdPersonCharacter.AddKP` _myplayercharacter_10 10)
            (`/Game/Dialogue/WB_Dialogue.AddChatLine` _ui (`KismetTextLibrary.Conv_StringToText` "Correct! Those are the charges — though I have only ever encouraged the young to think for themselves.") false)
            (`self.CompleteSpecificObjective` "obj_greece_learn_trial")
            (`self.CompleteSpecificObjective` "obj_greece_socrates_quiz")
            (bind _myplayercharacter_11 (`/Game/ThirdPerson/CommonFunctionLibrary.GetMyPlayerCharacter`))
            (`/Game/ThirdPerson/Codex/BP_CodexSystem.UnlockEntry` (`/Game/ThirdPerson/Blueprints/BP_ThirdPersonCharacter.CodexSystem` _myplayercharacter_11) "codex_greece_socrates")
            (`|ExecutionSequence`
              (:`then_0`
                (set `self.DialogueStage` (+ (`self.DialogueStage`) 1))
                (`self.ShowCurrentDialogueStage` self)))
            (else
              (bind _myplayercharacter_12 (`/Game/ThirdPerson/CommonFunctionLibrary.GetMyPlayerCharacter`))
              (bind _bgameover_4 (`/Game/ThirdPerson/Blueprints/BP_ThirdPersonCharacter.DeductKP` _myplayercharacter_12 5))
              (if _bgameover_4
                (bind _returnvalue_4 (`|CreateWidget` "/Game/ThirdPerson/QuestSYstem/UI/WBP_GameOver.WBP_GameOver_C"))
                (`UserWidget.AddToViewport` _returnvalue_4 0)
                (else
                  (`/Game/Dialogue/WB_Dialogue.AddChatLine` _ui (`KismetTextLibrary.Conv_StringToText` "Not quite. I was charged with corrupting the youth and impiety — for asking questions that made powerful men uncomfortable.") false)
                  (`self.ShowCurrentDialogueStage`))))))))))

(fn `ProcessQuestForCodex`
  (params (QuestActor :type "/Game/ThirdPerson/QuestSYstem/BP_QuestBase Object Reference"))
  (bind _returnvalue (`self.GetComponentByClass` (`GameplayStatics.GetPlayerCharacter` 0) "/Game/ThirdPerson/Codex/BP_CodexSystem.BP_CodexSystem_C"))
  (bind (_value _returnvalue_2) (`BlueprintMapLibrary.Map_Find` (`self.QuestToCodexMap`) "obj_bonus"))
  (set `self.CompletedCount` 0)
  (for _array_element (`self.ObjectivesToComplete`)
    (bind _iscomplete (`/Game/ThirdPerson/QuestSYstem/BP_QuestBase.IsObjectiveComplete` QuestActor _array_element))
    (if _iscomplete
      (set `self.CompletedCount` (+ (`self.CompletedCount`) 1))
      (bind (_value_2 _returnvalue_3) (`BlueprintMapLibrary.Map_Find` (`self.QuestToCodexMap`) _array_element))
      (if _returnvalue_3
        (`/Engine/EditorBlueprintResources/StandardMacros.IsValid` _returnvalue
          (:`Is Valid`
            (`/Game/ThirdPerson/Codex/BP_CodexSystem.UnlockEntry` _returnvalue (`KismetStringLibrary.Conv_StringToName` _value_2)))))))
  (if (== (`self.CompletedCount`) (`KismetArrayLibrary.Array_Length` (`self.ObjectivesToComplete`)))
    (if _returnvalue_2
      (`/Game/ThirdPerson/Codex/BP_CodexSystem.UnlockEntry` (`self.GetComponentByClass` (`GameplayStatics.GetPlayerCharacter` 0) "/Game/ThirdPerson/Codex/BP_CodexSystem.BP_CodexSystem_C") (`KismetStringLibrary.Conv_StringToName` _value)))))

(fn `UserConstructionScript`
  (`parent.UserConstructionScript`))